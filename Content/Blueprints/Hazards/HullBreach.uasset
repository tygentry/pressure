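; Hull breach hazard that sprays water with looping or triggered audio and lowers hull integrity until it is plugged.
; StartBreach, optionally run on play, activates the leak effects, enables PressReceiver query collision and reduces integrity through SystemsController.
; PlugBreach stops the leak, briefly shows welding effects with sound unless loading a save, then restores integrity.
; It also decrements the SubDisplayInterface breach count keyed by the actor's first tag.
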(event `self.ReceiveBeginPlay`
  ;[1 1 1] Setup
  (`parent.ReceiveBeginPlay`)
  (`FXSystemComponent.SetFloatParameter` (`self.ParticleSystem`) "Lifetime" (`self.WaterParticleLifetime`))
  (`PrimitiveComponent.SetCollisionEnabled` (`self.PressReceiver`) "NoCollision")
  (if (`self.StartOnPlay`)
    (`self.StartBreach`)))

(event `PlugBreach`
  (params (`LoadingSave?` :type Boolean))
  (bind _weldedparticlesystem (`self.WeldedParticleSystem`))
  (bind _returnvalue (`KismetStringLibrary.Conv_NameToString` (`|GetArrayItem` (`self.Tags`))))
  ;[1 1 1] Plug breach
  (`ActorComponent.Deactivate` (`self.ParticleSystem`))
  (`AudioComponent.Stop` (`self.Audio`))
  (if (not `LoadingSave?`)
    (`ActorComponent.Activate` _weldedparticlesystem false)
    (`GameplayStatics.PlaySound2D` "/Game/SFX/WeldBreachCue.WeldBreachCue" 1.0 1.0 0.0 null null))
  (set `self.BreachActive?` false)
  (`PrimitiveComponent.SetCollisionEnabled` (`self.PressReceiver`) "NoCollision")
  (`KismetSystemLibrary.Delay` 0.9)
  (`ActorComponent.Deactivate` _weldedparticlesystem)
  (bind _outactors (`GameplayStatics.GetAllActorsOfClass` "/Game/Blueprints/Controllers/SystemsController.SystemsController_C"))
  (`/Game/Blueprints/Controllers/SystemsController.ChangeHullIntegrity` (`|GetArrayItem` _outactors) 10)
  ;[1 1 1] Update Status Display
  (bind _outactors_2 (`GameplayStatics.GetAllActorsOfClass` "/Game/Blueprints/Interfaces/Bridge/SubDisplayInterface.SubDisplayInterface_C"))
  (bind _hullbreaches (`/Game/Blueprints/Interfaces/Bridge/SubDisplayInterface.HullBreaches` (`|GetArrayItem` _outactors_2)))
  (bind (_value _returnvalue_2) (`BlueprintMapLibrary.Map_Find` _hullbreaches _returnvalue))
  (if _returnvalue_2
    (`BlueprintMapLibrary.Map_Add` _hullbreaches _returnvalue (- _value 1))))

(event `StartBreach`
  ;[1 1 1] Start hull breach
  (`ActorComponent.Activate` (`self.ParticleSystem`) false)
  (`AudioComponent.Play` (`self.Audio`) 0.0)
  (set `self.BreachActive?` true)
  (`PrimitiveComponent.SetCollisionEnabled` (`self.PressReceiver`) "QueryOnly")
  (bind _outactors (`GameplayStatics.GetAllActorsOfClass` "/Game/Blueprints/Controllers/SystemsController.SystemsController_C"))
  (`/Game/Blueprints/Controllers/SystemsController.ChangeHullIntegrity` (`|GetArrayItem` _outactors) -10))

(fn `UserConstructionScript`)