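; WallLight is an environmental light actor that switches its look between a low-power and a high-power state.
; The LowPower event gives the Bulb a red lamp material and turns the PointLight red, while HighPower applies the standard lamp material and a warm light color.
; Both events change only material and color, and the construction script just calls its parent.
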(event `LowPower`
  (`PrimitiveComponent.SetMaterial` (`self.Bulb`) 0 "/Game/EnvironmentalMaterials/LampLightRed.LampLightRed")
  (`LightComponent.SetLightColor` (`self.PointLight`) (struct :`R` 0.890196 :`B` 0.015686 :`A` 1.0) true))

(event `HighPower`
  (`PrimitiveComponent.SetMaterial` (`self.Bulb`) 0 "/Game/EnvironmentalMaterials/LampLight.LampLight")
  (`LightComponent.SetLightColor` (`self.PointLight`) (struct :`R` 0.991102 :`G` 0.775822 :`B` 0.48515 :`A` 1.0) true))

(fn `UserConstructionScript`
  (`parent.UserConstructionScript`))