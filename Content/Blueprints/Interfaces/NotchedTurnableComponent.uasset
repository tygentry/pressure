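; Base for a notched dial that the player turns with the mouse in discrete steps, with a click sound per step.
; BeginPlay builds the notch angle list from count and spacing, then yaws the dial to its initial notch, assuming zero starting local rotation.
; While held, Tick compares mouse angle to grab offset, stepping one notch past half-spacing, within end limits.
; SetNotchPosition jumps to a given notch without sound or bounds checks.
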(event `self.ReceiveBeginPlay`
  (bind _notchedrotationslist (`self.NotchedRotationsList`))
  (bind _initialnotchposition (`self.InitialNotchPosition`))
  (bind _notchedrotationslist_2 (`self.NotchedRotationsList`))
  (bind _initialnotchposition_2 (`self.InitialNotchPosition`))
  (bind _returnvalue (/ (`self.NotchSpacingDistance`) 2.0))
  (bind _returnvalue_2 (- (/ (`self.NotchCount`) 2) 1))
  (bind _returnvalue_3 (/ (- (`self.NotchCount`) 1) 2))
  ;[1 1 1] Find the rotations each notch represents
  (`parent.ReceiveBeginPlay`)
  (if (== (mod (`self.NotchCount`) 2) 0)
    (`KismetArrayLibrary.Array_Add` _notchedrotationslist (+ (* -1 _returnvalue) (`self.NotchBaseRotation`))) ; even notch count
    (`KismetArrayLibrary.Array_Add` _notchedrotationslist (+ (`self.NotchBaseRotation`) _returnvalue))
    (for _index (range 1 (+ _returnvalue_2 1))
      (`KismetArrayLibrary.Array_Add` (`self.NotchedRotationsList`) (+ (/ (`self.NotchSpacingDistance`) 2.0) (* _index (`self.NotchSpacingDistance`)))))
    (for _index_2 (range 1 (+ _returnvalue_2 1))
      (`KismetArrayLibrary.Array_Insert` (`self.NotchedRotationsList`) (+ (* -1 (/ (`self.NotchSpacingDistance`) 2.0)) (* (* _index_2 -1) (`self.NotchSpacingDistance`)))))
    (else
      (`KismetArrayLibrary.Array_Add` (`self.NotchedRotationsList`) (`self.NotchBaseRotation`)) ; odd notch count
      (for _index_3 (range 1 (+ _returnvalue_3 1))
        (`KismetArrayLibrary.Array_Add` (`self.NotchedRotationsList`) (+ (`self.NotchBaseRotation`) (* _index_3 (`self.NotchSpacingDistance`)))))
      (for _index_4 (range 1 (+ _returnvalue_3 1))
        (`KismetArrayLibrary.Array_Insert` (`self.NotchedRotationsList`) (+ (`self.NotchBaseRotation`) (* (* _index_4 -1) (`self.NotchSpacingDistance`)))))))
  (for (_array_element _array_index) _notchedrotationslist_2
    (if (> _array_element 360.0)
      (`KismetArrayLibrary.Array_Set` (`self.NotchedRotationsList`) _array_index (- _array_element 360.0)) ; too high
      (elif (< _array_element 0.0)
        (`KismetArrayLibrary.Array_Set` (`self.NotchedRotationsList`) _array_index (+ _array_element 360.0)) ; too low
      )))
  (for _array_element_2 _notchedrotationslist_2
    _)
  ;;[1 1 1] Rotate Dial to match Initial Notch Position
  (`SceneComponent.K2_AddLocalRotation` (`self.DefaultSceneRoot`) (`KismetMathLibrary.MakeRotator` 0.0 0.0 (`|GetArrayItem` (`self.NotchedRotationsList`) _initialnotchposition)) false false) ; REALLY FUCKING IMPORTANT: we assume the dial starts with local rotation of 0, if it doesn't things break
  (set `self.CurrentNotchPosition` _initialnotchposition)
  ;[1 1 1] Alert if InitialNotch is Invalid
  (if (< _initialnotchposition_2 0)
    (`KismetSystemLibrary.PrintString` (`KismetStringLibrary.Concat_StrStr` (`KismetSystemLibrary.GetObjectName` self) " IS BROKEN CUZ YOU SET UR INITIAL NOTCH POSITION LESS THAN ZERO!!!") true true (struct :`R` 0.71875 :`G` 0.010981 :`A` 1.0) 10.0)
    (elif (>= _initialnotchposition_2 (`self.NotchCount`))
      (`KismetSystemLibrary.PrintString` (`KismetStringLibrary.Concat_StrStr` (`KismetSystemLibrary.GetObjectName` self) " IS BROKEN CUZ YOU SET UR INITIAL NOTCH POSITION TO BE GREATER THAN OR EQUAL TO YOUR NOTCH COUNT!!! LMAO!!!") true true (struct :`R` 0.625 :`B` 0.003511 :`A` 1.0) 10.0))))

(event `self.ReceiveTick`
  (params (DeltaSeconds :type "Float (single-precision)"))
  (bind _pointingupvector (`self.PointingUpVector`))
  (bind _returnvalue (/ (`self.NotchSpacingDistance`) 2.0))
  (bind _returnvalue_2 (`KismetMathLibrary.Normal` (`SceneComponent.GetRightVector` (`self.DefaultSceneRoot`))))
  (bind _returnvalue_3 (`KismetMathLibrary.DegAcos` (/ (`KismetMathLibrary.Dot_VectorVector` _pointingupvector _returnvalue_2) (* (`KismetMathLibrary.VSize` _pointingupvector) (`KismetMathLibrary.VSize` _returnvalue_2)))))
  ;[1 1 1] Tick Loop
  ;;[1 1 1] Get The Dial's Current Rotation
  (if (`self.Held`)
    (if (< (`KismetMathLibrary.Dot_VectorVector` _returnvalue_2 (`KismetMathLibrary.RotateAngleAxis` _pointingupvector 90.0 (`SceneComponent.GetUpVector` (`self.DefaultSceneRoot`)))) 0.0)
      (set `self.DialRotation` (- 360.0 _returnvalue_3))
      (else
        (set `self.DialRotation` _returnvalue_3)))
    ;;[1 1 1] Rotate The Dial if Needed
    (bind _rotation (`self.GetMouseRotationRelativeToOrigin`))
    (bind _deltarot (`self.Compare Mouse and Offset Rotation` _rotation (`self.PointClickedOffset`)))
    (if (> _deltarot _returnvalue)
      (if (< (`self.CurrentNotchPosition`) (- (`self.NotchCount`) 1))
        (`SceneComponent.K2_AddLocalRotation` (`self.DefaultSceneRoot`) (`KismetMathLibrary.MakeRotator` 0.0 0.0 (`self.NotchSpacingDistance`)) false false)
        (set `self.CurrentNotchPosition` (+ (`self.CurrentNotchPosition`) 1))
        (`GameplayStatics.PlaySoundAtLocation` "/Game/SFX/QuietKnobTurnCue.QuietKnobTurnCue" (`SceneComponent.K2_GetComponentLocation` (`self.DefaultSceneRoot`)) (struct) 1.0 1.0 0.0 null null null :!label _label))
      (elif (< _deltarot (* _returnvalue -1.0))
        (if (> (`self.CurrentNotchPosition`) 0)
          (`SceneComponent.K2_AddLocalRotation` (`self.DefaultSceneRoot`) (`KismetMathLibrary.MakeRotator` 0.0 0.0 (* (`self.NotchSpacingDistance`) -1.0)) false false)
          (set `self.CurrentNotchPosition` (- (`self.CurrentNotchPosition`) 1))
          (goto _label))))))

(event `SetNotchPosition`
  (params (Position :type Integer))
  ;[1 1 1] Set Notch Position
  (`SceneComponent.K2_AddLocalRotation` (`self.DefaultSceneRoot`) (`KismetMathLibrary.MakeRotator` 0.0 0.0 (* (- Position (`self.CurrentNotchPosition`)) (`self.NotchSpacingDistance`))) false false)
  (set `self.CurrentNotchPosition` Position))

(fn `GetOppositeRotation`
  (params (Rotation :type "Float (double-precision)"))
  (returns (OppositeRotation :type "Float (double-precision)"))
  (bind _returnvalue (+ Rotation 180.0))
  (if (> _returnvalue 360.0)
    (return (- _returnvalue 360.0))
    (else
      (return _returnvalue))))

(fn `UserConstructionScript`
  (`parent.UserConstructionScript`))