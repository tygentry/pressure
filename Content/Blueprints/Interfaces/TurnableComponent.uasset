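; Turnable dial that the player rotates with the mouse, spinning its root in local yaw between Hold and LetGo.
; Each held tick projects the cursor hit onto the root's axes and applies the shortest signed angle from the grab point.
; With TrackRot, DeltaRot accumulates for optional min/max limits, with lock flags blocking large jumps across a stop.
; DialRotation records the angle from the starting orientation; events can reset or set the rotation.
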(event `Hold`
  ;[1 1 1] Hold and Let Go Events
  (bind _rotation (`self.GetMouseRotationRelativeToOrigin`))
  (bind _output_get (set `self.PointClickedOffset` _rotation))
  (set `self.Held` true))

(event `Let Go`
  ;[1 1 1] Hold and Let Go Events
  (set `self.Held` false))

(event `self.ReceiveBeginPlay`
  ;[1 1 1] Set PointingUpVector on begin play
  (set `self.PointingUpVector` (`SceneComponent.GetRightVector` (`self.DefaultSceneRoot`))))

(event `ResetRotation`
  ;[1 1 1] Reset turnable to base rotation
  (`SceneComponent.K2_AddLocalRotation` (`self.DefaultSceneRoot`) (`KismetMathLibrary.MakeRotator` 0.0 0.0 (* -1 (`self.DeltaRot`))) false false)
  (set `self.DeltaRot` 0.0))

(event `self.ReceiveTick`
  (params (DeltaSeconds :type "Float (single-precision)"))
  (bind _pointingupvector (`self.PointingUpVector`))
  (bind _returnvalue (`KismetMathLibrary.Normal` (`SceneComponent.GetRightVector` (`self.DefaultSceneRoot`))))
  (bind _returnvalue_2 (`KismetMathLibrary.DegAcos` (/ (`KismetMathLibrary.Dot_VectorVector` _pointingupvector _returnvalue) (* (`KismetMathLibrary.VSize` _pointingupvector) (`KismetMathLibrary.VSize` _returnvalue)))))
  ;[1 1 1] Update DialRotation and rotate if needed
  (if (`self.Held`)
    (if (< (`KismetMathLibrary.Dot_VectorVector` _returnvalue (`KismetMathLibrary.RotateAngleAxis` _pointingupvector 90.0 (`SceneComponent.GetUpVector` (`self.DefaultSceneRoot`)))) 0.0)
      (set `self.DialRotation` (- 360.0 _returnvalue_2))
      (else
        (set `self.DialRotation` _returnvalue_2)))
    (bind _rotation (`self.GetMouseRotationRelativeToOrigin`))
    (bind _deltarot (`self.Compare Mouse and Offset Rotation` _rotation (`self.PointClickedOffset`)))
    (bind _returnvalue_3 (* _deltarot 1.0))
    (if (> _returnvalue_3 0.0)
      (if (or (and (> (+ (`self.DeltaRot`) _returnvalue_3) (`self.MaxDeltaRot`)) (!= (`self.MinDeltaRot`) (`self.MaxDeltaRot`))) (and (`self.LockedCounterclockwiseRot`) (> _returnvalue_3 (/ (`self.MaxDeltaRot`) 10.0))))
        (set `self.LockedClockwiseRot` true)
        (else
          (`SceneComponent.K2_AddLocalRotation` (`self.DefaultSceneRoot`) (`KismetMathLibrary.MakeRotator` 0.0 0.0 _returnvalue_3) false false :!label _label)
          (if (`self.TrackRot`)
            (bind _output_get (set `self.DeltaRot` (+ (stale _output_get) _returnvalue_3)))
            (set `self.LockedClockwiseRot` false)
            (set `self.LockedCounterclockwiseRot` false))))
      (elif (or (and (`self.LockedClockwiseRot`) (< _returnvalue_3 (* -1 (/ (`self.MaxDeltaRot`) 10.0)))) (and (< (+ (`self.DeltaRot`) _returnvalue_3) (`self.MinDeltaRot`)) (!= (`self.MinDeltaRot`) (`self.MaxDeltaRot`))))
        (set `self.LockedCounterclockwiseRot` true)
        (else
          (goto _label))))))

(event `SetTurnableDeltaRot`
  (params (Rotation :type "Float (double-precision)"))
  ;[1 1 1] Set turnable rotation and delta rot
  (`self.ResetRotation`)
  (`SceneComponent.K2_AddLocalRotation` (`self.DefaultSceneRoot`) (`KismetMathLibrary.MakeRotator` 0.0 0.0 Rotation) false false)
  (set `self.DeltaRot` Rotation))

(fn `Compare Mouse and Offset Rotation`
  (params (`Mouse Rotation` :type "Float (double-precision)") (`Offset Rotation` :type "Float (double-precision)"))
  (returns (DeltaRot :type "Float (double-precision)"))
  (bind _returnvalue (- `Offset Rotation` `Mouse Rotation`))
  (bind _returnvalue_2 (- `Mouse Rotation` `Offset Rotation`))
  (bind _returnvalue_3 (+ `Mouse Rotation` (- 360.0 `Offset Rotation`)))
  (bind _returnvalue_4 (+ `Offset Rotation` (- 360.0 `Mouse Rotation`)))
  (if (== `Mouse Rotation` `Offset Rotation`)
    (return 0.0)
    (elif (< `Mouse Rotation` `Offset Rotation`)
      (if (< _returnvalue _returnvalue_3)
        (return (* -1 _returnvalue)) ; counterclockwise
        (else
          (return _returnvalue_3) ; clockwise
        ))
      (elif (< _returnvalue_2 _returnvalue_4)
        (return _returnvalue_2) ; clockwise
        (else
          (return (* _returnvalue_4 -1.0)) ; counterclockwise
        )))))

(fn `DrawVectorLine`
  (params (Vector :type "Vector Structure") (Color :type "LinearColor Structure") (Duration :type "Float (double-precision)"))
  (bind _returnvalue (`SceneComponent.K2_GetComponentLocation` (`self.DefaultSceneRoot`)))
  (`KismetSystemLibrary.DrawDebugArrow` _returnvalue (+ _returnvalue (* (`KismetMathLibrary.Normal` Vector) 100.0)) 0.0 Color Duration 1.0))

(fn `GetMouseRotationRelativeToOrigin`
  (returns (Rotation :type "Float (double-precision)"))
  (bind _returnvalue (- (`.Location` (`GameplayStatics.BreakHitResult` (`PlayerController.GetHitResultUnderCursorByChannel` (`GameplayStatics.GetPlayerController` 0) "TraceTypeQuery1" true))) (`SceneComponent.K2_GetComponentLocation` (`self.DefaultSceneRoot`))))
  (bind _returnvalue_2 (- (`KismetMathLibrary.DegAtan2` (`KismetMathLibrary.Dot_VectorVector` _returnvalue (`KismetMathLibrary.Normal` (`SceneComponent.GetRightVector` (`self.DefaultSceneRoot`)))) (`KismetMathLibrary.Dot_VectorVector` _returnvalue (`KismetMathLibrary.Normal` (`SceneComponent.GetForwardVector` (`self.DefaultSceneRoot`))))) 90.0))
  (if (< _returnvalue_2 0.0)
    (return (+ _returnvalue_2 360.0))
    (else
      (return _returnvalue_2))))

(fn `PrintCurrentBearing`
  (`KismetSystemLibrary.PrintString` (`KismetStringLibrary.Conv_VectorToString` (`KismetMathLibrary.Normal` (`SceneComponent.GetRightVector` (`self.DefaultSceneRoot`)))) true true (struct :`R` 1.0 :`B` 0.767256 :`A` 1.0) 10.0))

(fn `UserConstructionScript`
  (`parent.UserConstructionScript`))