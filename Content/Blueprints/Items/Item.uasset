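; Base item Blueprint for physical objects that can be held and placed in receptacles.
; On BeginPlay, items flagged static turn off physics simulation, become unholdable and switch their mesh to the WorldStatic collision type.
; A timed lockout temporarily blocks receptacle placement so a removed item does not snap straight back in.
; A setter event records the item's most recent receptacle.
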(event `self.ReceiveBeginPlay`
  ;[1 1 1] Static Variable Check to Disable Phys Simulation
  (`parent.ReceiveBeginPlay`)
  (if (`self.IsStatic`)
    (`PrimitiveComponent.SetSimulatePhysics` (`self.StaticMesh`) false)
    (set `self.CanBeHeld` false)
    (`PrimitiveComponent.SetCollisionObjectType` (`self.StaticMesh`) "ECC_WorldStatic")))

(event `Prevent From Being Put In Receptacle`
  (params (Duration :type "Float (double-precision)"))
  ;[1 1 1] Prevent this item from being placed in a receptacle for a period of time (called when an object is removed from receptacle so it doesn't immediately go back in)
  (set `self.CanBePutInReceptacle` false)
  (`KismetSystemLibrary.Delay` Duration)
  (set `self.CanBePutInReceptacle` true))

(event `Set Most Recent Receptacle`
  (params (ItemReceptacle :type "/Game/Blueprints/Items/ItemReceptacle Object Reference"))
  (set `self.MostRecentReceptacle` ItemReceptacle))

(fn `UserConstructionScript`)