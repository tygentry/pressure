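; Usable fire extinguisher that sprays particles with looping or one-shot audio while in use and puts out fires.
; While active, Tick traces from the first-person camera, lowering the intensity of a hit Fire or letting an empty UsableReceptacle grab the extinguisher.
; Physics impacts above speed and impulse thresholds play light, medium or heavy metal clangs by velocity, throttled by a DoOnce and short delay.
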(event `self.ReceiveHit`
  (params (MyComp :type "PrimitiveComponent Object Reference") (Other :type "Actor Object Reference") (OtherComp :type "PrimitiveComponent Object Reference") (bSelfMoved :type Boolean) (HitLocation :type "Vector Structure") (HitNormal :type "Vector Structure") (NormalImpulse :type "Vector Structure") (Hit :type "HitResult Structure (by ref)"))
  (bind _returnvalue (`KismetMathLibrary.RandomFloatInRange` 0.99 1.01))
  (bind _returnvalue_2 (`SceneComponent.K2_GetComponentLocation` (`self.StaticMesh`)))
  (bind _returnvalue_3 (`PrimitiveComponent.GetPhysicsLinearVelocity` (`self.StaticMesh`) "None"))
  (bind _returnvalue_4 (`KismetMathLibrary.VSize` _returnvalue_3))
  (if (and (> _returnvalue_4 30.0) (> (`KismetMathLibrary.VSize` NormalImpulse) 600.0))
    (`/Engine/EditorBlueprintResources/StandardMacros.DoOnce` false :!label _label
      (:`Completed`
        (if (< _returnvalue_4 200.0)
          (`GameplayStatics.PlaySoundAtLocation` "/Game/SFX/MetalCollisionLightCue.MetalCollisionLightCue" _returnvalue_2 (struct) 1.0 _returnvalue 0.0 "/Game/SFX/PipeClangAttenuation.PipeClangAttenuation" null null)
          (`KismetSystemLibrary.Delay` 0.2)
          (goto _label :!via `Reset`)
          (elif (< _returnvalue_4 500.0)
            (`GameplayStatics.PlaySoundAtLocation` "/Game/SFX/MetalCollisionMedCue.MetalCollisionMedCue" _returnvalue_2 (struct) 1.0 _returnvalue 0.0 "/Game/SFX/PipeClangAttenuation.PipeClangAttenuation" null null)
            (`KismetSystemLibrary.Delay` 0.2)
            (goto _label :!via `Reset`)
            (else
              (`GameplayStatics.PlaySoundAtLocation` "/Game/SFX/MetalCollisionHeavyCue.MetalCollisionHeavyCue" _returnvalue_2 (struct) 1.0 _returnvalue 0.0 "/Game/SFX/PipeClangAttenuation.PipeClangAttenuation" null null)
              (`KismetSystemLibrary.Delay` 0.2)
              (goto _label :!via `Reset`))))))))

(event `self.UseUsable`
  (`ActorComponent.Activate` (`self.ParticleSystem`) false)
  (set `self.Active?` true)
  (`AudioComponent.Play` (`self.Audio`) 0.0))

(event `self.StopUsingUsable`
  (`ActorComponent.Deactivate` (`self.ParticleSystem`))
  (set `self.Active?` false)
  (`AudioComponent.Stop` (`self.Audio`)))

(event `self.ReceiveTick`
  (params (DeltaSeconds :type "Float (single-precision)"))
  (bind _asfirst_person_character (cast `/Game/FirstPersonBP/Blueprints/FirstPersonCharacter` (`GameplayStatics.GetPlayerCharacter` 0)))
  (if (`self.Active?`)
    (bind _firstpersoncamera (`/Game/FirstPersonBP/Blueprints/FirstPersonCharacter.FirstPersonCamera` _asfirst_person_character))
    (bind _returnvalue (`SceneComponent.K2_GetComponentLocation` _firstpersoncamera))
    (bind (_outhit _returnvalue_2) (`KismetSystemLibrary.LineTraceSingle` :`Start` _returnvalue :`End` (+ _returnvalue (- (* (`SceneComponent.GetForwardVector` _firstpersoncamera) 255.0) (-5.0 -10.0 15.0))) :`TraceChannel` "TraceTypeQuery1" :`DrawTime` 3.0))
    (if _returnvalue_2
      (bind (_bblockinghit _binitialoverlap _time _distance _location _impactpoint _normal _impactnormal _physmat _hitactor) (`GameplayStatics.BreakHitResult` _outhit))
      (bind _returnvalue_3 (`GameplayStatics.GetObjectClass` _hitactor))
      (if (== _returnvalue_3 "/Game/Blueprints/Usables/UsableReceptacle.UsableReceptacle_C")
        (bind _asusable_receptacle (cast `/Game/Blueprints/Usables/UsableReceptacle` _hitactor))
        (if (not (`/Game/Blueprints/Usables/UsableReceptacle.IsHoldingObject?` _asusable_receptacle))
          (`/Game/Blueprints/Usables/UsableReceptacle.GrabUsable` _asusable_receptacle self false))
        (elif (== _returnvalue_3 "/Game/Blueprints/Hazards/Fire.Fire_C")
          (bind _asfire (cast `/Game/Blueprints/Hazards/Fire` _hitactor))
          (`/Game/Blueprints/Hazards/Fire.ChangeIntensity` _asfire -1.0))))))

(fn `UserConstructionScript`
  (`parent.UserConstructionScript`))