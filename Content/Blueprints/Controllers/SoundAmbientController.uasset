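; SoundAmbientController is an actor that controls the game's music, with character theme, requiem and post-mortem events plus an engines tutorial theme.
; Most theme events fade out the shared PreAmbientTrack component, set its sound (some left empty) and fade back in without waiting.
; PlayNewAmbientTrack fades out any playing requiem, plays a 2D track via GetRandomTrack, then re-calls itself after a track-length plus random delay.
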(event `Play First Mate Post Mortem Theme`
  (bind _preambienttrack (`self.PreAmbientTrack`))
  ;[1 1 1] First Mate Post Mortem Theme
  (`AudioComponent.FadeOut` _preambienttrack 6.0 0.0 "Linear")
  (`AudioComponent.SetSound` _preambienttrack null)
  (`AudioComponent.FadeIn` _preambienttrack 8.0 1.0 0.0 "Linear"))

(event `Play Captain's Requiem`
  (bind _preambienttrack (`self.PreAmbientTrack`))
  ;[1 1 1] Captain's Requiem
  (`AudioComponent.FadeOut` _preambienttrack 4.0 0.0 "Linear")
  (`AudioComponent.SetSound` _preambienttrack null)
  (`AudioComponent.FadeIn` _preambienttrack 6.0 1.0 0.0 "Linear")
  (set `self.isRequiemPlaying` true))

(event `Play First Mate Theme`
  ;[1 1 1] First Mate Theme
  (`AudioComponent.FadeOut` (`self.PreAmbientTrack`) 6.0 0.0 "Linear")
  (`AudioComponent.SetSound` (`self.PreAmbientTrack`) "/Game/SoundMusic/Nate_s_Theme.Nate_s_Theme")
  (`AudioComponent.FadeIn` (`self.PreAmbientTrack`) 8.0 1.0 0.0 "Linear"))

(event `Play Captain's Theme`
  ;[1 1 1] Captain's Theme
  (`AudioComponent.FadeOut` (`self.PreAmbientTrack`) 6.0 0.0 "Linear")
  (`AudioComponent.SetSound` (`self.PreAmbientTrack`) "/Game/SoundMusic/Captain_s_Theme.Captain_s_Theme")
  (`AudioComponent.FadeIn` (`self.PreAmbientTrack`) 8.0 1.0 0.0 "Linear"))

(event `Play Engines Tutorial Theme`
  ;[1 1 1] Engines Tutorial Theme
  (`GameplayStatics.PushSoundMixModifier` "/Game/SoundMusic/SM_Music.SM_Music")
  (`AudioComponent.FadeIn` (`self.PreAmbientTrack`) 8.0 1.0 0.0 "Linear"))

(event `Play Sonar Theme`
  ;[1 1 1] Sonar Theme
  (`AudioComponent.FadeOut` (`self.PreAmbientTrack`) 6.0 0.0 "Linear")
  (`AudioComponent.SetSound` (`self.PreAmbientTrack`) "/Game/SoundMusic/Mort_s_Theme.Mort_s_Theme")
  (`AudioComponent.FadeIn` (`self.PreAmbientTrack`) 8.0 1.0 0.0 "Linear"))

(event `Play Kevin's Theme`
  ;[1 1 1] Kevin's Theme
  (`AudioComponent.FadeOut` (`self.PreAmbientTrack`) 6.0 0.0 "Linear")
  (`AudioComponent.SetSound` (`self.PreAmbientTrack`) "/Game/SoundMusic/Kevin_s_Theme.Kevin_s_Theme")
  (`AudioComponent.FadeIn` (`self.PreAmbientTrack`) 8.0 1.0 0.0 "Linear"))

(event `Play Sonar's Post Mortem Theme`
  (bind _preambienttrack (`self.PreAmbientTrack`))
  ;[1 1 1] Sonar Post Mortem Theme
  (`AudioComponent.FadeOut` _preambienttrack 6.0 0.0 "Linear")
  (`AudioComponent.SetSound` _preambienttrack "/Game/SoundMusic/Mort_Post_Mortem.Mort_Post_Mortem")
  (`AudioComponent.FadeIn` _preambienttrack 8.0 1.0 0.0 "Linear"))

(event `Play Kevin's Post Mortem Theme`
  (bind _preambienttrack (`self.PreAmbientTrack`))
  ;[1 1 1] Kevin's Post Mortem Theme
  (`AudioComponent.FadeOut` _preambienttrack 6.0 0.0 "Linear")
  (`AudioComponent.SetSound` _preambienttrack null)
  (`AudioComponent.FadeIn` _preambienttrack 8.0 1.0 0.0 "Linear"))

(event `PlayNewAmbientTrack`
  (bind _track (`self.GetRandomTrack` (`self.A_Tracks`)))
  (if (`self.isRequiemPlaying`)
    (`AudioComponent.FadeOut` (`self.PreAmbientTrack`) 8.0 0.0 "Linear")
    (set `self.isRequiemPlaying` false))
  (`GameplayStatics.PushSoundMixModifier` "/Game/SoundMusic/SM_Music.SM_Music")
  (`GameplayStatics.PlaySound2D` _track 0.3 1.0 0.0 null null)
  (`GameplayStatics.PopSoundMixModifier` "/Game/SoundMusic/SM_Music.SM_Music")
  (`KismetSystemLibrary.Delay` (+ (`SoundBase.Duration` _track) (`KismetMathLibrary.RandomFloatInRange` 35.0 90.0)))
  (`self.PlayNewAmbientTrack`))

(fn `UserConstructionScript`)