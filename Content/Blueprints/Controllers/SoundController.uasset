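; SoundController starts the game's muffled ambience as a 2D sound, either on BeginPlay when BeginSoundsOnStart is set or through the BeginGameSound event.
; Tick sets a Volume variable high while the DialogueController reports dialogue playing and low otherwise, but no live node applies it.
; Disconnected, unused nodes remain for volume fading, delayed music themes and a Play call.
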(event `Begin Game Sound`
  (`GameplayStatics.PlaySound2D` "/Game/SFX/AmbienceMuffledSub.AmbienceMuffledSub" 0.5 1.0 0.0 null null))

(event `self.ReceiveBeginPlay`
  (if (`self.BeginSoundsOnStart?`)
    (`self.Begin Game Sound`)))

(event `self.ReceiveTick`
  (params (DeltaSeconds :type "Float (single-precision)"))
  (if (`/Game/Blueprints/Controllers/DialogueController.isDialoguePlaying` (`self.DialogueControllerRef`))
    (bind _output_get (set `self.Volume` 1.0))
    (else
      (bind _output_get_2 (set `self.Volume` 0.1)))))

(fn `UserConstructionScript`)