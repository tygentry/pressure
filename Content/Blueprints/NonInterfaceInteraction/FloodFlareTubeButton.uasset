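; Pressable button that floods the flare tube, readying it in the flare interface display.
; A press depresses the button with a sound; if the tube holds an object, is open and is neither flooded nor flooding, it closes the door and starts flooding.
; After a fixed delay it marks the tube flooded, makes the object unholdable and switches the display from Flooding to Ready.
; Invalid presses flash an alert light; release resets the button.
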(event `self.OnPressed`
  (bind _flaretube (`self.FlareTube`))
  (bind _flaretube_2 (`self.FlareTube`))
  (bind _flaredisplaywidget (`/Game/Blueprints/Interfaces/WeaponsRoom/FlareInterface.FlareDisplayWidget` (`self.FlareInterface`)))
  (`parent.OnPressed`)
  (`SceneComponent.K2_SetRelativeLocation` (`self.ButtonCollision`) (0.0 -2.0 0.0) false false)
  (`GameplayStatics.PlaySoundAtLocation` "/Game/SFX/ButtonPressCue.ButtonPressCue" (`SceneComponent.K2_GetComponentLocation` (`self.DefaultSceneRoot`)) (struct) 1.0 1.0 0.0 null null null)
  (if (and (`/Game/Blueprints/Items/ItemReceptacle.isGrabbingObject` _flaretube) (not (`/Game/Blueprints/Interfaces/WeaponsRoom/FlareReceptacle.IsFlooded` _flaretube)) (`/Game/Blueprints/Interfaces/WeaponsRoom/FlareTube.IsOpen` (`self.FlareTubeMesh`)) (not (`/Game/Blueprints/Interfaces/WeaponsRoom/FlareReceptacle.IsFlooding` _flaretube)))
    (set `/Game/Blueprints/Interfaces/WeaponsRoom/FlareReceptacle.IsFlooding` true _flaretube_2)
    (`/Game/Blueprints/Interfaces/WeaponsRoom/FlareTube.CloseDoor` (`self.FlareTubeMesh`))
    (`KismetSystemLibrary.Delay` 8.0)
    (set `/Game/Blueprints/Interfaces/WeaponsRoom/FlareReceptacle.IsFlooding` false _flaretube_2)
    (set `/Game/Blueprints/Interfaces/WeaponsRoom/FlareReceptacle.IsFlooded` true _flaretube)
    (set `/Game/Blueprints/Items/Item.CanBeHeld` false (`/Game/Blueprints/Items/ItemReceptacle.MostRecentGrabbedObject` _flaretube))
    (`Widget.SetVisibility` (`/Game/Blueprints/Interfaces/WeaponsRoom/FlareInterfaceWidget.Flooding` _flaredisplaywidget) "Hidden")
    (`Widget.SetVisibility` (`/Game/Blueprints/Interfaces/WeaponsRoom/FlareInterfaceWidget.Ready` _flaredisplaywidget) "Visible")
    (else
      (`/Game/Blueprints/Interfaces/AlertLight.AlertFlash` (`self.AlertLight`)))))

(event `self.ButtonReleased`
  (`parent.ButtonReleased`)
  (`SceneComponent.K2_SetRelativeLocation` (`self.ButtonCollision`) (0.0 0.0 0.0) false false)
  (`GameplayStatics.PlaySoundAtLocation` "/Game/SFX/ButtonReleaseCue.ButtonReleaseCue" (`SceneComponent.K2_GetComponentLocation` (`self.DefaultSceneRoot`)) (struct) 1.0 1.0 0.0 null null null))

(fn `UserConstructionScript`
  (`parent.UserConstructionScript`))