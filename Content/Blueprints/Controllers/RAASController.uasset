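; RAAS controller, the submarine's voice alert system that warns the player of hazards and announces depth milestones.
; After the tutorial, Tick checks CO2, oxygen, sonar, hull integrity and depth, while a timeline checks imminent collisions.
; Checks feed an AlertsQueue, mostly gated by DoOnce, which plays one line at a time as audio or mapped subtitled dialogue.
; It also triggers the hull alarm, saves at certain depths and offers direct playback for tutorial lines.
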(event `self.ReceiveBeginPlay`
  (bind _alertsqueue (`self.AlertsQueue`))
  ;[1 1 1] Setup and collision check
  (`self.AssociateSubtitles`)
  (`Timeline|CollisionCheckTimeline`
    (:`CheckEvent`
      (if (`/Game/Blueprints/Controllers/DialogueController.IsTutorialDone` (`self.DialogueController`))
        (bind _collisionimminent_ (`/Game/Blueprints/NavigationSupport/SubMarker.ImminentCollisionCheck` (`self.SubMarker`)))
        (if _collisionimminent_
          (switch `int` (`KismetMathLibrary.RandomIntegerInRange` 0 1)
            (:`Default`
              (`KismetArrayLibrary.Array_Add` _alertsqueue "/Game/VO/Placeholder/RAASVO/RAASCollisionCourse1.RAASCollisionCourse1" :!label _label))
            (:`0`
              (goto _label))
            (:`1`
              (`KismetArrayLibrary.Array_Add` _alertsqueue "/Game/VO/Placeholder/RAASVO/RAASCollisionCourse2.RAASCollisionCourse2"))))))))

(event `CO2Check`
  (bind _alertsqueue (`self.AlertsQueue`))
  ;[1 1 1] CO2 Check
  (if (> (`/Game/Blueprints/Interfaces/LifeSupportRoom/CO2ScrubberInterface.CO2Composition` (`self.CO2Scrubber`)) 350.0)
    (`/Engine/EditorBlueprintResources/StandardMacros.DoOnce` false :!label _label_2
      (:`Completed`
        (switch `int` (`KismetMathLibrary.RandomIntegerInRange` 0 1)
          (:`Default`
            (`KismetArrayLibrary.Array_Add` _alertsqueue "/Game/VO/Placeholder/RAASVO/RAASCarbonDioxideLevelsDangerous.RAASCarbonDioxideLevelsDangerous" :!label _label_3))
          (:`0`
            (goto _label_3))
          (:`1`
            (`KismetArrayLibrary.Array_Add` _alertsqueue "/Game/VO/Placeholder/RAASVO/RAASCarbonDioxideLevelsDangerous2.RAASCarbonDioxideLevelsDangerous2")))))
    (else
      (goto _label_2 :!via `Reset`))))

(event `self.ReceiveTick`
  (params (DeltaSeconds :type "Float (single-precision)"))
  ;[1 1 1] Tick loop
  (bind _aspressure_game_instance (cast `/Game/FirstPersonBP/Blueprints/PressureGameInstance` (`GameplayStatics.GetGameInstance`)))
  (set `self.ShowSubtitles?` (`/Game/FirstPersonBP/Blueprints/PressureGameInstance.ShowSubtitles` _aspressure_game_instance))
  (if (`/Game/Blueprints/Controllers/DialogueController.IsTutorialDone` (`self.DialogueController`))
    (`self.CO2Check`)
    (`self.OxygenCheck`)
    (`self.SonarCheck`)
    (`self.HullIntegrityCheck`)
    (`self.DepthCheck`)
    (`self.PlayLines`)))

(event `OxygenCheck`
  (bind _alertsqueue (`self.AlertsQueue`))
  ;[1 1 1] Oxygen Check
  (if (< (`/Game/Blueprints/Interfaces/LifeSupportRoom/OxygenSupplyInterface.OxygenLevel` (`self.OxygenInterface`)) 50.0)
    (`/Engine/EditorBlueprintResources/StandardMacros.DoOnce` false :!label _label_4
      (:`Completed`
        (switch `int` (`KismetMathLibrary.RandomIntegerInRange` 0 1)
          (:`Default`
            (`KismetArrayLibrary.Array_Add` _alertsqueue "/Game/VO/Placeholder/RAASVO/RAASOxygenLevelsDangerous.RAASOxygenLevelsDangerous" :!label _label_5))
          (:`0`
            (goto _label_5))
          (:`1`
            (`KismetArrayLibrary.Array_Add` _alertsqueue "/Game/VO/Placeholder/RAASVO/RAASOxygenLevelsDangerous2.RAASOxygenLevelsDangerous2")))))
    (else
      (goto _label_4 :!via `Reset`))))

(event `PlayLines`
  (bind _alertsqueue (`self.AlertsQueue`))
  (bind _audio (`self.Audio`))
  (bind _output (`|GetArrayItem` _alertsqueue))
  ;[1 1 1] Play currently queued sound line, if nothing is being played
  (if (and (not (`AudioComponent.IsPlaying` _audio)) (> (`KismetArrayLibrary.Array_Length` _alertsqueue) 0) (not (`KismetSystemLibrary.IsValid` (stale _returnvalue))))
    (if (`self.ShowSubtitles?`)
      (bind _returnvalue (`GameplayStatics.SpawnDialogueAttached` (`BlueprintMapLibrary.Map_Find` (`self.AssociatedSubtitles`) _output) (`self.RAASToPlayer`) _audio "None" (0.0 0.0 0.0) (struct) "KeepRelativeOffset" false 1.0 1.0 0.0 null))
      (else
        (`AudioComponent.SetSound` _audio _output)
        (`AudioComponent.Play` _audio 0.0)))
    (`KismetArrayLibrary.Array_Remove` _alertsqueue)))

(event `SonarCheck`
  (bind _sonarscreen (`self.SonarScreen`))
  ;[1 1 1] Sonar Check
  (if (and (`/Game/Blueprints/Interfaces/Interfaces_V1/SonarScreen.FrequenciesMatched?` _sonarscreen) (`/Game/Blueprints/Interfaces/Interfaces_V1/SonarScreen.MonsterBlipIsActive?` _sonarscreen))
    (`/Engine/EditorBlueprintResources/StandardMacros.DoOnce` false :!label _label_6
      (:`Completed`
        (`KismetArrayLibrary.Array_Add` (`self.AlertsQueue`) "/Game/VO/Placeholder/RAASVO/RAASUnidentifiedSonarContact.RAASUnidentifiedSonarContact")))
    (elif (not (`/Game/Blueprints/Controllers/MonsterController.MonsterPresent?` (`/Game/Blueprints/Interfaces/Interfaces_V1/SonarScreen.MonsterController` _sonarscreen)))
      (goto _label_6 :!via `Reset`))))

(event `PlayLineTutorial`
  (params (Line :type "SoundBase Object Reference"))
  (bind _audio (`self.Audio`))
  ;[1 1 1] Event to force play dialogue for tutorial
  (`AudioComponent.SetSound` _audio Line)
  (`AudioComponent.Play` _audio 0.0))

(event `PlayLineSubtitledTutorial`
  (params (Dialogue :type "DialogueWave Object Reference") (Context :type "DialogueContext Structure"))
  ;[1 1 1] Event to force play dialogue with subtitles for tutorial
  (`GameplayStatics.SpawnDialogueAttached` Dialogue Context (`self.Audio`) "None" (0.0 0.0 0.0) (struct) "KeepRelativeOffset" false 1.0 1.0 0.0 null))

(event `HullIntegrityCheck`
  (bind _hullintegrity (`/Game/Blueprints/Controllers/SystemsController.HullIntegrity` (`self.SystemsController`)))
  ;[1 1 1] Hull Integrity check
  (if (<= _hullintegrity 0)
    (`|DoOnceMultiInput` :!label _label_7
      (:`A Out`
        (`KismetArrayLibrary.Array_Add` (`self.AlertsQueue`) "/Game/VO/Placeholder/RAASVO/RAASHullCollapseCountdown.RAASHullCollapseCountdown"))
      (:`Reset Out`
        (if (== (`AudioComponent.Sound` (`self.Audio`)) "/Game/VO/Placeholder/RAASVO/RAASHullCollapseCountdown.RAASHullCollapseCountdown")
          (`self.StopCurrentLine`))
        (if (<= _hullintegrity 20)
          (`|DoOnceMultiInput` :!label _label_8
            (:`A Out`
              (`KismetArrayLibrary.Array_Add` (`self.AlertsQueue`) "/Game/VO/Placeholder/RAASVO/RAASHullIntegrity20_.RAASHullIntegrity20_")
              (`KismetSystemLibrary.Delay` 5.0)
              (`AudioComponent.Play` (`self.AlarmAudio`) 0.0))
            (:`Reset Out`
              (`AudioComponent.Stop` (`self.AlarmAudio`))
              (if (<= _hullintegrity 50)
                (`/Engine/EditorBlueprintResources/StandardMacros.DoOnce` false :!label _label_9
                  (:`Completed`
                    (`KismetArrayLibrary.Array_Add` (`self.AlertsQueue`) "/Game/VO/Placeholder/RAASVO/RAASHullIntegrity50_.RAASHullIntegrity50_")))
                (else
                  (goto _label_9 :!via `Reset`)))))
          (else
            (goto _label_8 :!via `Reset In`)))))
    (else
      (goto _label_7 :!via `Reset In`))))

(event `StopCurrentLine`
  (bind _audio (`self.Audio`))
  ;[1 1 1] Stop current RAAS line and move on to next if applicible
  (`AudioComponent.Stop` _audio)
  (`AudioComponent.SetSound` _audio "/Game/SFX/SmallPipeFitSub.SmallPipeFitSub")
  (`KismetSystemLibrary.PrintString` "ssHello"))

(event `DepthCheck`
  (bind _alertsqueue (`self.AlertsQueue`))
  (bind _savegamecontroller (`self.SaveGameController`))
  (bind _returnvalue (`KismetMathLibrary.Round` (`/Game/Blueprints/Controllers/SystemsController.Depth` (`self.SystemsController`))))
  ;[1 1 1] Depth check
  (if (and (== (mod _returnvalue 100) 0) (< _returnvalue (`self.PrevDepthThreshold`)))
    (set `self.PrevDepthThreshold` _returnvalue)
    (switch `int` (/ _returnvalue 100)
      (:`0`
        (`KismetSystemLibrary.PrintString` "raas did something wrong lol"))
      (:`1`
        (`KismetArrayLibrary.Array_Add` _alertsqueue "/Game/VO/Placeholder/RAASVO/RAAS100Meters.RAAS100Meters")
        (`KismetArrayLibrary.Array_Add` _alertsqueue "/Game/VO/Placeholder/RAASVO/RAASChangeSonarFrequencyDisk.RAASChangeSonarFrequencyDisk"))
      (:`2`
        (`KismetArrayLibrary.Array_Add` _alertsqueue "/Game/VO/Placeholder/RAASVO/RAAS200Meters.RAAS200Meters")
        (`KismetArrayLibrary.Array_Add` _alertsqueue "/Game/VO/Placeholder/RAASVO/RAASChangeSonarFrequencyDisk.RAASChangeSonarFrequencyDisk")
        (`/Game/Blueprints/Controllers/SaveGameController.SaveGame` _savegamecontroller))
      (:`3`
        (`KismetArrayLibrary.Array_Add` _alertsqueue "/Game/VO/Placeholder/RAASVO/RAAS300Meters.RAAS300Meters"))
      (:`4`
        (`KismetArrayLibrary.Array_Add` _alertsqueue "/Game/VO/Placeholder/RAASVO/RAAS400Meters.RAAS400Meters")
        (`KismetArrayLibrary.Array_Add` _alertsqueue "/Game/VO/Placeholder/RAASVO/RAASChangeSonarFrequencyDisk.RAASChangeSonarFrequencyDisk")
        (`/Game/Blueprints/Controllers/SaveGameController.SaveGame` _savegamecontroller))
      (:`5`
        (`KismetArrayLibrary.Array_Add` _alertsqueue "/Game/VO/Placeholder/RAASVO/RAAS500Meters.RAAS500Meters"))
      (:`6`
        (`KismetArrayLibrary.Array_Add` _alertsqueue "/Game/VO/Placeholder/RAASVO/RAAS600Meters.RAAS600Meters")
        (`KismetArrayLibrary.Array_Add` _alertsqueue "/Game/VO/Placeholder/RAASVO/RAASChangeSonarFrequencyDisk.RAASChangeSonarFrequencyDisk")
        (`/Game/Blueprints/Controllers/SaveGameController.SaveGame` _savegamecontroller))
      (:`7`
        (`KismetArrayLibrary.Array_Add` _alertsqueue "/Game/VO/Placeholder/RAASVO/RAAS700Meters.RAAS700Meters"))
      (:`8`
        (`KismetArrayLibrary.Array_Add` _alertsqueue "/Game/VO/Placeholder/RAASVO/RAAS800Meters.RAAS800Meters")
        (`KismetArrayLibrary.Array_Add` _alertsqueue "/Game/VO/Placeholder/RAASVO/RAASChangeSonarFrequencyDisk.RAASChangeSonarFrequencyDisk")
        (`/Game/Blueprints/Controllers/SaveGameController.SaveGame` _savegamecontroller))
      (:`9`
        (`KismetArrayLibrary.Array_Add` _alertsqueue "/Game/VO/Placeholder/RAASVO/RAAS900Meters.RAAS900Meters")))))

(fn `AssociateSubtitles`
  (bind _associatedsubtitles (`self.AssociatedSubtitles`))
  (bind _associatedsubtitles_2 (`self.AssociatedSubtitles`))
  (bind _associatedsubtitles_3 (`self.AssociatedSubtitles`))
  (bind _associatedsubtitles_4 (`self.AssociatedSubtitles`))
  (bind _associatedsubtitles_5 (`self.AssociatedSubtitles`))
  (bind _associatedsubtitles_6 (`self.AssociatedSubtitles`))
  (bind _associatedsubtitles_7 (`self.AssociatedSubtitles`))
  (`BlueprintMapLibrary.Map_Add` _associatedsubtitles_4 "/Game/VO/Placeholder/RAASVO/RAAS100Meters.RAAS100Meters" "/Game/VO/Placeholder/RAASVO/RAAS100Meters_Dialogue.RAAS100Meters_Dialogue")
  (`BlueprintMapLibrary.Map_Add` _associatedsubtitles_4 "/Game/VO/Placeholder/RAASVO/RAAS200Meters.RAAS200Meters" "/Game/VO/Placeholder/RAASVO/RAAS200Meters_Dialogue.RAAS200Meters_Dialogue")
  (`BlueprintMapLibrary.Map_Add` _associatedsubtitles_4 "/Game/VO/Placeholder/RAASVO/RAAS300Meters.RAAS300Meters" "/Game/VO/Placeholder/RAASVO/RAAS300Meters_Dialogue.RAAS300Meters_Dialogue")
  (`BlueprintMapLibrary.Map_Add` _associatedsubtitles_5 "/Game/VO/Placeholder/RAASVO/RAAS400Meters.RAAS400Meters" "/Game/VO/Placeholder/RAASVO/RAAS400Meters_Dialogue.RAAS400Meters_Dialogue")
  (`BlueprintMapLibrary.Map_Add` _associatedsubtitles_5 "/Game/VO/Placeholder/RAASVO/RAAS500Meters.RAAS500Meters" "/Game/VO/Placeholder/RAASVO/RAAS500Meters_Dialogue.RAAS500Meters_Dialogue")
  (`BlueprintMapLibrary.Map_Add` _associatedsubtitles_5 "/Game/VO/Placeholder/RAASVO/RAAS600Meters.RAAS600Meters" "/Game/VO/Placeholder/RAASVO/RAAS600Meters_Dialogue.RAAS600Meters_Dialogue")
  (`BlueprintMapLibrary.Map_Add` _associatedsubtitles_6 "/Game/VO/Placeholder/RAASVO/RAAS700Meters.RAAS700Meters" "/Game/VO/Placeholder/RAASVO/RAAS700Meters_Dialogue.RAAS700Meters_Dialogue")
  (`BlueprintMapLibrary.Map_Add` _associatedsubtitles_6 "/Game/VO/Placeholder/RAASVO/RAAS800Meters.RAAS800Meters" "/Game/VO/Placeholder/RAASVO/RAAS800Meters_Dialogue.RAAS800Meters_Dialogue")
  (`BlueprintMapLibrary.Map_Add` _associatedsubtitles_6 "/Game/VO/Placeholder/RAASVO/RAAS900Meters.RAAS900Meters" "/Game/VO/Placeholder/RAASVO/RAAS900Meters_Dialogue.RAAS900Meters_Dialogue")
  (`BlueprintMapLibrary.Map_Add` _associatedsubtitles_7 "/Game/VO/Placeholder/RAASVO/RAASCarbonDioxideLevelsDangerous.RAASCarbonDioxideLevelsDangerous" "/Game/VO/Placeholder/RAASVO/RAASCarbonDioxideLevelsDangerous_Dialogue.RAASCarbonDioxideLevelsDangerous_Dialogue")
  (`BlueprintMapLibrary.Map_Add` _associatedsubtitles_7 "/Game/VO/Placeholder/RAASVO/RAASCarbonDioxideLevelsDangerous2.RAASCarbonDioxideLevelsDangerous2" "/Game/VO/Placeholder/RAASVO/RAASCarbonDioxideLevelsDangerous2_Dialogue.RAASCarbonDioxideLevelsDangerous2_Dialogue")
  (`BlueprintMapLibrary.Map_Add` _associatedsubtitles_7 "/Game/VO/Placeholder/RAASVO/RAASChangeSonarFrequencyDisk.RAASChangeSonarFrequencyDisk" "/Game/VO/Placeholder/RAASVO/RAASChangeSonarFrequencyDisk_Dialogue.RAASChangeSonarFrequencyDisk_Dialogue")
  (`BlueprintMapLibrary.Map_Add` _associatedsubtitles_2 "/Game/VO/Placeholder/RAASVO/RAASCollisionCourse1.RAASCollisionCourse1" "/Game/VO/Placeholder/RAASVO/RAASCollisionCourse1_Dialogue.RAASCollisionCourse1_Dialogue")
  (`BlueprintMapLibrary.Map_Add` _associatedsubtitles_2 "/Game/VO/Placeholder/RAASVO/RAASCollisionCourse2.RAASCollisionCourse2" "/Game/VO/Placeholder/RAASVO/RAASCollisionCourse2_Dialogue.RAASCollisionCourse2_Dialogue")
  (`BlueprintMapLibrary.Map_Add` _associatedsubtitles_2 "/Game/VO/Placeholder/RAASVO/RAASHullCollapseCountdown.RAASHullCollapseCountdown" "/Game/VO/Placeholder/RAASVO/RAASHullCollapseCountdown_Dialogue.RAASHullCollapseCountdown_Dialogue")
  (`BlueprintMapLibrary.Map_Add` _associatedsubtitles_3 "/Game/VO/Placeholder/RAASVO/RAASHullCollapseWarning.RAASHullCollapseWarning" "/Game/VO/Placeholder/RAASVO/RAASHullCollapseWarning_Dialogue.RAASHullCollapseWarning_Dialogue")
  (`BlueprintMapLibrary.Map_Add` _associatedsubtitles_3 "/Game/VO/Placeholder/RAASVO/RAASHullIntegrity20_.RAASHullIntegrity20_" "/Game/VO/Placeholder/RAASVO/RAASHullIntegrity20__Dialogue.RAASHullIntegrity20__Dialogue")
  (`BlueprintMapLibrary.Map_Add` _associatedsubtitles_3 "/Game/VO/Placeholder/RAASVO/RAASHullIntegrity50_.RAASHullIntegrity50_" "/Game/VO/Placeholder/RAASVO/RAASHullIntegrity50__Dialogue.RAASHullIntegrity50__Dialogue")
  (`BlueprintMapLibrary.Map_Add` _associatedsubtitles "/Game/VO/Placeholder/RAASVO/RAASOxygenLevelsDangerous.RAASOxygenLevelsDangerous" "/Game/VO/Placeholder/RAASVO/RAASOxygenLevelsDangerous_Dialogue.RAASOxygenLevelsDangerous_Dialogue")
  (`BlueprintMapLibrary.Map_Add` _associatedsubtitles "/Game/VO/Placeholder/RAASVO/RAASOxygenLevelsDangerous2.RAASOxygenLevelsDangerous2" "/Game/VO/Placeholder/RAASVO/RAASOxygenLevelsDangerous2_Dialogue.RAASOxygenLevelsDangerous2_Dialogue")
  (`BlueprintMapLibrary.Map_Add` _associatedsubtitles "/Game/VO/Placeholder/RAASVO/RAASUnidentifiedSonarContact.RAASUnidentifiedSonarContact" "/Game/VO/Placeholder/RAASVO/RAASUnidentifiedSonarContact_Dialogue.RAASUnidentifiedSonarContact_Dialogue"))

(fn `CheckCO2`
  (if (> (`/Game/Blueprints/Interfaces/LifeSupportRoom/CO2ScrubberInterface.CO2Composition` (`self.CO2Scrubber`)) 15.0)
    (`/Engine/EditorBlueprintResources/StandardMacros.DoOnce` false :!label _label
      (:`Completed`
        (`KismetArrayLibrary.Array_Add` (`self.AlertsQueue`) "/Game/VO/Placeholder/RAASVO/RAASCarbonDioxideLevelsDangerous.RAASCarbonDioxideLevelsDangerous")))
    (else
      (goto _label :!via `Reset`))))

(fn `UserConstructionScript`)