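; Saves and restores the submarine's state in a single "autosave" slot, covering ship systems, navigation, monster, doors, switches and items.
; SaveGame fills a PressureSaveGame through per-subsystem events, mostly using actor-keyed maps for world objects.
; LoadGame, also bound to X, replays these, re-seating items in receptacles, and queues a depth-based RAAS voice line.
; Loading resets player, usables and hazards; saved player location and flare draining states go unused.
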(event `SaveFlareLaunchers`
  (params (Save :type "/Game/Blueprints/PressureSaveGame Object Reference"))
  ;[1 1 1] Save Flare Launchers
  (bind _outactors (`GameplayStatics.GetAllActorsOfClass` "/Game/Blueprints/Interfaces/WeaponsRoom/FlareTube.FlareTube_C"))
  (for _array_element _outactors
    (`BlueprintMapLibrary.Map_Add` (`/Game/Blueprints/PressureSaveGame.FlareDoorsOpen?` Save) _array_element (`/Game/Blueprints/Interfaces/WeaponsRoom/FlareTube.IsOpen` _array_element)))
  (bind _outactors_2 (`GameplayStatics.GetAllActorsOfClass` "/Game/Blueprints/Interfaces/WeaponsRoom/FlareReceptacle.FlareReceptacle_C"))
  (for _array_element_2 _outactors_2
    (`BlueprintMapLibrary.Map_Add` (`/Game/Blueprints/PressureSaveGame.FlareLaunchersFlooded?` Save) _array_element_2 (`/Game/Blueprints/Interfaces/WeaponsRoom/FlareReceptacle.IsFlooded` _array_element_2))
    (`BlueprintMapLibrary.Map_Add` (`/Game/Blueprints/PressureSaveGame.FlareLaunchersDraining?` Save) _array_element_2 (`/Game/Blueprints/Interfaces/WeaponsRoom/FlareReceptacle.IsDraining` _array_element_2))))

(event `SaveSwitchStates`
  (params (Save :type "/Game/Blueprints/PressureSaveGame Object Reference"))
  ;[1 1 1] Save Switch States
  (bind _outactors (`GameplayStatics.GetAllActorsOfClass` "/Game/Blueprints/Interfaces/SwitchComponent.SwitchComponent_C"))
  (for _array_element _outactors
    (`BlueprintMapLibrary.Map_Add` (`/Game/Blueprints/PressureSaveGame.SwitchStates` Save) _array_element (`/Game/Blueprints/Interfaces/SwitchComponent.SwitchState` _array_element))))

(event `SaveEngineRoom`
  (params (Save :type "/Game/Blueprints/PressureSaveGame Object Reference"))
  (bind _systemscontroller (`self.SystemsController`))
  ;[1 1 1] Save Engine room
  (set `/Game/Blueprints/PressureSaveGame.BatteryPumpPercentages` (`/Game/Blueprints/Interfaces/EngineRoom/WaterDistributionInterface.PumpPercentages` (`/Game/Blueprints/Controllers/SystemsController.BatteryPump` _systemscontroller)) Save)
  (set `/Game/Blueprints/PressureSaveGame.WaterTankLevel` (`/Game/Blueprints/Interfaces/EngineRoom/WaterTank.WaterLevel` (`/Game/Blueprints/Controllers/SystemsController.WaterTank` _systemscontroller)) Save)
  (bind _outactors (`GameplayStatics.GetAllActorsOfClass` "/Game/Blueprints/Interfaces/EngineRoom/WaterBoiler.WaterBoiler_C"))
  (bind _output (`|GetArrayItem` _outactors))
  (set `/Game/Blueprints/PressureSaveGame.BoilerWaterLevel` (`/Game/Blueprints/Interfaces/EngineRoom/WaterBoiler.WaterLevel` _output) Save)
  (set `/Game/Blueprints/PressureSaveGame.BoilerSaltLevel` (`/Game/Blueprints/Interfaces/EngineRoom/WaterBoiler.SaltLevel` _output) Save)
  (set `/Game/Blueprints/PressureSaveGame.BoilerEvaporatedLevel` (`/Game/Blueprints/Interfaces/EngineRoom/WaterBoiler.EvaporatedWater` _output) Save)
  (bind _outactors_2 (`GameplayStatics.GetAllActorsOfClass` "/Game/Blueprints/Interfaces/EngineRoom/WaterTesting.WaterTesting_C"))
  (bind _output_2 (`|GetArrayItem` _outactors_2))
  (set `/Game/Blueprints/PressureSaveGame.TesterWaterLevel` (`/Game/Blueprints/Interfaces/EngineRoom/WaterTesting.WaterLevel` _output_2) Save)
  (set `/Game/Blueprints/PressureSaveGame.TesterPurityPercentage` (`/Game/Blueprints/Interfaces/EngineRoom/WaterTesting.PurityPercent` _output_2) Save)
  (set `/Game/Blueprints/PressureSaveGame.TesterKleinPercents` (`/Game/Blueprints/Interfaces/EngineRoom/WaterTesting.KleinPercents` _output_2) Save)
  (set `/Game/Blueprints/PressureSaveGame.TesterOrganicPercents` (`/Game/Blueprints/Interfaces/EngineRoom/WaterTesting.OrganicPercents` _output_2) Save))

(event `SaveNotchedTurnables`
  (params (Save :type "/Game/Blueprints/PressureSaveGame Object Reference"))
  ;[1 1 1] Save Notched Turnable States
  (bind _outactors (`GameplayStatics.GetAllActorsOfClass` "/Game/Blueprints/Interfaces/NotchedTurnableComponent.NotchedTurnableComponent_C"))
  (for _array_element _outactors
    (`BlueprintMapLibrary.Map_Add` (`/Game/Blueprints/PressureSaveGame.NotchedTurnableStates` Save) _array_element (`/Game/Blueprints/Interfaces/NotchedTurnableComponent.CurrentNotchPosition` _array_element))))

(event `SaveSystemControllerVars`
  (params (Save :type "/Game/Blueprints/PressureSaveGame Object Reference"))
  ;[1 1 1] Save system controller variables
  (set `/Game/Blueprints/PressureSaveGame.Depth` (`/Game/Blueprints/Controllers/SystemsController.Depth` (`self.SystemsController`)) Save))

(event `SaveMonsterController`
  (params (Save :type "/Game/Blueprints/PressureSaveGame Object Reference"))
  (bind _monstercontroller (`self.MonsterController`))
  ;[1 1 1] Monster Controller vars
  (set `/Game/Blueprints/PressureSaveGame.IsMonsterPresent?` (`/Game/Blueprints/Controllers/MonsterController.MonsterPresent?` _monstercontroller) Save)
  (set `/Game/Blueprints/PressureSaveGame.MonsterCoords` (`KismetMathLibrary.MakeVector2D` (`/Game/Blueprints/Controllers/MonsterController.MonsterX` _monstercontroller) (`/Game/Blueprints/Controllers/MonsterController.MonsterY` _monstercontroller)) Save)
  (set `/Game/Blueprints/PressureSaveGame.MonsterState` (`/Game/Blueprints/Controllers/MonsterController.AIState` _monstercontroller) Save)
  (set `/Game/Blueprints/PressureSaveGame.MonsterLoiterPointsVisted` (`/Game/Blueprints/Controllers/MonsterController.LoiterPointsVisited` _monstercontroller) Save)
  (set `/Game/Blueprints/PressureSaveGame.LeftFlareCoords` (`/Game/Blueprints/Controllers/MonsterController.LeftFlareLoc` _monstercontroller) Save)
  (set `/Game/Blueprints/PressureSaveGame.RightFlareCoords` (`/Game/Blueprints/Controllers/MonsterController.RightFlareLoc` _monstercontroller) Save))

(event `SaveDoorStates`
  (params (Save :type "/Game/Blueprints/PressureSaveGame Object Reference"))
  ;[1 1 1] Save Door States
  (bind _outactors (`GameplayStatics.GetAllActorsOfClass` "/Game/Blueprints/EnvironmentalActors/Door.Door_C"))
  (for _array_element _outactors
    (`BlueprintMapLibrary.Map_Add` (`/Game/Blueprints/PressureSaveGame.DoorStates` Save) _array_element (`/Game/Blueprints/EnvironmentalActors/Door.DoorOpen?` _array_element))))

(event `SaveItemLocations`
  (params (Save :type "/Game/Blueprints/PressureSaveGame Object Reference"))
  ;[1 1 1] Save Item locations
  (`BlueprintMapLibrary.Map_Clear` (`/Game/Blueprints/PressureSaveGame.ItemTransforms` Save))
  (`BlueprintMapLibrary.Map_Clear` (`/Game/Blueprints/PressureSaveGame.ItemsToReceptacles` Save))
  (bind _outactors (`GameplayStatics.GetAllActorsOfClass` "/Game/Blueprints/Items/Item.Item_C"))
  (for _array_element _outactors
    (if (`/Game/Blueprints/Items/Item.IsInReceptacle` _array_element)
      (`BlueprintMapLibrary.Map_Add` (`/Game/Blueprints/PressureSaveGame.ItemsToReceptacles` Save) _array_element (`/Game/Blueprints/Items/Item.MostRecentReceptacle` _array_element))
      (else
        (bind _staticmesh (`/Game/Blueprints/Items/Item.StaticMesh` _array_element))
        (`BlueprintMapLibrary.Map_Add` (`/Game/Blueprints/PressureSaveGame.ItemTransforms` Save) _array_element (`KismetMathLibrary.MakeTransform` (`SceneComponent.K2_GetComponentLocation` _staticmesh) (`SceneComponent.K2_GetComponentRotation` _staticmesh)))))))

(event `SavePlayerLocation`
  (params (Save :type "/Game/Blueprints/PressureSaveGame Object Reference"))
  (bind _capsulecomponent (`Character.CapsuleComponent` (`self.PlayerCharacter`)))
  ;[1 1 1] Save Player location (unused)
  (set `/Game/Blueprints/PressureSaveGame.PlayerLocation` (`SceneComponent.K2_GetComponentLocation` _capsulecomponent) Save)
  (set `/Game/Blueprints/PressureSaveGame.PlayerCapsuleRotation` (`SceneComponent.K2_GetComponentRotation` _capsulecomponent) Save))

(event `SaveLifeSupport`
  (params (Save :type "/Game/Blueprints/PressureSaveGame Object Reference"))
  (bind _systemscontroller (`self.SystemsController`))
  (bind _co2scrubber (`/Game/Blueprints/Controllers/SystemsController.CO2Scrubber` _systemscontroller))
  ;[1 1 1] Save life support room
  (set `/Game/Blueprints/PressureSaveGame.OxygenLevel` (`/Game/Blueprints/Interfaces/LifeSupportRoom/OxygenSupplyInterface.OxygenLevel` (`/Game/Blueprints/Controllers/SystemsController.OxygenSystem` _systemscontroller)) Save)
  (set `/Game/Blueprints/PressureSaveGame.CO2Level` (`/Game/Blueprints/Interfaces/LifeSupportRoom/CO2ScrubberInterface.CO2Composition` _co2scrubber) Save)
  (set `/Game/Blueprints/PressureSaveGame.FilterEfficiency` (`/Game/Blueprints/Interfaces/LifeSupportRoom/CO2ScrubberInterface.FilterEfficiency` _co2scrubber) Save)
  (set `/Game/Blueprints/PressureSaveGame.Co2ScrubberBroken?` (`/Game/Blueprints/Interfaces/LifeSupportRoom/CO2ScrubberInterface.IsBroken?` _co2scrubber) Save))

(event `SaveNavigationInstruments`
  (params (Save :type "/Game/Blueprints/PressureSaveGame Object Reference"))
  ;[1 1 1] Save Navigation Instrument Positions
  (bind _outactors (`GameplayStatics.GetAllActorsOfClass` "/Game/Blueprints/Interfaces/Bridge/NavigationThrottle.NavigationThrottle_C"))
  (set `/Game/Blueprints/PressureSaveGame.ThrottleDeltaY` (`/Game/Blueprints/Interfaces/SliderComponent.DeltaY` (`|GetArrayItem` _outactors)) Save)
  (bind _outactors_2 (`GameplayStatics.GetAllActorsOfClass` "/Game/Blueprints/Interfaces/Bridge/NavigationWheel.NavigationWheel_C"))
  (set `/Game/Blueprints/PressureSaveGame.NavigationWheelDeltaRot` (`/Game/Blueprints/Interfaces/TurnableComponent.DeltaRot` (`|GetArrayItem` _outactors_2)) Save))

(event `SaveNavigationMarkers`
  (params (Save :type "/Game/Blueprints/PressureSaveGame Object Reference"))
  (bind _staticmesh (`/Game/Blueprints/NavigationSupport/SubMarker.StaticMesh` (`self.SubMarker`)))
  ;[1 1 1] Save Navigation Markers
  (set `/Game/Blueprints/PressureSaveGame.SubMarkerLocation` (`SceneComponent.K2_GetComponentLocation` _staticmesh) Save)
  (set `/Game/Blueprints/PressureSaveGame.SubMarkerRotation` (`SceneComponent.K2_GetComponentRotation` _staticmesh) Save)
  (bind _outactors (`GameplayStatics.GetAllActorsOfClass` "/Game/Blueprints/NavigationSupport/RockMarker.RockMarker_C"))
  (for _array_element _outactors
    (`BlueprintMapLibrary.Map_Add` (`/Game/Blueprints/PressureSaveGame.RockLocations` Save) _array_element (`SceneComponent.K2_GetComponentLocation` (`/Game/Blueprints/NavigationSupport/RockMarker.StaticMesh` _array_element)))))

(event `SaveSonarRoom`
  (params (Save :type "/Game/Blueprints/PressureSaveGame Object Reference"))
  ;[1 1 1] Save Sonar Room
  (bind _outactors (`GameplayStatics.GetAllActorsOfClass` "/Game/Blueprints/Interfaces/SonarRoom/FrequencyDial.FrequencyDial_C"))
  (for (_array_element _array_index) _outactors
    (`KismetArrayLibrary.Array_Set` (`/Game/Blueprints/PressureSaveGame.FrequencyChangerDeltaRots` Save) _array_index (`/Game/Blueprints/Interfaces/TurnableComponent.DeltaRot` _array_element)))
  (set `/Game/Blueprints/PressureSaveGame.FreqWiresConnected?` (`/Game/Blueprints/Interfaces/SonarRoom/WireBoxInterface.AllConnected?` (`/Game/Blueprints/Controllers/SystemsController.WireBox` (`self.SystemsController`))) Save))

(event `SaveGame`
  ;[1 1 1] Save
  (bind _returnvalue (`|CreateWidget` "/Game/Widgets/SaveLogoWidget.SaveLogoWidget_C" (`GameplayStatics.GetPlayerController` 0)))
  (`UserWidget.AddToViewport` _returnvalue 0)
  (bind _returnvalue_2 (`GameplayStatics.CreateSaveGameObject` "/Game/Blueprints/PressureSaveGame.PressureSaveGame_C"))
  (`self.SaveNavigationMarkers` _returnvalue_2)
  (`self.SaveNavigationInstruments` _returnvalue_2)
  (`self.SavePlayerLocation` _returnvalue_2)
  (`self.SaveMonsterController` _returnvalue_2)
  (`self.SaveEngineRoom` _returnvalue_2)
  (`self.SaveSonarRoom` _returnvalue_2)
  (`self.SaveLifeSupport` _returnvalue_2)
  (`self.SaveItemLocations` _returnvalue_2)
  (`self.SaveSystemControllerVars` _returnvalue_2)
  (`self.SaveFlareLaunchers` _returnvalue_2)
  (`self.SaveSwitchStates` _returnvalue_2)
  (`self.SaveNotchedTurnables` _returnvalue_2)
  (`self.SaveDoorStates` _returnvalue_2)
  (bind _returnvalue_3 (`GameplayStatics.SaveGameToSlot` _returnvalue_2 "autosave"))
  (if _returnvalue_3
    (`KismetSystemLibrary.PrintString` "saved")
    (else
      (`KismetSystemLibrary.PrintString` "save failed for some reason"))))

(event `RAASVoiceLine`
  (params (Save :type "/Game/Blueprints/PressureSaveGame Object Reference"))
  (bind _alertsqueue (`/Game/Blueprints/Controllers/RAASController.AlertsQueue` (`self.RAASController`)))
  ;[1 1 1] RAAS Voice Line upon loading
  (switch `int` (/ (`KismetMathLibrary.Round` (`/Game/Blueprints/PressureSaveGame.Depth` Save)) 200)
    (:`1`
      (`KismetArrayLibrary.Array_Add` _alertsqueue "/Game/VO/Placeholder/RAASVO/RAAS200Meters.RAAS200Meters"))
    (:`2`
      (`KismetArrayLibrary.Array_Add` _alertsqueue "/Game/VO/Placeholder/RAASVO/RAAS400Meters.RAAS400Meters"))
    (:`3`
      (`KismetArrayLibrary.Array_Add` _alertsqueue "/Game/VO/Placeholder/RAASVO/RAAS600Meters.RAAS600Meters"))
    (:`4`
      (`KismetArrayLibrary.Array_Add` _alertsqueue "/Game/VO/Placeholder/RAASVO/RAAS800Meters.RAAS800Meters"))))

(event `Key|Z`
  (params (Key :type "Key Structure")))

(event `LoadGame`
  ;[1 1 1] Load
  (bind _returnvalue (`GameplayStatics.DoesSaveGameExist` "autosave"))
  (if _returnvalue
    (bind _returnvalue_2 (`GameplayStatics.LoadGameFromSlot` "autosave"))
    (bind _aspressure_save_game (cast `/Game/Blueprints/PressureSaveGame` _returnvalue_2))
    (`self.ResetPlayer`)
    (`self.LoadNavigationMarkers` _aspressure_save_game)
    (`self.LoadNavigationInstruments` _aspressure_save_game)
    (`self.LoadMonsterController` _aspressure_save_game)
    (`self.LoadEngineRoom` _aspressure_save_game)
    (`self.LoadLifeSupport` _aspressure_save_game)
    (`self.LoadSonar` _aspressure_save_game)
    (`self.LoadItemLocations` _aspressure_save_game)
    (`self.LoadSystemControllerVars` _aspressure_save_game)
    (`self.LoadFlareLaunchers` _aspressure_save_game)
    (`self.LoadSwitchStates` _aspressure_save_game)
    (`self.LoadNotchedTurnables` _aspressure_save_game)
    (`self.LoadDoorStates` _aspressure_save_game)
    (`self.ResetUsables`)
    (`self.ResetHazards`)
    (`self.RAASVoiceLine` _aspressure_save_game)
    (`KismetSystemLibrary.PrintString` "loaded")
    (else
      (`KismetSystemLibrary.PrintString` "no save game found!!"))))

(event `Key|X`
  (params (Key :type "Key Structure"))
  ;[1 1 1] Load
  (:`Pressed`
    (`self.LoadGame`)))

(event `LoadSwitchStates`
  (params (Save :type "/Game/Blueprints/PressureSaveGame Object Reference"))
  (bind _switchstates (`/Game/Blueprints/PressureSaveGame.SwitchStates` Save))
  ;[1 1 1] Load Switch States
  (bind _keys (`BlueprintMapLibrary.Map_Keys` _switchstates))
  (for _array_element _keys
    (if (!= (`/Game/Blueprints/Interfaces/SwitchComponent.SwitchState` _array_element) (`BlueprintMapLibrary.Map_Find` _switchstates _array_element))
      (`/Game/Blueprints/Interfaces/SwitchComponent.OnFlickSoundless` _array_element))))

(event `LoadSonar`
  (params (Save :type "/Game/Blueprints/PressureSaveGame Object Reference"))
  (bind _wirebox (`/Game/Blueprints/Controllers/SystemsController.WireBox` (`self.SystemsController`)))
  ;[1 1 1] Load Sonar
  (bind _outactors (`GameplayStatics.GetAllActorsOfClass` "/Game/Blueprints/Interfaces/SonarRoom/FrequencyDial.FrequencyDial_C"))
  (for (_array_element _array_index) _outactors
    (set `/Game/Blueprints/Interfaces/TurnableComponent.DeltaRot` (`|GetArrayItem` (`/Game/Blueprints/PressureSaveGame.FrequencyChangerDeltaRots` Save) _array_index) _array_element))
  (if (`/Game/Blueprints/PressureSaveGame.FreqWiresConnected?` Save)
    (`/Game/Blueprints/Interfaces/SonarRoom/WireBoxInterface.ResetWires` _wirebox)
    (else
      (`/Game/Blueprints/Interfaces/SonarRoom/WireBoxInterface.DropWires` _wirebox))))

(event `LoadNavigationMarkers`
  (params (Save :type "/Game/Blueprints/PressureSaveGame Object Reference"))
  (bind _staticmesh (`/Game/Blueprints/NavigationSupport/SubMarker.StaticMesh` (`self.SubMarker`)))
  ;[1 1 1] Load Navigation Markers
  (`SceneComponent.K2_SetWorldLocation` _staticmesh (`/Game/Blueprints/PressureSaveGame.SubMarkerLocation` Save) false false)
  (`SceneComponent.K2_SetWorldRotation` _staticmesh (`/Game/Blueprints/PressureSaveGame.SubMarkerRotation` Save) false false)
  (bind _outactors (`GameplayStatics.GetAllActorsOfClass` "/Game/Blueprints/NavigationSupport/RockMarker.RockMarker_C"))
  (for _array_element _outactors
    (`SceneComponent.K2_SetWorldLocation` (`/Game/Blueprints/NavigationSupport/RockMarker.StaticMesh` _array_element) (`BlueprintMapLibrary.Map_Find` (`/Game/Blueprints/PressureSaveGame.RockLocations` Save) _array_element) false false)))

(event `LoadNotchedTurnables`
  (params (Save :type "/Game/Blueprints/PressureSaveGame Object Reference"))
  (bind _notchedturnablestates (`/Game/Blueprints/PressureSaveGame.NotchedTurnableStates` Save))
  ;[1 1 1] load notched turnables
  (bind _keys (`BlueprintMapLibrary.Map_Keys` _notchedturnablestates))
  (for _array_element _keys
    (`/Game/Blueprints/Interfaces/NotchedTurnableComponent.SetNotchPosition` _array_element (`BlueprintMapLibrary.Map_Find` _notchedturnablestates _array_element))))

(event `LoadLifeSupport`
  (params (Save :type "/Game/Blueprints/PressureSaveGame Object Reference"))
  (bind _systemscontroller (`self.SystemsController`))
  (bind _co2scrubber (`/Game/Blueprints/Controllers/SystemsController.CO2Scrubber` _systemscontroller))
  (bind _repair_interface (`/Game/Blueprints/Interfaces/LifeSupportRoom/CO2ScrubberInterface.Repair Interface` _co2scrubber))
  ;[1 1 1] Load Life Support
  (set `/Game/Blueprints/Interfaces/LifeSupportRoom/OxygenSupplyInterface.OxygenLevel` (`/Game/Blueprints/PressureSaveGame.OxygenLevel` Save) (`/Game/Blueprints/Controllers/SystemsController.OxygenSystem` _systemscontroller))
  (set `/Game/Blueprints/Interfaces/LifeSupportRoom/CO2ScrubberInterface.CO2Composition` (`/Game/Blueprints/PressureSaveGame.CO2Level` Save) _co2scrubber)
  (set `/Game/Blueprints/Interfaces/LifeSupportRoom/CO2ScrubberInterface.FilterEfficiency` (`/Game/Blueprints/PressureSaveGame.FilterEfficiency` Save) _co2scrubber)
  (if (`/Game/Blueprints/PressureSaveGame.Co2ScrubberBroken?` Save)
    (`/Game/Blueprints/Interfaces/LifeSupportRoom/CO2ScrubberRepairInterface.BreakEvent` _repair_interface)
    (else
      (`/Game/Blueprints/Interfaces/LifeSupportRoom/CO2ScrubberRepairInterface.RepairComplete` _repair_interface)
      (`/Game/Blueprints/Interfaces/LifeSupportRoom/CO2ScrubberRepairInterface.CloseDoor` _repair_interface))))

(event `LoadNavigationInstruments`
  (params (Save :type "/Game/Blueprints/PressureSaveGame Object Reference"))
  ;[1 1 1] Load Navigation Instruments
  (bind _outactors (`GameplayStatics.GetAllActorsOfClass` "/Game/Blueprints/Interfaces/Bridge/NavigationThrottle.NavigationThrottle_C"))
  (`/Game/Blueprints/Interfaces/SliderComponent.SetHandleY` (`|GetArrayItem` _outactors) (`/Game/Blueprints/PressureSaveGame.ThrottleDeltaY` Save))
  (bind _outactors_2 (`GameplayStatics.GetAllActorsOfClass` "/Game/Blueprints/Interfaces/Bridge/NavigationWheel.NavigationWheel_C"))
  (`/Game/Blueprints/Interfaces/TurnableComponent.SetTurnableDeltaRot` (`|GetArrayItem` _outactors_2) (`/Game/Blueprints/PressureSaveGame.NavigationWheelDeltaRot` Save)))

(event `ResetPlayer`
  (bind _playercharacter (`self.PlayerCharacter`))
  ;[1 1 1] Reset Player
  (set `/Game/FirstPersonBP/Blueprints/FirstPersonCharacter.CurrentHealth` 100.0 _playercharacter)
  (if (not (`/Game/FirstPersonBP/Blueprints/FirstPersonCharacter.InterfaceUnlocked` _playercharacter))
    (`/Game/FirstPersonBP/Blueprints/FirstPersonCharacter.ExitInterface` _playercharacter))
  (if (`/Game/FirstPersonBP/Blueprints/FirstPersonCharacter.HoldingObject` _playercharacter)
    (`/Game/FirstPersonBP/Blueprints/FirstPersonCharacter.Release Object` _playercharacter))
  (if (`/Game/FirstPersonBP/Blueprints/FirstPersonCharacter.HoldingUsable` _playercharacter)
    (`/Game/FirstPersonBP/Blueprints/FirstPersonCharacter.DropUsable` _playercharacter))
  (`SceneComponent.K2_SetWorldLocationAndRotation` :`self` (`Character.CapsuleComponent` _playercharacter) :`NewLocation` (0.0 127.0 126.0))
  (`Controller.SetControlRotation` (`Pawn.GetController` _playercharacter) (`KismetMathLibrary.MakeRotator` 0.0 0.0 270.0)))

(event `LoadItemLocations`
  (params (Save :type "/Game/Blueprints/PressureSaveGame Object Reference"))
  (bind _itemtransforms (`/Game/Blueprints/PressureSaveGame.ItemTransforms` Save))
  (bind _itemstoreceptacles (`/Game/Blueprints/PressureSaveGame.ItemsToReceptacles` Save))
  ;[1 1 1] Load Item Locations
  (bind _keys (`BlueprintMapLibrary.Map_Keys` _itemtransforms))
  (for _array_element _keys
    (if (`/Game/Blueprints/Items/Item.IsInReceptacle` _array_element)
      (`/Game/Blueprints/Items/ItemReceptacle.ReleaseObject` (`/Game/Blueprints/Items/Item.MostRecentReceptacle` _array_element)))
    (`SceneComponent.K2_SetWorldLocationAndRotation` (`/Game/Blueprints/Items/Item.StaticMesh` _array_element) (.location (`BlueprintMapLibrary.Map_Find` _itemtransforms _array_element)) (.rotation (`BlueprintMapLibrary.Map_Find` _itemtransforms _array_element)) false false))
  (bind _keys_2 (`BlueprintMapLibrary.Map_Keys` _itemstoreceptacles))
  (for _array_element_2 _keys_2
    (bind _mostrecentreceptacle (`/Game/Blueprints/Items/Item.MostRecentReceptacle` _array_element_2))
    (if (and (!= _mostrecentreceptacle (`BlueprintMapLibrary.Map_Find` _itemstoreceptacles _array_element_2)) (`/Game/Blueprints/Items/Item.IsInReceptacle` _array_element_2))
      (`KismetSystemLibrary.PrintString` (`KismetSystemLibrary.GetDisplayName` _array_element_2) true true (struct :`R` 0.424815 :`G` 1.0 :`B` 0.476745 :`A` 1.0))
      (`/Game/Blueprints/Items/ItemReceptacle.ReleaseObject` _mostrecentreceptacle)
      (set `/Game/Blueprints/Items/Item.CanBePutInReceptacle` true _array_element_2)))
  (for _array_element_3 _keys_2
    (bind _value (`BlueprintMapLibrary.Map_Find` _itemstoreceptacles _array_element_3))
    (`/Game/Blueprints/Items/ItemReceptacle.GrabObject` _value _array_element_3 true)
    (if (== (`GameplayStatics.GetObjectClass` _value) "/Game/Blueprints/Items/PipeReceptacle.PipeReceptacle_C")
      (bind _aspipe_receptacle (cast `/Game/Blueprints/Items/PipeReceptacle` _value))
      (`/Game/Blueprints/Items/PipeReceptacle.StopWaterFlowOnIncomingConnections` _aspipe_receptacle))))

(event `LoadMonsterController`
  (params (Save :type "/Game/Blueprints/PressureSaveGame Object Reference"))
  (bind _monstercontroller (`self.MonsterController`))
  (bind (_x _y) (`KismetMathLibrary.BreakVector2D` (`/Game/Blueprints/PressureSaveGame.MonsterCoords` Save)))
  ;[1 1 1] Load Monster Controller
  (set `/Game/Blueprints/Controllers/MonsterController.MonsterPresent?` (`/Game/Blueprints/PressureSaveGame.IsMonsterPresent?` Save) _monstercontroller)
  (set `/Game/Blueprints/Controllers/MonsterController.MonsterX` _x _monstercontroller)
  (set `/Game/Blueprints/Controllers/MonsterController.MonsterY` _y _monstercontroller)
  (set `/Game/Blueprints/Controllers/MonsterController.AIState` (`/Game/Blueprints/PressureSaveGame.MonsterState` Save) _monstercontroller)
  (set `/Game/Blueprints/Controllers/MonsterController.LoiterPointsVisited` (`/Game/Blueprints/PressureSaveGame.MonsterLoiterPointsVisted` Save) _monstercontroller)
  (set `/Game/Blueprints/Controllers/MonsterController.LeftFlareLoc` (`/Game/Blueprints/PressureSaveGame.LeftFlareCoords` Save) _monstercontroller)
  (set `/Game/Blueprints/Controllers/MonsterController.RightFlareLoc` (`/Game/Blueprints/PressureSaveGame.RightFlareCoords` Save) _monstercontroller))

(event `ResetUsables`
  ;[1 1 1] Reset Usable
  (bind _outactors (`GameplayStatics.GetAllActorsOfClass` "/Game/Blueprints/Usables/UsableReceptacle.UsableReceptacle_C"))
  (bind _outactors_2 (`GameplayStatics.GetAllActorsOfClass` "/Game/Blueprints/Usables/Usable.Usable_C"))
  (for (_array_element _array_index) _outactors
    (`/Game/Blueprints/Usables/UsableReceptacle.GrabUsable` _array_element (`|GetArrayItem` _outactors_2 _array_index) true)))

(event `LoadDoorStates`
  (params (Save :type "/Game/Blueprints/PressureSaveGame Object Reference"))
  (bind _doorstates (`/Game/Blueprints/PressureSaveGame.DoorStates` Save))
  ;[1 1 1] Load Door States
  (bind _keys (`BlueprintMapLibrary.Map_Keys` _doorstates))
  (for _array_element _keys
    (if (not (not (xor (`/Game/Blueprints/EnvironmentalActors/Door.DoorOpen?` _array_element) (`BlueprintMapLibrary.Map_Find` _doorstates _array_element))))
      (`/Game/Blueprints/EnvironmentalActors/Door.ChangeState` _array_element))))

(event `LoadSystemControllerVars`
  (params (Save :type "/Game/Blueprints/PressureSaveGame Object Reference"))
  ;[1 1 1] Load System Variables
  (set `/Game/Blueprints/Controllers/SystemsController.Depth` (`/Game/Blueprints/PressureSaveGame.Depth` Save) (`self.SystemsController`)))

(event `LoadEngineRoom`
  (params (Save :type "/Game/Blueprints/PressureSaveGame Object Reference"))
  (bind _systemscontroller (`self.SystemsController`))
  ;[1 1 1] Load Engine Room
  (set `/Game/Blueprints/Interfaces/EngineRoom/WaterDistributionInterface.PumpPercentages` (`/Game/Blueprints/PressureSaveGame.BatteryPumpPercentages` Save) (`/Game/Blueprints/Controllers/SystemsController.BatteryPump` _systemscontroller))
  (set `/Game/Blueprints/Interfaces/EngineRoom/WaterTank.WaterLevel` (`/Game/Blueprints/PressureSaveGame.WaterTankLevel` Save) (`/Game/Blueprints/Controllers/SystemsController.WaterTank` _systemscontroller))
  (bind _outactors (`GameplayStatics.GetAllActorsOfClass` "/Game/Blueprints/Interfaces/EngineRoom/WaterBoiler.WaterBoiler_C"))
  (bind _output (`|GetArrayItem` _outactors))
  (set `/Game/Blueprints/Interfaces/EngineRoom/WaterBoiler.WaterLevel` (`/Game/Blueprints/PressureSaveGame.BoilerWaterLevel` Save) _output)
  (set `/Game/Blueprints/Interfaces/EngineRoom/WaterBoiler.SaltLevel` (`/Game/Blueprints/PressureSaveGame.BoilerSaltLevel` Save) _output)
  (set `/Game/Blueprints/Interfaces/EngineRoom/WaterBoiler.EvaporatedWater` (`/Game/Blueprints/PressureSaveGame.BoilerEvaporatedLevel` Save) _output)
  (bind _outactors_2 (`GameplayStatics.GetAllActorsOfClass` "/Game/Blueprints/Interfaces/EngineRoom/WaterTesting.WaterTesting_C"))
  (bind _output_2 (`|GetArrayItem` _outactors_2))
  (set `/Game/Blueprints/Interfaces/EngineRoom/WaterTesting.WaterLevel` (`/Game/Blueprints/PressureSaveGame.WaterTankLevel` Save) _output_2)
  (set `/Game/Blueprints/Interfaces/EngineRoom/WaterTesting.PurityPercent` (`/Game/Blueprints/PressureSaveGame.TesterPurityPercentage` Save) _output_2)
  (set `/Game/Blueprints/Interfaces/EngineRoom/WaterTesting.KleinPercents` (`/Game/Blueprints/PressureSaveGame.TesterKleinPercents` Save) _output_2)
  (set `/Game/Blueprints/Interfaces/EngineRoom/WaterTesting.OrganicPercents` (`/Game/Blueprints/PressureSaveGame.TesterOrganicPercents` Save) _output_2))

(event `LoadFlareLaunchers`
  (params (Save :type "/Game/Blueprints/PressureSaveGame Object Reference"))
  (bind _flarelaunchersflooded_ (`/Game/Blueprints/PressureSaveGame.FlareLaunchersFlooded?` Save))
  (bind _flaredoorsopen_ (`/Game/Blueprints/PressureSaveGame.FlareDoorsOpen?` Save))
  ;[1 1 1] Load flare launchers
  (bind _keys (`BlueprintMapLibrary.Map_Keys` _flaredoorsopen_))
  (for _array_element _keys
    (if (`BlueprintMapLibrary.Map_Find` _flaredoorsopen_ _array_element)
      (`/Game/Blueprints/Interfaces/WeaponsRoom/FlareTube.OpenDoor` _array_element)
      (else
        (`/Game/Blueprints/Interfaces/WeaponsRoom/FlareTube.CloseDoor` _array_element)))
    (bind _keys_2 (`BlueprintMapLibrary.Map_Keys` _flarelaunchersflooded_))
    (for _array_element_2 _keys_2
      (set `/Game/Blueprints/Interfaces/WeaponsRoom/FlareReceptacle.IsFlooded` (`BlueprintMapLibrary.Map_Find` _flarelaunchersflooded_ _array_element_2) _array_element_2))))

(event `ResetHazards`
  ;[1 1 1] Reset Hazards
  (bind _outactors (`GameplayStatics.GetAllActorsOfClass` "/Game/Blueprints/Hazards/Fire.Fire_C"))
  (for _array_element _outactors
    (`/Game/Blueprints/Hazards/Fire.ChangeIntensity` _array_element -100.0))
  (bind _outactors_2 (`GameplayStatics.GetAllActorsOfClass` "/Game/Blueprints/Hazards/HullBreach.HullBreach_C"))
  (for _array_element_2 _outactors_2
    (if (`/Game/Blueprints/Hazards/HullBreach.BreachActive?` _array_element_2)
      (`/Game/Blueprints/Hazards/HullBreach.PlugBreach` _array_element_2 true))))

(fn `UserConstructionScript`)