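; Controller for submarine impacts from rocks, monsters and scripted moments, handling sound, physics impulses, camera shake and damage.
; The main driver converts hit direction to an angle selecting a room handler, which picks affected rooms, breaks room-specific equipment and randomly causes hull breaches or fires.
; Shake intensifies, with a concussion widget, when the player's room is affected.
; Major hits also flicker lights red via a timeline, then restore recorded intensities.
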(event `RecordLightIntensities`
  ;[1 1 1] Record Light Intensities
  (bind _outactors (`GameplayStatics.GetAllActorsOfClassWithTag` "/Script/Engine.PointLight" "AffectedByImpact"))
  (for _array_element _outactors
    (bind _aspoint_light (cast `PointLight` _array_element))
    (bind _pointlightcomponent (`PointLight.PointLightComponent` _aspoint_light))
    (`BlueprintMapLibrary.Map_Add` (`self.LightIntensities`) _pointlightcomponent (`LightComponentBase.Intensity` _pointlightcomponent)))
  (bind _outactors_2 (`GameplayStatics.GetAllActorsOfClass` "/Game/Blueprints/EnvironmentalActors/HangingLight.HangingLight_C"))
  (for _array_element_2 _outactors_2
    (bind _pointlight (`/Game/Blueprints/EnvironmentalActors/HangingLight.PointLight` _array_element_2))
    (`BlueprintMapLibrary.Map_Add` (`self.LightIntensities`) _pointlight (`LightComponentBase.Intensity` _pointlight)))
  (bind _outactors_3 (`GameplayStatics.GetAllActorsOfClass` "/Game/Blueprints/EnvironmentalActors/CeilingLight.CeilingLight_C"))
  (for _array_element_3 _outactors_3
    (bind _pointlight_2 (`/Game/Blueprints/EnvironmentalActors/CeilingLight.PointLight` _array_element_3))
    (`BlueprintMapLibrary.Map_Add` (`self.LightIntensities`) _pointlight_2 (`LightComponentBase.Intensity` _pointlight_2)))
  (bind _outactors_4 (`GameplayStatics.GetAllActorsOfClass` "/Game/Blueprints/EnvironmentalActors/WallLight.WallLight_C"))
  (for _array_element_4 _outactors_4
    (bind _pointlight_3 (`/Game/Blueprints/EnvironmentalActors/WallLight.PointLight` _array_element_4))
    (`BlueprintMapLibrary.Map_Add` (`self.LightIntensities`) _pointlight_3 (`LightComponentBase.Intensity` _pointlight_3))))

(event `self.ReceiveBeginPlay`
  ;[1 1 1] Setup
  (bind _outactors (`GameplayStatics.GetAllActorsOfClassWithTag` "/Script/Engine.PointLight" "AffectedByImpact"))
  (for _array_element _outactors
    (bind _aspoint_light (cast `PointLight` _array_element))
    (bind _pointlightcomponent (`PointLight.PointLightComponent` _aspoint_light))
    (`KismetArrayLibrary.Array_Add` (`self.Lights`) _pointlightcomponent)
    (`BlueprintMapLibrary.Map_Add` (`self.LightIntensities`) _pointlightcomponent (`LightComponentBase.Intensity` _pointlightcomponent)))
  (bind _outactors_2 (`GameplayStatics.GetAllActorsOfClass` "/Game/Blueprints/EnvironmentalActors/HangingLight.HangingLight_C"))
  (for _array_element_2 _outactors_2
    (bind _pointlight (`/Game/Blueprints/EnvironmentalActors/HangingLight.PointLight` _array_element_2))
    (`KismetArrayLibrary.Array_Add` (`self.Lights`) _pointlight)
    (`BlueprintMapLibrary.Map_Add` (`self.LightIntensities`) _pointlight (`LightComponentBase.Intensity` _pointlight)))
  (bind _outactors_3 (`GameplayStatics.GetAllActorsOfClass` "/Game/Blueprints/EnvironmentalActors/CeilingLight.CeilingLight_C"))
  (for _array_element_3 _outactors_3
    (bind _pointlight_2 (`/Game/Blueprints/EnvironmentalActors/CeilingLight.PointLight` _array_element_3))
    (`KismetArrayLibrary.Array_Add` (`self.Lights`) _pointlight_2)
    (`BlueprintMapLibrary.Map_Add` (`self.LightIntensities`) _pointlight_2 (`LightComponentBase.Intensity` _pointlight_2)))
  (bind _outactors_4 (`GameplayStatics.GetAllActorsOfClass` "/Game/Blueprints/EnvironmentalActors/WallLight.WallLight_C"))
  (for _array_element_4 _outactors_4
    (bind _pointlight_3 (`/Game/Blueprints/EnvironmentalActors/WallLight.PointLight` _array_element_4))
    (`KismetArrayLibrary.Array_Add` (`self.Lights`) _pointlight_3)
    (`BlueprintMapLibrary.Map_Add` (`self.LightIntensities`) _pointlight_3 (`LightComponentBase.Intensity` _pointlight_3)))
  (`self.EnableInput` (`GameplayStatics.GetPlayerController` 0)))

(event `Key|N`
  (params (Key :type "Key Structure")))

(event `Key|M`
  (params (Key :type "Key Structure")))

(event `HitEventRock`
  (params (Direction :type "Vector Structure") (Strength :type "Float (double-precision)"))
  (`GameplayStatics.PlaySound2D` "/Game/SFX/RockImpactSub.RockImpactSub" 1.5 1.0 0.0 null null)
  (`self.HitEventDriver` Direction Strength))

(event `HitEventDriver`
  (params (Direction :type "Vector Structure") (Strength :type "Float (double-precision)"))
  (bind _returnvalue (* Direction (+ 12000.0 (* 6000 Strength))))
  ;[1 1 1] Hit Event
  (`self.ImpulseOnPhysicsObjects` _returnvalue)
  (bind _direction (`self.GetHitEventDirection` Direction))
  (if (or (> _direction 315.0) (< _direction 45.0))
    (`self.HitEventTorpedoRoom` Strength)
    (elif (< _direction 120.0)
      (`self.HitEventSonarRoom` Strength)
      (elif (< _direction 240.0)
        (`self.HitEventEngineRoom` _returnvalue Strength)
        (else
          (`self.HitEventLifeSupportRoom` Strength)))))
  (for _array_element (`self.Lights`) :!label _label
    (`LightComponent.SetLightColor` _array_element (struct :`R` 0.890196 :`B` 0.015686 :`A` 1.0) true))
  (`self.RecordLightIntensities`)
  (bind (_direction_2 _lightflicker) (`Timeline|LightFlickerTimeline` :!via `PlayFromStart`)
    (:`Update`
      (for _array_element_2 (`self.Lights`)
        (`LightComponent.SetIntensity` _array_element_2 (* _lightflicker (`BlueprintMapLibrary.Map_Find` (`self.LightIntensities`) _array_element_2)))))
    (:`Finished`
      (for _array_element_3 (`self.Lights`)
        (`LightComponent.SetLightColor` _array_element_3 (struct :`R` 0.991102 :`G` 0.775822 :`B` 0.48515 :`A` 1.0) true)
        (`LightComponent.SetIntensity` _array_element_3 (`BlueprintMapLibrary.Map_Find` (`self.LightIntensities`) _array_element_3))))))

(event `HitEventMonster`
  (params (Direction :type "Vector Structure") (Strength :type "Float (double-precision)"))
  (`GameplayStatics.PlaySound2D` "/Game/SFX/MediumImpactSub.MediumImpactSub" 0.5 0.85 0.2 null null)
  (`self.HitEventDriver` Direction Strength))

(event `PipesTutorial`
  (params (`Hit Vector` :type "Vector Structure") (Strength :type "Float (double-precision)"))
  ;[1 1 1] Hit Event
  ;;[1 1 1] Driver for the Pipes Tutorial collision
  (`GameplayStatics.PlaySound2D` "/Game/SFX/MediumImpactSub.MediumImpactSub" 0.5 0.85 0.2 null null)
  (`self.ImpulseOnPhysicsObjects` (* `Hit Vector` 4000.0) true)
  (`self.PipesTutorialHitEvent` `Hit Vector` Strength)
  (goto _label))

(event `HitEventWithoutBreakage`
  ;[1 1 1] Hit Event withut breakage (for scripted sequences
  (`GameplayStatics.PlaySound2D` "/Game/SFX/MediumImpactSub.MediumImpactSub" 0.5 0.85 0.2 null null)
  (`self.ImpulseOnPhysicsObjects` (1750.0 8000.0 0.0) true)
  (`PlayerController.ClientStartCameraShake` :`self` (`GameplayStatics.GetPlayerController` 0) :`Shake` "/Game/Blueprints/ImpactCameraShake.ImpactCameraShake_C")
  (goto _label))

(event `BumpEvent`
  ;[1 1 1] Smaller Bump
  (`GameplayStatics.PlaySound2D` "/Game/SFX/MediumHullBangCue.MediumHullBangCue" 1.0 1.0 0.0 null null)
  (`PlayerController.ClientStartCameraShake` :`self` (`GameplayStatics.GetPlayerController` 0) :`Shake` "/Game/Blueprints/ImpactCameraShake.ImpactCameraShake_C" :`Scale` 0.5))

(fn `CameraShake`
  (params (Strength :type "Float (double-precision)") (Rooms :type "Array of String"))
  (locals (`PlayerInAffectedRoom?` :type Boolean))
  (bind _returnvalue (`GameplayStatics.GetPlayerController` 0))
  (bind _returnvalue_2 (+ Strength 1.0))
  (bind _returnvalue_3 (* _returnvalue_2 1.2))
  (bind _asfirst_person_character (cast `/Game/FirstPersonBP/Blueprints/FirstPersonCharacter` (`GameplayStatics.GetPlayerCharacter` 0)))
  (for _array_element Rooms
    (if (`KismetStringLibrary.EqualEqual_StrStr` (`/Game/FirstPersonBP/Blueprints/FirstPersonCharacter.CurrentRoom` _asfirst_person_character) _array_element)
      (set `local.PlayerInAffectedRoom?` true)))
  (if (`local.PlayerInAffectedRoom?`)
    (`PlayerController.ClientStartCameraShake` :`self` _returnvalue :`Shake` "/Game/Blueprints/ImpactConcussionCamerashake.ImpactConcussionCameraShake_C" :`Scale` _returnvalue_3)
    (`PlayerController.ClientStartCameraShake` :`self` _returnvalue :`Shake` "/Game/Blueprints/ImpactCameraShake.ImpactCameraShake_C" :`Scale` (* _returnvalue_3 0.75))
    (bind _returnvalue_4 (`|CreateWidget` "/Game/Widgets/HitEventConcussionWidget.HitEventConcussionWidget_C" _returnvalue))
    (`UserWidget.AddToViewport` _returnvalue_4 0)
    (else
      (`PlayerController.ClientStartCameraShake` :`self` _returnvalue :`Shake` "/Game/Blueprints/ImpactCameraShake.ImpactCameraShake_C" :`Scale` _returnvalue_2))))

(fn `CreateFires`
  (params (Room :type Name) (Strength :type "Float (double-precision)"))
  (if (== Room "EngineRoom")
    (if (`KismetMathLibrary.RandomBool`)
      (bind _returnvalue (`|SpawnActorFromClass` "/Game/Blueprints/Hazards/Fire.Fire_C" (`KismetMathLibrary.MakeTransform` (`KismetMathLibrary.MakeVector` 210.0 (`KismetMathLibrary.RandomFloatInRange` 260.0 540.0) 50.0)) "Undefined" "OverrideRootScale" null null))
      (set `/Game/Blueprints/Hazards/Fire.Room` "EngineRoom" _returnvalue)
      (else
        (bind _returnvalue_2 (`|SpawnActorFromClass` "/Game/Blueprints/Hazards/Fire.Fire_C" (`KismetMathLibrary.MakeTransform` (`KismetMathLibrary.MakeVector` (`KismetMathLibrary.RandomFloatInRange` -100.0 100.0) -400.0 50.0)) "Undefined" "OverrideRootScale" null null))
        (set `/Game/Blueprints/Hazards/Fire.Room` "EngineRoom" _returnvalue_2)))
    (elif (== Room "LifeSupport")
      (bind _returnvalue_3 (`|SpawnActorFromClass` "/Game/Blueprints/Hazards/Fire.Fire_C" (`KismetMathLibrary.MakeTransform` (`KismetMathLibrary.MakeVector` 190.0 (`KismetMathLibrary.RandomFloatInRange` 1880.0 2060.0) 260.0)) "Undefined" "OverrideRootScale" null null))
      (set `/Game/Blueprints/Hazards/Fire.Room` "LifeSupport" _returnvalue_3)
      (elif (== Room "SonarRoom")
        (bind _returnvalue_4 (`|SpawnActorFromClass` "/Game/Blueprints/Hazards/Fire.Fire_C" (`KismetMathLibrary.MakeTransform` (`KismetMathLibrary.MakeVector` (`KismetMathLibrary.RandomFloatInRange` -250.0 -220.0) (`KismetMathLibrary.RandomFloatInRange` 1930.0 2080.0) 260.0)) "Undefined" "OverrideRootScale" null null))
        (set `/Game/Blueprints/Hazards/Fire.Room` "SonarRoom" _returnvalue_4)
        (elif (== Room "Mess")
          (bind _returnvalue_5 (`|SpawnActorFromClass` "/Game/Blueprints/Hazards/Fire.Fire_C" (`KismetMathLibrary.MakeTransform` (`KismetMathLibrary.MakeVector` (`KismetMathLibrary.RandomFloatInRange` -310.0 -170.0) (`KismetMathLibrary.RandomFloatInRange` 1170.0 1640.0) 260.0)) "Undefined" "OverrideRootScale" null null))
          (set `/Game/Blueprints/Hazards/Fire.Room` "Mess" _returnvalue_5)
          (elif (== Room "Bridge")
            (switch `int` (`KismetMathLibrary.RandomIntegerInRange` 0 2)
              (:`0`
                (bind _returnvalue_6 (`|SpawnActorFromClass` "/Game/Blueprints/Hazards/Fire.Fire_C" (`KismetMathLibrary.MakeTransform` (`KismetMathLibrary.MakeVector` -220.0 (`KismetMathLibrary.RandomFloatInRange` 2700.0 2950.0) 260.0)) "Undefined" "OverrideRootScale" null null)) ; sonar side
                (set `/Game/Blueprints/Hazards/Fire.Room` "Bridge" _returnvalue_6))
              (:`1`
                (bind _returnvalue_7 (`|SpawnActorFromClass` "/Game/Blueprints/Hazards/Fire.Fire_C" (`KismetMathLibrary.MakeTransform` (`KismetMathLibrary.MakeVector` (`KismetMathLibrary.RandomFloatInRange` -120.0 120.0) 3145.0 260.0)) "Undefined" "OverrideRootScale" null null)) ; nav side
                (set `/Game/Blueprints/Hazards/Fire.Room` "Bridge" _returnvalue_7))
              (:`2`
                (bind _returnvalue_8 (`|SpawnActorFromClass` "/Game/Blueprints/Hazards/Fire.Fire_C" (`KismetMathLibrary.MakeTransform` (`KismetMathLibrary.MakeVector` 220.0 (`KismetMathLibrary.RandomFloatInRange` 2700.0 2950.0) 260.0)) "Undefined" "OverrideRootScale" null null)) ; status display side
                (set `/Game/Blueprints/Hazards/Fire.Room` "Bridge" _returnvalue_8)))
            (elif (== Room "Quarters")
              (bind _returnvalue_9 (`|SpawnActorFromClass` "/Game/Blueprints/Hazards/Fire.Fire_C" (`KismetMathLibrary.MakeTransform` (`KismetMathLibrary.MakeVector` 260.0 (`KismetMathLibrary.RandomFloatInRange` 970.0 1485.0) 260.0)) "Undefined" "OverrideRootScale" null null))
              (set `/Game/Blueprints/Hazards/Fire.Room` "Quarters" _returnvalue_9)
              (elif (== Room "Torpedo")
                (bind _returnvalue_10 (`|SpawnActorFromClass` "/Game/Blueprints/Hazards/Fire.Fire_C" (`KismetMathLibrary.MakeTransform` (`KismetMathLibrary.MakeVector` (`KismetMathLibrary.RandomFloatInRange` -190.0 190.0) (`KismetMathLibrary.RandomFloatInRange` 3095.0 3235.0) -40.0)) "Undefined" "OverrideRootScale" null null))
                (set `/Game/Blueprints/Hazards/Fire.Room` "Torpedo" _returnvalue_10)
                (else
                  (`KismetSystemLibrary.PrintString` (`KismetStringLibrary.Concat_StrStr` "tried to create fire in nonexstient room " "" (`KismetStringLibrary.Conv_NameToString` Room)) true true (struct :`R` 1.0 :`G` 0.034501 :`A` 1.0) 5.0))))))))))

(fn `CreateHullBreaches`
  (params (Room :type Name) (Strength :type "Float (double-precision)"))
  (locals (BreachesToCause :type Integer))
  (bind _subdisplay (`self.SubDisplay`))
  (if (< Strength 0.2)
    (set `local.BreachesToCause` 0)
    (elif (< Strength 0.5)
      (set `local.BreachesToCause` 1)
      (elif (< Strength 0.8)
        (set `local.BreachesToCause` 1)
        (else
          (set `local.BreachesToCause` 2)))))
  (bind _outactors (`GameplayStatics.GetAllActorsOfClassWithTag` "/Game/Blueprints/Hazards/HullBreach.HullBreach_C" Room))
  (for _array_element _outactors
    (bind _ashull_breach (cast `/Game/Blueprints/Hazards/HullBreach` _array_element))
    (if (`/Game/Blueprints/Hazards/HullBreach.BreachActive?` _ashull_breach)
      (`KismetArrayLibrary.Array_RemoveItem` _outactors _array_element)))
  (for _ (range 1 (+ (`local.BreachesToCause`) 1))
    (bind _ashull_breach_2 (cast `/Game/Blueprints/Hazards/HullBreach` (`|GetArrayItem` _outactors (`KismetMathLibrary.RandomIntegerInRange` 0 (- (`KismetArrayLibrary.Array_Length` _outactors) 1)))))
    (`/Game/Blueprints/Hazards/HullBreach.StartBreach` _ashull_breach_2)
    (bind _returnvalue (`KismetStringLibrary.Conv_NameToString` (`|GetArrayItem` (`Actor.Tags` _ashull_breach_2))))
    (bind (_value _returnvalue_2) (`BlueprintMapLibrary.Map_Find` (`/Game/Blueprints/Interfaces/Bridge/SubDisplayInterface.HullBreaches` _subdisplay) _returnvalue))
    ;[1 1 1] Add Breach to Status Display
    (if _returnvalue_2
      (`BlueprintMapLibrary.Map_Add` (`/Game/Blueprints/Interfaces/Bridge/SubDisplayInterface.HullBreaches` _subdisplay) _returnvalue (+ _value 1)))))

(fn `GetHitEventDirection`
  (params (HitVector :type "Vector Structure"))
  (returns (Direction :type "Float (double-precision)"))
  (bind _returnvalue (+ (`KismetMathLibrary.DegAtan2` (.y HitVector) (.x HitVector)) 90.0))
  (if (> _returnvalue 360.0)
    (return (- _returnvalue 360.0))
    (elif (< _returnvalue 0.0)
      (return (+ _returnvalue 360.0))
      (else
        (return _returnvalue)))))

(fn `HitEventEngineRoom`
  (params (HitVector :type "Vector Structure") (HitStrength :type "Float (double-precision)"))
  (locals (RoomsToAffect :type "Array of String"))
  (bind _roomstoaffect (`local.RoomsToAffect`))
  (switch `int` (`KismetMathLibrary.RandomIntegerInRange` 0 2)
    (:`0`
      (`KismetArrayLibrary.Array_Add` _roomstoaffect "Quarters"))
    (:`1`
      (`KismetArrayLibrary.Array_Add` _roomstoaffect "Mess"))
    (:`2`
      _))
  (`self.CameraShake` HitStrength _roomstoaffect)
  (bind _outactors (`GameplayStatics.GetAllActorsOfClass` "/Game/Blueprints/Items/PipeReceptacle.PipeReceptacle_C"))
  (for _array_element _outactors
    (if (> (- (* HitStrength 100.0) (`KismetMathLibrary.RandomFloatInRange` 0.0 50.0)) (`/Game/Blueprints/Items/PipeReceptacle.KnockOffRequirement` _array_element))
      (`/Game/Blueprints/Items/PipeReceptacle.Drop Pipe` _array_element (`KismetMathLibrary.MakeVector` (* (`KismetMathLibrary.Abs` (.x HitVector)) -1.0) (.y HitVector) (.z HitVector)))))
  (for _array_element_2 (`local.RoomsToAffect`)
    (if (> (`KismetMathLibrary.RandomIntegerInRange` 0 100) 30)
      (bind _returnvalue (`KismetStringLibrary.Conv_StringToName` _array_element_2))
      (`self.CreateHullBreaches` _returnvalue HitStrength)
      (else
        (`self.CreateFires` _returnvalue HitStrength)))))

(fn `HitEventLifeSupportRoom`
  (params (Strength :type "Float (double-precision)"))
  (locals (RoomsToAffect :type "Array of String"))
  (bind _roomstoaffect (`local.RoomsToAffect`))
  (switch `int` (`KismetMathLibrary.RandomIntegerInRange` 0 2)
    (:`0`
      (`KismetArrayLibrary.Array_Add` _roomstoaffect "Quarters"))
    (:`1`
      (`KismetArrayLibrary.Array_Add` _roomstoaffect "Bridge"))
    (:`2`
      _))
  (`self.CameraShake` Strength _roomstoaffect)
  (bind _outactors (`GameplayStatics.GetAllActorsOfClass` "/Game/Blueprints/Interfaces/LifeSupportRoom/CO2ScrubberRepairInterface.CO2ScrubberRepairInterface_C"))
  (`/Game/Blueprints/Interfaces/LifeSupportRoom/CO2ScrubberRepairInterface.BreakEvent` (`|GetArrayItem` _outactors))
  (for _array_element (`local.RoomsToAffect`)
    (if (> (`KismetMathLibrary.RandomIntegerInRange` 0 100) 30)
      (bind _returnvalue (`KismetStringLibrary.Conv_StringToName` _array_element))
      (`self.CreateHullBreaches` _returnvalue Strength)
      (else
        (`self.CreateFires` _returnvalue Strength)))))

(fn `HitEventSonarRoom`
  (params (Strength :type "Float (double-precision)"))
  (locals (RoomsToAffect :type "Array of String"))
  (bind _roomstoaffect (`local.RoomsToAffect`))
  (switch `int` (`KismetMathLibrary.RandomIntegerInRange` 0 2)
    (:`0`
      (`KismetArrayLibrary.Array_Add` _roomstoaffect "Mess"))
    (:`1`
      (`KismetArrayLibrary.Array_Add` _roomstoaffect "Bridge"))
    (:`2`
      _))
  (`self.CameraShake` Strength _roomstoaffect)
  (bind _outactors (`GameplayStatics.GetAllActorsOfClass` "/Game/Blueprints/Interfaces/SonarRoom/WireBoxInterface.WireBoxInterface_C"))
  (`/Game/Blueprints/Interfaces/SonarRoom/WireBoxInterface.DropWires` (`|GetArrayItem` _outactors))
  (for _array_element (`local.RoomsToAffect`)
    (if (> (`KismetMathLibrary.RandomIntegerInRange` 0 100) 30)
      (bind _returnvalue (`KismetStringLibrary.Conv_StringToName` _array_element))
      (`self.CreateHullBreaches` _returnvalue Strength)
      (else
        (`self.CreateFires` _returnvalue Strength)))))

(fn `HitEventTorpedoRoom`
  (params (Strength :type "Float (double-precision)"))
  (locals (RoomsToAffect :type "Array of String"))
  (bind _roomstoaffect (`local.RoomsToAffect`))
  (if (`KismetMathLibrary.RandomBool`)
    (`KismetArrayLibrary.Array_Add` _roomstoaffect "Bridge"))
  (`self.CameraShake` Strength _roomstoaffect)
  (for _array_element (`local.RoomsToAffect`)
    (if (> (`KismetMathLibrary.RandomIntegerInRange` 0 100) 30)
      (bind _returnvalue (`KismetStringLibrary.Conv_StringToName` _array_element))
      (`self.CreateHullBreaches` _returnvalue Strength)
      (else
        (`self.CreateFires` _returnvalue Strength)))))

(fn `ImpulseOnPhysicsObjects`
  (params (ForceVector :type "Vector Structure") (`Lights Only?` :type Boolean))
  (if (not `Lights Only?`)
    (bind _outactors (`GameplayStatics.GetAllActorsOfClass` "/Game/Blueprints/Items/Item.Item_C"))
    (for _array_element _outactors
      (bind _staticmesh (`/Game/Blueprints/Items/Item.StaticMesh` _array_element))
      (if (`SceneComponent.IsSimulatingPhysics` _staticmesh "None")
        (`PrimitiveComponent.AddImpulse` _staticmesh ForceVector "None" false)))
    (bind _outactors_2 (`GameplayStatics.GetAllActorsOfClass` "/Game/Blueprints/Usables/Usable.Usable_C"))
    (for _array_element_2 _outactors_2
      (bind _staticmesh_2 (`/Game/Blueprints/Usables/Usable.StaticMesh` _array_element_2))
      (if (`SceneComponent.IsSimulatingPhysics` _staticmesh_2 "None")
        (`PrimitiveComponent.AddImpulse` _staticmesh_2 ForceVector "None" false))))
  (bind _outactors_3 (`GameplayStatics.GetAllActorsOfClass` "/Game/Blueprints/EnvironmentalActors/HangingLight.HangingLight_C"))
  (for _array_element_3 _outactors_3
    (`PrimitiveComponent.AddImpulse` (`/Game/Blueprints/EnvironmentalActors/HangingLight.Light` _array_element_3) (`KismetMathLibrary.MakeVector` (* (.x ForceVector) (`KismetMathLibrary.RandomFloatInRange` 0.05 0.15)) (* (.y ForceVector) (`KismetMathLibrary.RandomFloatInRange` 0.05 0.15)) (* (.z ForceVector) (`KismetMathLibrary.RandomFloatInRange` 0.05 0.15))) "None" false)))

(fn `PipesTutorialHitEvent`
  (params (HitVector :type "Vector Structure") (HitStrength :type "Float (double-precision)"))
  (locals (RoomsToAffect :type "Array of String"))
  (bind _roomstoaffect (`local.RoomsToAffect`))
  (`KismetArrayLibrary.Array_Add` _roomstoaffect "Quarters")
  (`KismetArrayLibrary.Array_Add` _roomstoaffect "Mess")
  (`KismetArrayLibrary.Array_Add` _roomstoaffect "LifeSupport")
  (`KismetArrayLibrary.Array_Add` _roomstoaffect "SonarRoom")
  (`self.CameraShake` HitStrength _roomstoaffect)
  (bind _outactors (`GameplayStatics.GetAllActorsOfClass` "/Game/Blueprints/Items/PipeReceptacle.PipeReceptacle_C"))
  (for _array_element _outactors
    (if (> (- (* HitStrength 100.0) (`KismetMathLibrary.RandomFloatInRange` 0.0 50.0)) (`/Game/Blueprints/Items/PipeReceptacle.KnockOffRequirement` _array_element))
      (`/Game/Blueprints/Items/PipeReceptacle.Drop Pipe` _array_element (`KismetMathLibrary.MakeVector` (* (`KismetMathLibrary.Abs` (.x HitVector)) -3000.0) (.y HitVector) (.z HitVector))))))

(fn `UserConstructionScript`)