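; Physical button that fires a flare from a linked flare tube.
; On press it depresses its collision component, plays a click sound and checks the tube's state.
; It fires only when the tube is flooded, grabbing an object, not draining and its mesh is not open; otherwise it flashes an alert light.
; Release restores the button position and plays a release sound.
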(event `self.OnPressed`
  (bind _flaretube (`self.FlareTube`))
  (`parent.OnPressed`)
  (`SceneComponent.K2_SetRelativeLocation` (`self.ButtonCollision`) (0.0 -2.0 0.0) false false)
  (`GameplayStatics.PlaySoundAtLocation` "/Game/SFX/ButtonPressCue.ButtonPressCue" (`SceneComponent.K2_GetComponentLocation` (`self.DefaultSceneRoot`)) (struct) 1.0 1.0 0.0 null null null)
  (if (and (not (`/Game/Blueprints/Interfaces/WeaponsRoom/FlareReceptacle.IsDraining` _flaretube)) (and (`/Game/Blueprints/Interfaces/WeaponsRoom/FlareReceptacle.IsFlooded` _flaretube) (`/Game/Blueprints/Items/ItemReceptacle.isGrabbingObject` _flaretube)) (not (`/Game/Blueprints/Interfaces/WeaponsRoom/FlareTube.IsOpen` (`self.FlareTubeMesh`))))
    (`/Game/Blueprints/Interfaces/WeaponsRoom/FlareReceptacle.Fire` _flaretube)
    (else
      (`/Game/Blueprints/Interfaces/AlertLight.AlertFlash` (`self.AlertLight`)))))

(event `self.ButtonReleased`
  (`parent.ButtonReleased`)
  (`SceneComponent.K2_SetRelativeLocation` (`self.ButtonCollision`) (0.0 0.0 0.0) false false)
  (`GameplayStatics.PlaySoundAtLocation` "/Game/SFX/ButtonReleaseCue.ButtonReleaseCue" (`SceneComponent.K2_GetComponentLocation` (`self.DefaultSceneRoot`)) (struct) 1.0 1.0 0.0 null null null))

(fn `UserConstructionScript`
  (`parent.UserConstructionScript`))