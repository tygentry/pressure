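; Central controller for the submarine's systems: starts and stops them, tracks depth and hull integrity, and supports skipping the tutorial.
; A timeline-driven SystemsCheck scales battery pumping by pipe flow, refreshes the status display, and updates oxygen decay from fires.
; Powered battery count feeds the sub marker and timer-lerped light dimming.
; Depth, accumulated from marker velocity, selects the required floppy disk and triggers surfacing; depleted hull integrity triggers delayed implosion death.
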(event `SkipTutorial`
  (`self.OpenAllDoors`)
  (`KismetSystemLibrary.Delay` 0.2)
  (`self.StartAllSystems`)
  (set `/Game/Blueprints/Controllers/DialogueController.IsTutorialDone` true (`self.DialogueController`))
  (`KismetSystemLibrary.Delay` 30.0)
  (`/Game/Blueprints/Controllers/MonsterController.SummonMonster` (`self.MonsterController`)))

(event `self.ReceiveBeginPlay`
  (bind _startlightintensities (`self.StartLightIntensities`))
  ;[1 1 1] Setup
  (if (`self.DevMode`)
    (`self.SkipTutorial`))
  (bind _outactors (`GameplayStatics.GetAllActorsOfClassWithTag` "/Game/Blueprints/Items/PipeReceptacle.PipeReceptacle_C" "Flows Into Terminus")) ; check all paths into terminus, and get the proportion that have flow
  (for _array_element _outactors
    (bind _aspipe_receptacle (cast `/Game/Blueprints/Items/PipeReceptacle` _array_element))
    (`BlueprintMapLibrary.Map_Add` (`self.BrokenPaths`) _aspipe_receptacle))
  (bind _outactors_2 (`GameplayStatics.GetAllActorsOfClassWithTag` "/Game/Blueprints/Items/PipeReceptacle.PipeReceptacle_C" "Pipe Terminus"))
  (bind _aspipe_receptacle_2 (cast `/Game/Blueprints/Items/PipeReceptacle` (`|GetArrayItem` _outactors_2)))
  (set `self.PipeTerminus` _aspipe_receptacle_2)
  (bind _outactors_3 (`GameplayStatics.GetAllActorsOfClass` "/Script/Engine.PointLight"))
  (for _array_element_2 _outactors_3
    (bind _pointlightcomponent (`PointLight.PointLightComponent` _array_element_2))
    (`KismetArrayLibrary.Array_Add` (`self.DimmingLights`) _pointlightcomponent)
    (`BlueprintMapLibrary.Map_Add` _startlightintensities _pointlightcomponent (`LightComponentBase.Intensity` _pointlightcomponent)))
  (bind _outactors_4 (`GameplayStatics.GetAllActorsOfClass` "/Game/Blueprints/EnvironmentalActors/HangingLight.HangingLight_C"))
  (for _array_element_3 _outactors_4
    (bind _pointlight (`/Game/Blueprints/EnvironmentalActors/HangingLight.PointLight` _array_element_3))
    (`KismetArrayLibrary.Array_Add` (`self.DimmingLights`) _pointlight)
    (`BlueprintMapLibrary.Map_Add` _startlightintensities _pointlight (`LightComponentBase.Intensity` _pointlight)))
  (bind _outactors_5 (`GameplayStatics.GetAllActorsOfClass` "/Game/Blueprints/EnvironmentalActors/WallLight.WallLight_C"))
  (for _array_element_4 _outactors_5
    (`KismetArrayLibrary.Array_Add` (`self.AlertWallLights`) _array_element_4))
  (bind _outactors_6 (`GameplayStatics.GetAllActorsOfClass` "/Game/Blueprints/EnvironmentalActors/CeilingLight.CeilingLight_C"))
  (for _array_element_5 _outactors_6
    (`KismetArrayLibrary.Array_Add` (`self.AlertCeilingLights`) _array_element_5))
  (`Timeline|CheckTimeline` :!via `PlayFromStart`
    (:`CheckSystemsEvent`
      (`self.SystemsCheck`))))

(event `OpenDoor`
  (params (Index :type Integer))
  ;[1 1 1] Open Door
  (`/Game/Blueprints/EnvironmentalActors/Door.OpenDoor` (`|GetArrayItem` (`self.Doors`) Index)))

(event `ChangeHullIntegrity`
  (params (Delta :type Integer))
  ;[1 1 1] Change hull integrity
  (set `self.HullIntegrity` (+ (`self.HullIntegrity`) Delta)))

(event `OpenAllDoors`
  ;[1 1 1] Open Door
  (for _array_element (`self.Doors`)
    (`/Game/Blueprints/EnvironmentalActors/Door.OpenDoor` _array_element)))

(event `HullCollapseFunction`
  (set `self.CollapseImminent?` true)
  (`KismetSystemLibrary.PrintString` "ah")
  (`KismetSystemLibrary.Delay` 15.5)
  (if (<= (`self.HullIntegrity`) 0)
    (`GameplayStatics.PlaySound2D` "/Game/SFX/HullCollapseDeathSub.HullCollapseDeathSub" 1.0 1.0 0.0 null null)
    (bind _outactors (`GameplayStatics.GetAllActorsOfClass` "/Game/FirstPersonBP/Blueprints/FirstPersonCharacter.FirstPersonCharacter_C"))
    (`/Game/FirstPersonBP/Blueprints/FirstPersonCharacter.Die` (`|GetArrayItem` _outactors) "Cause: Hull implosion")
    (else
      (set `self.CollapseImminent?` false))))

(fn `CheckEnginePipes`
  (returns (FlowStrength :type "Float (double-precision)"))
  (locals (BrokenPathsCount :type Integer))
  (bind _brokenpaths (`self.BrokenPaths`))
  (bind _keys (`BlueprintMapLibrary.Map_Keys` (`self.BrokenPaths`)))
  (for _array_element _keys
    (bind _hasflow_ (`/Game/Blueprints/Items/PipeReceptacle.Check Water Flow` _array_element))
    (if _hasflow_
      (`BlueprintMapLibrary.Map_Add` _brokenpaths _array_element)
      (if (not (`/Game/Blueprints/Items/ItemReceptacle.isGrabbingObject` (`self.PipeTerminus`)))
        (bind _aspipe (cast `/Game/Blueprints/Items/Pipe` (`/Game/Blueprints/Items/ItemReceptacle.MostRecentGrabbedObject` _array_element)))
        (`/Game/Blueprints/Items/Pipe.WaterFlowingOn` _aspipe) ; if this path has flow but the terminus is not attached, start flowing water effect
      )
      (else
        (`/Engine/EditorBlueprintResources/StandardMacros.IncrementInt` (`local.BrokenPathsCount`)
          (:`  `
            (`BlueprintMapLibrary.Map_Add` _brokenpaths _array_element true))))))
  (if (`/Game/Blueprints/Items/ItemReceptacle.isGrabbingObject` (`self.PipeTerminus`))
    (return (- 1.0 (/ (`KismetMathLibrary.Conv_IntToDouble` (`local.BrokenPathsCount`)) (`KismetMathLibrary.Conv_IntToDouble` (`KismetArrayLibrary.Array_Length` _keys)))))
    (else
      (return 0.0))))

(fn `PowerLights`
  ;[1 1 1] Dimming DimLights based on power
  (for _array_element (`self.DimmingLights`)
    (bind _intensity (`LightComponentBase.Intensity` _array_element))
    (bind _returnvalue (* (`BlueprintMapLibrary.Map_Find` (`self.StartLightIntensities`) _array_element) (/ (+ (`KismetMathLibrary.Conv_IntToDouble` (`self.PrevPoweredBatteryNum`)) 1.0) 3.5)))
    (`LightComponent.SetIntensity` _array_element (`KismetMathLibrary.Lerp` _intensity _returnvalue 0.6)))
  (if (`KismetMathLibrary.NearlyEqual_FloatFloat` _intensity _returnvalue)
    (`KismetSystemLibrary.K2_ClearTimer` null "PowerLights")))

(fn `StartAllSystems`
  (bind _navthrottle (`self.NavThrottle`))
  (`/Game/Blueprints/Interfaces/EngineRoom/WaterDistributionInterface.StartWaterDecay` (`self.BatteryPump`))
  (`/Game/Blueprints/Interfaces/LifeSupportRoom/OxygenSupplyInterface.StartOxygenDecay` (`self.OxygenSystem`))
  (`/Game/Blueprints/Interfaces/SonarRoom/FrequencyInterface.StartFrequencyDecay` (`self.FrequencyMatch`))
  (set `/Game/Blueprints/Interfaces/LifeSupportRoom/CO2ScrubberInterface.IsUnlocked?` true (`self.CO2Scrubber`))
  (set `/Game/Blueprints/Interfaces/Bridge/NavigationThrottle.IsEnabled` true _navthrottle)
  (`/Game/Blueprints/Interfaces/Bridge/NavigationThrottle.StartMovement` _navthrottle)
  (`SceneComponent.SetVisibility` (`/Game/Blueprints/Interfaces/Bridge/NavigationScreen.Screen` (`self.NavScreen`)) true true)
  (for _array_element (`self.FlareTubes`)
    (set `/Game/Blueprints/Interfaces/WeaponsRoom/FlareReceptacle.TutorialFired` true _array_element)
    (set `/Game/Blueprints/Interfaces/WeaponsRoom/FlareReceptacle.AllowFiring` true _array_element)))

(fn `StopAllSystems`
  (`/Game/Blueprints/Interfaces/EngineRoom/WaterDistributionInterface.StopWaterDecay` (`self.BatteryPump`))
  (`/Game/Blueprints/Interfaces/LifeSupportRoom/OxygenSupplyInterface.StopOxygenDecay` (`self.OxygenSystem`))
  (`/Game/Blueprints/Interfaces/SonarRoom/FrequencyInterface.StopFrequencyDecay` (`self.FrequencyMatch`))
  (set `/Game/Blueprints/Interfaces/LifeSupportRoom/CO2ScrubberInterface.IsUnlocked?` false (`self.CO2Scrubber`))
  (set `/Game/Blueprints/Interfaces/Bridge/NavigationThrottle.IsEnabled` false (`self.NavThrottle`))
  (`SceneComponent.SetVisibility` (`/Game/Blueprints/Interfaces/Bridge/NavigationScreen.Screen` (`self.NavScreen`)) false true))

(fn `SystemsCheck`
  (bind _batterypump (`self.BatteryPump`))
  (bind _co2scrubber (`self.CO2Scrubber`))
  (bind _submarker (`self.SubMarker`))
  (bind _hullintegrity (`self.HullIntegrity`))
  (bind _subdisplaywidget (`/Game/Blueprints/Interfaces/Bridge/SubDisplayInterface.SubDisplayWidget` (`self.SubDisplay`)))
  ;[1 1 1] Pipes and Water Pumping
  (bind _flowstrength (`self.CheckEnginePipes`))
  (`/Game/Blueprints/Interfaces/Bridge/SubDisplayWidget.ChangePipesBroken` (`/Game/Blueprints/Interfaces/Bridge/SubDisplayInterface.SubDisplayWidget` (`self.SubDisplay`)) (not (== _flowstrength 1.0)))
  (set `/Game/Blueprints/Interfaces/EngineRoom/WaterDistributionInterface.PumpSpeedTotal` (* _flowstrength (`/Game/Blueprints/Interfaces/EngineRoom/WaterDistributionInterface.PumpSpeedDefault` _batterypump)) _batterypump)
  (`/Game/Blueprints/Interfaces/Bridge/SubDisplayWidget.ChangeWaterTank` (`/Game/Blueprints/Interfaces/Bridge/SubDisplayInterface.SubDisplayWidget` (`self.SubDisplay`)) (`/Game/Blueprints/Interfaces/EngineRoom/WaterTank.WaterLevel` (`self.WaterTank`)))
  (bind _poweredbatteries (`/Game/Blueprints/Interfaces/EngineRoom/WaterDistributionInterface.PoweredBatteries` (`self.BatteryPump`)))
  (`/Game/Blueprints/Interfaces/Bridge/SubDisplayWidget.ChangeBatteryIcons` (`/Game/Blueprints/Interfaces/Bridge/SubDisplayInterface.SubDisplayWidget` (`self.SubDisplay`)) _poweredbatteries)
  ;[1 1 1] Life Support Systems
  (`/Game/Blueprints/Interfaces/Bridge/SubDisplayWidget.ChangeOxygenVent` (`/Game/Blueprints/Interfaces/Bridge/SubDisplayInterface.SubDisplayWidget` (`self.SubDisplay`)) (`/Game/Blueprints/Interfaces/LifeSupportRoom/OxygenSupplyInterface.OxygenLevel` (`self.OxygenSystem`)))
  (`/Game/Blueprints/Interfaces/Bridge/SubDisplayWidget.ChangeCO2Scrubber` (`/Game/Blueprints/Interfaces/Bridge/SubDisplayInterface.SubDisplayWidget` (`self.SubDisplay`)) (`/Game/Blueprints/Interfaces/LifeSupportRoom/CO2ScrubberInterface.CO2Composition` _co2scrubber) (`/Game/Blueprints/Interfaces/LifeSupportRoom/CO2ScrubberInterface.IsBroken?` _co2scrubber))
  ;[1 1 1] Sonar Systems Checks
  (bind _numcorrectfreq (`/Game/Blueprints/Interfaces/SonarRoom/FrequencyInterface.GetCorrectFreq` (`self.FrequencyMatch`)))
  (`/Game/Blueprints/Interfaces/Bridge/SubDisplayWidget.ChangeFreqIcons` _subdisplaywidget _numcorrectfreq (`/Game/Blueprints/Interfaces/SonarRoom/FDReceptacle.CorrectDiskIn` (`self.DiskReader`)))
  (`/Game/Blueprints/Interfaces/Bridge/SubDisplayWidget.ChangeFreqDisplay` _subdisplaywidget (not (`/Game/Blueprints/Interfaces/SonarRoom/FrequencyInterface.DisplayOn` (`self.FrequencyMatch`))))
  (`/Game/Blueprints/Interfaces/Bridge/SubDisplayWidget.ChangeJunctionBox` _subdisplaywidget (not (`/Game/Blueprints/Interfaces/SonarRoom/WireBoxInterface.AllConnected?` (`self.WireBox`))))
  (`/Game/Blueprints/Interfaces/Bridge/SubDisplayWidget.ChangeSonarDisplay` _subdisplaywidget (not (`/Game/Blueprints/Interfaces/Interfaces_V1/SonarScreen.HasSignal?` (`self.SonarScreen`))))
  ;[1 1 1] Battery Related Checks (Lighting and Speed)
  (bind _poweredbatteries_2 (`/Game/Blueprints/Interfaces/EngineRoom/WaterDistributionInterface.PoweredBatteries` (`self.BatteryPump`)))
  (if (not (== _poweredbatteries_2 (`self.PrevPoweredBatteryNum`)))
    (bind _output_get (set `self.PrevPoweredBatteryNum` _poweredbatteries_2))
    (`KismetSystemLibrary.K2_SetTimer` null "PowerLights" 0.1 true))
  (set `/Game/Blueprints/NavigationSupport/SubMarker.PoweredBatteries` _output_get _submarker)
  (bind _returnvalue (`PrimitiveComponent.GetPhysicsLinearVelocity` (`/Game/Blueprints/NavigationSupport/SubMarker.StaticMesh` _submarker) "None"))
  (bind _output_get_2 (set `self.Depth` (+ (/ (.y _returnvalue) 950.0) (`self.Depth`))))
  (set `/Game/Blueprints/NavigationSupport/SubMarker.Depth` _output_get_2 (`self.SubMarker`))
  ;[1 1 1] update freq disk
  (`self.UpdateFreqDisk`)
  ;[1 1 1] Oxygen Decay
  (`self.UpdateOxygenDecay`)
  ;[1 1 1] Updating Hull Integrity Display
  (if (and (<= _hullintegrity 0) (not (`self.CollapseImminent?`)))
    (`self.HullCollapseFunction`))
  (bind _assub_display_screen (cast `/Game/Blueprints/Interfaces/Bridge/SubDisplayScreen` (`ChildActorComponent.ChildActor` (`/Game/Blueprints/Interfaces/Bridge/SubDisplayInterface.SubDisplayScreen` (`self.SubDisplay`)))))
  (`TextRenderComponent.K2_SetText` (`/Game/Blueprints/Interfaces/Bridge/SubDisplayScreen.PercentText` _assub_display_screen) (`KismetTextLibrary.Conv_StringToText` (`KismetStringLibrary.Concat_StrStr` (`KismetStringLibrary.Conv_IntToString` (`KismetMathLibrary.Clamp` _hullintegrity 0 100)) "%")))
  ;[1 1 1] Once player reaches the surface
  (if (and (<= (`self.Depth`) 0.0) (not (`self.ReachedEnd`)))
    (set `self.ReachedEnd` true)
    (`/Game/Blueprints/Controllers/HitEventController.BumpEvent` (`self.HitEventController`))
    (`GameplayStatics.PlaySoundAtLocation` "/Game/SFX/RockImpactSub.RockImpactSub" (0.0 3565.0 210.0) (struct) 1.0 1.0 0.0 null null null)
    (`self.StopAllSystems`)
    (`/Game/Blueprints/EnvironmentalActors/Bridge/EscapeHatch.OpenHatch` (`self.EscapeHatch`))
    (bind _outactors (`GameplayStatics.GetAllActorsOfClass` "/Game/Blueprints/Controllers/RAASController.RAASController_C"))
    (`KismetArrayLibrary.Array_Add` (`/Game/Blueprints/Controllers/RAASController.AlertsQueue` (`|GetArrayItem` _outactors)) "/Game/VO/Placeholder/RAASVO/RAASReachedSurface.RAASReachedSurface")))

(fn `UpdateFreqDisk`
  (bind _diskreader (`self.DiskReader`))
  (bind _output (`|GetArrayItem` (`self.FloppyDisks`) 5))
  (bind _output_2 (`|GetArrayItem` (`self.FloppyDisks`) 4))
  (bind _output_3 (`|GetArrayItem` (`self.FloppyDisks`) 3))
  (bind _output_4 (`|GetArrayItem` (`self.FloppyDisks`) 2))
  (bind _output_5 (`|GetArrayItem` (`self.FloppyDisks`)))
  (bind _output_6 (`|GetArrayItem` (`self.FloppyDisks`) 1))
  (if (<= (`self.Depth`) 800.0)
    (if (<= (`self.Depth`) 600.0)
      (if (<= (`self.Depth`) 400.0)
        (if (<= (`self.Depth`) 200.0)
          (if (<= (`self.Depth`) 100.0)
            ;[1 1 1] 0-100m set
            (if (not (== (`/Game/Blueprints/Interfaces/SonarRoom/FDReceptacle.RequiredFD` _diskreader) _output_5))
              (set `/Game/Blueprints/Interfaces/SonarRoom/FDReceptacle.RequiredFD` _output_5 _diskreader)
              (set `/Game/Blueprints/Interfaces/SonarRoom/FDReceptacle.CorrectDiskIn` false _diskreader))
            (else
              ;[1 1 1] 100-200m set
              (if (not (== (`/Game/Blueprints/Interfaces/SonarRoom/FDReceptacle.RequiredFD` _diskreader) _output_6))
                (set `/Game/Blueprints/Interfaces/SonarRoom/FDReceptacle.RequiredFD` _output_6 _diskreader)
                (set `/Game/Blueprints/Interfaces/SonarRoom/FDReceptacle.CorrectDiskIn` false _diskreader))))
          (else
            ;[1 1 1] 200-400m set
            (if (not (== (`/Game/Blueprints/Interfaces/SonarRoom/FDReceptacle.RequiredFD` _diskreader) _output_4))
              (set `/Game/Blueprints/Interfaces/SonarRoom/FDReceptacle.RequiredFD` _output_4 _diskreader)
              (set `/Game/Blueprints/Interfaces/SonarRoom/FDReceptacle.CorrectDiskIn` false _diskreader))))
        (else
          ;[1 1 1] 400-600m set
          (if (not (== (`/Game/Blueprints/Interfaces/SonarRoom/FDReceptacle.RequiredFD` _diskreader) _output_3))
            (set `/Game/Blueprints/Interfaces/SonarRoom/FDReceptacle.RequiredFD` _output_3 _diskreader)
            (set `/Game/Blueprints/Interfaces/SonarRoom/FDReceptacle.CorrectDiskIn` false _diskreader))))
      (else
        ;[1 1 1] 600-800m set
        (if (not (== (`/Game/Blueprints/Interfaces/SonarRoom/FDReceptacle.RequiredFD` _diskreader) _output_2))
          (set `/Game/Blueprints/Interfaces/SonarRoom/FDReceptacle.RequiredFD` _output_2 _diskreader)
          (set `/Game/Blueprints/Interfaces/SonarRoom/FDReceptacle.CorrectDiskIn` false _diskreader))))
    (else
      ;[1 1 1] 800-1000m Disk set
      (if (not (== (`/Game/Blueprints/Interfaces/SonarRoom/FDReceptacle.RequiredFD` _diskreader) _output))
        (set `/Game/Blueprints/Interfaces/SonarRoom/FDReceptacle.RequiredFD` _output _diskreader)
        (set `/Game/Blueprints/Interfaces/SonarRoom/FDReceptacle.CorrectDiskIn` false _diskreader)))))

(fn `UpdateOxygenDecay`
  (set `/Game/Blueprints/Interfaces/LifeSupportRoom/OxygenSupplyInterface.DecayPercent` (+ (* (`self.FireCount`) 0.1) 0.1) (`self.OxygenSystem`)))

(fn `UserConstructionScript`)