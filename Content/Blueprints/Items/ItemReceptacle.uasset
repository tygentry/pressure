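; Item receptacle actor that snaps a held, eligible item into a fixed slot when the item touches it.
; On hit it casts to Item, freezes physics, teleports it to an offset and rotation, makes the player let go, and records itself on the item.
; It holds one item at a time and can lock it against pickup.
; Release restores physics and briefly blocks re-insertion; a loading-save flag skips the held check and player release.
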(event `self.ReceiveHit`
  (params (MyComp :type "PrimitiveComponent Object Reference") (Other :type "Actor Object Reference") (OtherComp :type "PrimitiveComponent Object Reference") (bSelfMoved :type Boolean) (HitLocation :type "Vector Structure") (HitNormal :type "Vector Structure") (NormalImpulse :type "Vector Structure") (Hit :type "HitResult Structure (by ref)"))
  ;[1 1 1] When this receptacle comes into contact with a held item, grab it
  (if (`KismetMathLibrary.ClassIsChildOf` (`GameplayStatics.GetObjectClass` Other) (`self.GrabbableObjectsSuperclass`))
    (bind _asitem (cast `/Game/Blueprints/Items/Item` Other)
      (:`then`
        (`self.GrabObject` _asitem))
      (:`CastFailed`
        (`KismetSystemLibrary.PrintString` "receptacle couldnt cast to item!! whoops!!")))))

(event `GrabObject`
  (params (Item :type "/Game/Blueprints/Items/Item Object Reference") (`LoadingSave?` :type Boolean :default false))
  (bind _staticmesh (`/Game/Blueprints/Items/Item.StaticMesh` Item))
  ;[1 1 1] When this receptacle comes into contact with a held item, grab it
  (if (and (and (or `LoadingSave?` (`/Game/Blueprints/Items/Item.IsBeingHeld` Item)) (`/Game/Blueprints/Items/Item.CanBePutInReceptacle` Item)) (not (`self.isGrabbingObject`)))
    (`PrimitiveComponent.SetSimulatePhysics` _staticmesh false)
    (`SceneComponent.K2_SetWorldLocationAndRotation` _staticmesh (+ (`SceneComponent.K2_GetComponentLocation` (`self.DefaultSceneRoot`)) (`self.RecievedObjectOffset`)) (`self.RecievedObjectRotation`) false true)
    (if `LoadingSave?`
      (set `/Game/Blueprints/Items/Item.IsInReceptacle` true Item :!label _label)
      (`/Game/Blueprints/Items/Item.Set Most Recent Receptacle` Item self) ; cant do this manually from within this blueprint for whatever reason
      (if (not (`self.GrabbedObjectCanBeTaken`))
        (set `/Game/Blueprints/Items/Item.CanBeHeld` false Item))
      (set `self.MostRecentGrabbedObject` Item)
      (set `self.isGrabbingObject` true)
      (else
        (bind _asfirst_person_character (cast `/Game/FirstPersonBP/Blueprints/FirstPersonCharacter` (`GameplayStatics.GetPlayerCharacter` 0))
          (:`then`
            (`/Game/FirstPersonBP/Blueprints/FirstPersonCharacter.Release Object` _asfirst_person_character)
            (goto _label))
          (:`CastFailed`
            (`KismetSystemLibrary.PrintString` "failed to cast player to firstpersoncharacter!!")))))))

(event `ReleaseObject`
  (bind _mostrecentgrabbedobject (`self.MostRecentGrabbedObject`))
  ;[1 1 1] release object
  (`PrimitiveComponent.SetSimulatePhysics` (`/Game/Blueprints/Items/Item.StaticMesh` _mostrecentgrabbedobject) true)
  (set `/Game/Blueprints/Items/Item.IsInReceptacle` false _mostrecentgrabbedobject)
  (`/Game/Blueprints/Items/Item.Prevent From Being Put In Receptacle` _mostrecentgrabbedobject 1.0)
  (set `self.isGrabbingObject` false)
  (set `/Game/Blueprints/Items/Item.CanBeHeld` true _mostrecentgrabbedobject))

(fn `UserConstructionScript`)