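; Controller for the sonar monster that threatens the submarine, simulated as a 2D point around the sub at the origin.
; Tick runs a string-keyed state machine (Loiter, Attack, Inspect, Fake Attack, Follow Flare, Leave) with weighted random transitions.
; Attacks trigger the hit event controller, launched flares lure the monster away, and leaving schedules a random respawn at the range edge.
; The monster's position is mapped into world space to drive its audio controller.
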(event `self.ReceiveBeginPlay`)

(event `self.ReceiveTick`
  (params (DeltaSeconds :type "Float (single-precision)"))
  (bind _aistate (`self.AIState`))
  ;[1 1 1] Monster Tick
  (if (`self.MonsterPresent?`)
    (`self.SetAudioControllerLocation`)
    (if (`KismetStringLibrary.EqualEqual_StrStr` (`self.AIState`) "Loiter")
      (`self.LoiterBehavior` 350.0)
      (elif (`KismetStringLibrary.EqualEqual_StrStr` (`self.AIState`) "Attack")
        (`self.AttackBehavior`)
        (elif (`KismetStringLibrary.EqualEqual_StrStr` (`self.AIState`) "Inspect")
          (`self.InspectBehavior`)
          (elif (`KismetStringLibrary.EqualEqual_StrStr` (`self.AIState`) "Fake Attack")
            (`self.FakeAttackBehavior`)
            (elif (`KismetStringLibrary.EqualEqual_StrStr` (`self.AIState`) "Follow Flare")
              (`self.FollowFlareBehavior`)
              (elif (`KismetStringLibrary.EqualEqual_StrStr` _aistate "Leave")
                (`self.LeaveBehavior`)
                (else
                  (`KismetSystemLibrary.PrintString` (`KismetStringLibrary.Concat_StrStr` _aistate " is not a valid AIState!") true true (struct :`R` 1.0 :`B` 0.089263 :`A` 1.0) 4.0)))))))))
  ;[1 1 1] Flares Tick
  (if (!= (`self.LeftFlareLoc`) (0.0 0.0))
    (`self.LeftFlareMovement`))
  (if (!= (`self.RightFlareLoc`) (0.0 0.0))
    (`self.RightFlareMovement`)))

(event `SummonMonster`
  ;[1 1 1] Summon Monster at random position on edge of sonar range
  (set `self.MonsterPresent?` true)
  (if (`KismetMathLibrary.RandomBool`)
    (if (`KismetMathLibrary.RandomBool`)
      (set `self.MonsterX` 400.0)
      (else
        (set `self.MonsterX` -400.0)))
    (set `self.MonsterY` (`KismetMathLibrary.RandomFloatInRange` -400.0 400.0))
    (else
      (if (`KismetMathLibrary.RandomBool`)
        (set `self.MonsterY` 400.0)
        (else
          (set `self.MonsterY` -400.0)))
      (set `self.MonsterX` (`KismetMathLibrary.RandomFloatInRange` -400.0 400.0))))
  (bind _output_get (set `self.StateSelector` (`KismetMathLibrary.RandomIntegerInRange` 0 100)))
  (if (< _output_get 20)
    (set `self.AIState` "Inspect") ; 20% chance to inspect
    (elif (< _output_get 60)
      (set `self.AIState` "Attack") ; 40% chance to attack
      (else
        (set `self.AIState` "Loiter") ; 40% chance to loiter
      )))
  (`KismetSystemLibrary.PrintString` (`KismetStringLibrary.Concat_StrStr` "summoned X:   " (`KismetStringLibrary.Conv_DoubleToString` (`self.MonsterX`)) "   Y:   " (`KismetStringLibrary.Conv_DoubleToString` (`self.MonsterY`))) true true (struct :`G` 0.66 :`B` 1.0 :`A` 1.0) 4.0))

(event `BringMonsterBack`
  (`KismetSystemLibrary.Delay` (`KismetMathLibrary.RandomFloatInRange` 1.0 8.0))
  (`self.SummonMonster`))

(fn `AttackBehavior`
  (bind _monstery (`self.MonsterY`))
  (bind _monsterx (`self.MonsterX`))
  (bind _returnvalue (`KismetMathLibrary.MakeVector2D` (`self.MonsterX`) (`self.MonsterY`)))
  (bind _returnvalue_2 (`KismetMathLibrary.Sqrt` (+ (`KismetMathLibrary.Square` _monstery) (`KismetMathLibrary.Square` _monsterx))))
  (`self.MoveMonsterTowardsLocation` 0.3)
  (if (`KismetMathLibrary.NearlyEqual_FloatFloat` (`KismetMathLibrary.Distance2D` _returnvalue) 15.0 1.0)
    (`/Game/Blueprints/Controllers/MonsterAudioController.PlayAttackSound` (`self.MonsterAudioController`)))
  (if (== _returnvalue (0.0 0.0) :`ErrorTolerance` 1.0)
    (`/Game/Blueprints/Controllers/HitEventController.HitEventMonster` (`self.HitEventController`) (`KismetMathLibrary.MakeVector` (/ _monsterx _returnvalue_2) (/ _monstery _returnvalue_2) (`KismetMathLibrary.RandomFloatInRange` -0.25 0.25)) (`KismetMathLibrary.RandomFloatInRange` 0.1 1.0))
    (set `self.AIState` "Leave")))

(fn `FakeAttackBehavior`
  (bind _targetloc (`self.TargetLoc`))
  (bind (_x _y) (`KismetMathLibrary.BreakVector2D` (`self.TargetLoc`)))
  (if (== _targetloc (0.0 0.0))
    (set `self.TargetLoc` (`KismetMathLibrary.MakeVector2D` (* -1 (`self.MonsterX`)) (* -1 (`self.MonsterY`))))
    (elif (== _targetloc (`KismetMathLibrary.MakeVector2D` (`self.MonsterX`) (`self.MonsterY`)) :`ErrorTolerance` 1.0)
      (set `self.AIState` "Leave")
      (else
        (`self.MoveMonsterTowardsLocation` 0.3 _x _y)))))

(fn `FollowFlareBehavior`
  (bind _returnvalue (!= (`self.LeftFlareLoc`) (0.0 0.0)))
  (bind _returnvalue_2 (!= (`self.RightFlareLoc`) (0.0 0.0)))
  (bind (_x _y) (`KismetMathLibrary.BreakVector2D` (`self.RightFlareLoc`)))
  (bind (_x_2 _y_2) (`KismetMathLibrary.BreakVector2D` (`self.LeftFlareLoc`)))
  (if (and _returnvalue _returnvalue_2)
    (if (< (`self.MonsterX`) 0.0)
      (`self.MoveMonsterTowardsLocation` 0.3 (+ _x_2 (`KismetMathLibrary.RandomFloatInRange` 5.0 20.0)) _y_2 :!label _label) ; follow left flare
      (else
        (`self.MoveMonsterTowardsLocation` 0.3 (- _x (`KismetMathLibrary.RandomFloatInRange` 5.0 20.0)) _y :!label _label_2) ; follow right flare
      ))
    (elif _returnvalue
      (goto _label)
      (elif _returnvalue_2
        (goto _label_2)))))

(fn `InspectBehavior`
  (bind _targetloc (`self.TargetLoc`))
  (bind _loiterpointsvisited (`self.LoiterPointsVisited`))
  (bind (_x _y) (`KismetMathLibrary.BreakVector2D` (`self.TargetLoc`)))
  (if (or (== _targetloc (0.0 0.0)) (== _targetloc (`KismetMathLibrary.MakeVector2D` (`self.MonsterX`) (`self.MonsterY`)) :`ErrorTolerance` 1.0))
    (`/Game/Blueprints/Controllers/MonsterAudioController.PlayInspectSound` (`self.MonsterAudioController`))
    (bind _output_get (set `self.TargetLoc` (`KismetMathLibrary.MakeVector2D` (`KismetMathLibrary.RandomFloatInRange` -50.0 50.0) (`KismetMathLibrary.RandomFloatInRange` -50.0 50.0))))
    (if (> _loiterpointsvisited (`KismetMathLibrary.RandomIntegerInRange` 1 4))
      (set `self.LoiterPointsVisited` 0)
      (set `self.TargetLoc` (0.0 0.0))
      (bind _output_get_2 (set `self.StateSelector` (`KismetMathLibrary.RandomIntegerInRange` 0 100)))
      (if (< _output_get_2 45)
        (set `self.AIState` "Leave") ; 45% chance to leave
        (else
          (set `self.AIState` "Loiter") ; 55% chance to loiter
        ))
      (else
        (`/Engine/EditorBlueprintResources/StandardMacros.IncrementInt` _loiterpointsvisited)))
    (elif (>= (`KismetMathLibrary.Sqrt` (+ (`KismetMathLibrary.Square` (`self.MonsterX`)) (`KismetMathLibrary.Square` (`self.MonsterY`)))) 60.0)
      (`self.MoveMonsterTowardsLocation` 0.3 _x _y)
      (else
        (`self.MoveMonsterTowardsLocation` 0.15 _x _y)))))

(fn `LaunchFlare`
  (params (Direction :type Boolean))
  (if Direction
    (set `self.LeftFlareLoc` (-5.0 0.0))
    (else
      (set `self.RightFlareLoc` (5.0 0.0))))
  (set `self.AIState` "Follow Flare")
  (set `self.TargetLoc` (0.0 0.0))
  (set `self.LoiterPointsVisited` 0))

(fn `LeaveBehavior`
  (bind (_x _y) (`KismetMathLibrary.BreakVector2D` (`self.TargetLoc`)))
  (bind _returnvalue (`KismetMathLibrary.DegAtan2` (`self.MonsterY`) (`self.MonsterX`)))
  (if (== (`self.TargetLoc`) (0.0 0.0) :`ErrorTolerance` 1.0)
    (set `self.TargetLoc` (`KismetMathLibrary.MakeVector2D` (* 475.0 (`KismetMathLibrary.DegCos` _returnvalue)) (* 475.0 (`KismetMathLibrary.DegSin` _returnvalue))))
    (else
      (`self.MoveMonsterTowardsLocation` 0.3 _x _y)
      (if (>= (`KismetMathLibrary.Sqrt` (+ (`KismetMathLibrary.Square` (`self.MonsterX`)) (`KismetMathLibrary.Square` (`self.MonsterY`)))) 420.0)
        (set `self.MonsterPresent?` false)
        (`KismetSystemLibrary.PrintString` "monsta has left the building")
        (`self.BringMonsterBack`)))))

(fn `LeftFlareMovement`
  (bind (_x _y) (`KismetMathLibrary.BreakVector2D` (`self.LeftFlareLoc`)))
  (set `self.LeftFlareLoc` (`KismetMathLibrary.MakeVector2D` (- _x 0.3) (- _y 0.0)))
  (if (< _x -400.0)
    (set `self.LeftFlareLoc` (0.0 0.0))
    (set `self.TargetLoc` (0.0 0.0))
    (set `self.AIState` "Leave")))

(fn `LoiterBehavior`
  (params (MinimumDistance :type "Float (double-precision)"))
  (bind _targetloc (`self.TargetLoc`))
  (bind _loiterpointsvisited (`self.LoiterPointsVisited`))
  (bind (_x _y) (`KismetMathLibrary.BreakVector2D` (`self.TargetLoc`)))
  (bind _returnvalue (+ MinimumDistance (`KismetMathLibrary.RandomFloatInRange` 0.0 20.0)))
  (bind _returnvalue_2 (+ (`KismetMathLibrary.DegAtan2` (`self.MonsterY`) (`self.MonsterX`)) (`KismetMathLibrary.RandomFloatInRange` -15.0 15.0)))
  (if (or (== _targetloc (0.0 0.0)) (== _targetloc (`KismetMathLibrary.MakeVector2D` (`self.MonsterX`) (`self.MonsterY`)) :`ErrorTolerance` 1.0))
    (set `self.TargetLoc` (`KismetMathLibrary.MakeVector2D` (* _returnvalue (`KismetMathLibrary.DegCos` _returnvalue_2)) (* _returnvalue (`KismetMathLibrary.DegSin` _returnvalue_2))))
    (if (> _loiterpointsvisited (`KismetMathLibrary.RandomIntegerInRange` 1 2))
      (set `self.LoiterPointsVisited` 0)
      (set `self.TargetLoc` (0.0 0.0))
      (bind _output_get (set `self.StateSelector` (`KismetMathLibrary.RandomIntegerInRange` 0 100)))
      (if (< _output_get 15)
        (set `self.AIState` "Inspect") ; 15% chance to inspect
        (elif (< _output_get 25)
          (set `self.AIState` "Fake Attack") ; 10% chance to fake attack
          (else
            (set `self.AIState` "Attack") ; 75% chance to attack
          )))
      (else
        (`/Engine/EditorBlueprintResources/StandardMacros.IncrementInt` _loiterpointsvisited)))
    (else
      (`self.MoveMonsterTowardsLocation` 0.25 _x _y))))

(fn `MoveMonsterTowardsLocation`
  (params (Speed :type "Float (double-precision)") (TargetX :type "Float (double-precision)") (TargetY :type "Float (double-precision)"))
  (bind _returnvalue (* -1 Speed))
  (bind _returnvalue_2 (- (`self.MonsterY`) TargetY))
  (bind _returnvalue_3 (- (`self.MonsterX`) TargetX))
  (bind _returnvalue_4 (`KismetMathLibrary.FMax` (`KismetMathLibrary.Abs` _returnvalue_2) (`KismetMathLibrary.Abs` _returnvalue_3)))
  (set `self.MonsterY` (+ (`self.MonsterY`) (* (/ _returnvalue_2 _returnvalue_4) _returnvalue)))
  (set `self.MonsterX` (+ (* _returnvalue (/ _returnvalue_3 _returnvalue_4)) (`self.MonsterX`)))
  (return))

(fn `RightFlareMovement`
  (bind (_x _y) (`KismetMathLibrary.BreakVector2D` (`self.RightFlareLoc`)))
  (set `self.RightFlareLoc` (`KismetMathLibrary.MakeVector2D` (+ _x 0.3) (- _y 0.0)))
  (if (> _x 400.0)
    (set `self.RightFlareLoc` (0.0 0.0))
    (set `self.TargetLoc` (0.0 0.0))
    (set `self.AIState` "Leave")))

(fn `SetAudioControllerLocation`
  (`SceneComponent.K2_SetWorldLocation` (`/Game/Blueprints/Controllers/MonsterAudioController.DefaultSceneRoot` (`self.MonsterAudioController`)) (`KismetMathLibrary.MakeVector` (* (`self.MonsterX`) -30.0) (+ (* (`self.MonsterY`) -40.0) 1650.0) 700.0) false false))

(fn `UserConstructionScript`)