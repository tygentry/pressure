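; Sticky note actor that toggles between its place in the world and a readable spot in front of the player camera.
; BeginPlay applies the note's text material and caches its starting transform.
; Each UpdateDisplay call either restores that transform or moves the note once to KillMeGod's camera-relative point, offset by XPos and YPos, rotated back toward the viewer.
; The older widget-removal branch is disconnected.
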(event `self.ReceiveBeginPlay`
  (bind _defaultsceneroot (`self.DefaultSceneRoot`))
  (`PrimitiveComponent.SetMaterial` (`self.Note`) 0 (`self.StickyNoteText`))
  (set `self.InitialLocation` (`SceneComponent.K2_GetComponentLocation` _defaultsceneroot))
  (set `self.InitialRotation` (`SceneComponent.K2_GetComponentRotation` _defaultsceneroot)))

(event `UpdateDisplay`
  (bind _rootcomponent (`Actor.RootComponent` (`GameplayStatics.GetPlayerCameraManager` 0)))
  (bind _returnvalue (`SceneComponent.K2_GetComponentLocation` _rootcomponent))
  (if (`self.OnViewport`)
    ;[1 1 1] Removing Sticky Note from viewport upon secondary trigger
    (set `self.OnViewport` false)
    (`SceneComponent.K2_SetWorldLocationAndRotation` (`self.DefaultSceneRoot`) (`self.InitialLocation`) (`self.InitialRotation`) false false)
    (else
      ;[1 1 1] Adding Sticky Note to viewport
      (set `self.OnViewport` true)
      (bind _vector (`self.KillMeGod`))
      (`SceneComponent.K2_SetWorldLocationAndRotation` (`self.DefaultSceneRoot`) _vector (`KismetMathLibrary.FindLookAtRotation` _returnvalue (+ _returnvalue (* (`KismetMathLibrary.Normal` (`SceneComponent.GetForwardVector` _rootcomponent)) -30.0))) false false))))

(fn `KillMeGod`
  (returns (Vector :type "Vector Structure"))
  (bind _rootcomponent (`Actor.RootComponent` (`GameplayStatics.GetPlayerCameraManager` 0)))
  (return (+ (+ (+ (`SceneComponent.K2_GetComponentLocation` _rootcomponent) (* (`KismetMathLibrary.Normal` (`SceneComponent.GetForwardVector` _rootcomponent)) 45.0)) (* (`KismetMathLibrary.Normal` (`SceneComponent.GetRightVector` _rootcomponent)) (`self.XPos`))) (* (`KismetMathLibrary.Normal` (`SceneComponent.GetUpVector` _rootcomponent)) (`self.YPos`)))))

(fn `UserConstructionScript`
  (`parent.UserConstructionScript`))