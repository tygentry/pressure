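; SwitchComponent is a Blueprint switch that holds an on/off state in the SwitchState boolean.
; OnFlick plays SwitchFlipCue at the DefaultSceneRoot location and inverts the state, while OnFlickSoundless inverts it silently.
; Both events repeat the same branch-and-set toggle, and nothing in this Blueprint broadcasts or reacts to the change.
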(event `OnFlickSoundless`
  (if (`self.SwitchState`)
    (set `self.SwitchState` false)
    (else
      (set `self.SwitchState` true))))

(event `OnFlick`
  (`GameplayStatics.PlaySoundAtLocation` "/Game/SFX/SwitchFlipCue.SwitchFlipCue" (`SceneComponent.K2_GetComponentLocation` (`self.DefaultSceneRoot`)) (struct) 1.0 1.0 0.0 null null null)
  (if (`self.SwitchState`)
    (set `self.SwitchState` false)
    (else
      (set `self.SwitchState` true))))

(fn `UserConstructionScript`
  (`parent.UserConstructionScript`))