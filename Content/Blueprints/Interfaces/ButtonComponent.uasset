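; ButtonComponent is a Blueprint for a pressable button that tracks whether it is held and whether it can be pressed.
; ButtonPressed sets the held flag, while ButtonReleased clears it and blocks pressing until a configurable delay between presses has elapsed.
; The indent animation and press sound logic are present but never run.
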(event `ButtonPressed`
  (set `self.IsBeingHeld` true))

(event `ButtonReleased`
  (set `self.IsBeingHeld` false)
  (set `self.CanBePressed` false)
  (`KismetSystemLibrary.Delay` (`self.DelayBetweenPresses`))
  (set `self.CanBePressed` true))

(fn `UserConstructionScript`
  (`parent.UserConstructionScript`))