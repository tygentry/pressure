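; Fire hazard placed in a room that burns the first-person character and keeps that room's fire count on the SubDisplayInterface actor current.
; Overlap runs BurnTimeline to call Burn on the character, and leaving stops it and starts a looping BurnRegen timer on them.
; ChangeIntensity scales particles and audio volume.
; At zero it shuts off effects and collision, decrements the count added on BeginPlay, and destroys itself.
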(event `self.ReceiveBeginPlay`
  (`FXSystemComponent.SetFloatParameter` (`self.ParticleSystem`) "FireIntensity" 1.0)
  (`KismetSystemLibrary.Delay` 0.2)
  (bind _outactors (`GameplayStatics.GetAllActorsOfClass` "/Game/Blueprints/Interfaces/Bridge/SubDisplayInterface.SubDisplayInterface_C"))
  (bind _output (`|GetArrayItem` _outactors))
  (for _array_element (`/Game/Blueprints/Interfaces/Bridge/SubDisplayInterface.RoomNames` _output)
    (if (`KismetStringLibrary.EqualEqual_StrStr` _array_element (`self.Room`))
      (bind _fires (`/Game/Blueprints/Interfaces/Bridge/SubDisplayInterface.Fires` _output))
      (`BlueprintMapLibrary.Map_Add` _fires _array_element (+ (`BlueprintMapLibrary.Map_Find` _fires _array_element) 1)))))

(event `self.ReceiveActorBeginOverlap`
  (params (OtherActor :type "Actor Object Reference"))
  (bind _asfirst_person_character (cast `/Game/FirstPersonBP/Blueprints/FirstPersonCharacter` OtherActor))
  (`Timeline|BurnTimeline` :!via `PlayFromStart` :!label _label
    (:`BurnTrack`
      (`/Game/FirstPersonBP/Blueprints/FirstPersonCharacter.Burn` _asfirst_person_character))))

(event `self.ReceiveActorEndOverlap`
  (params (OtherActor :type "Actor Object Reference"))
  (bind _asfirst_person_character (cast `/Game/FirstPersonBP/Blueprints/FirstPersonCharacter` OtherActor))
  (`KismetSystemLibrary.K2_SetTimer` _asfirst_person_character "BurnRegen" 1.0 true)
  (goto _label :!via `Stop`))

(event `ChangeIntensity`
  (params (Delta :type "Float (double-precision)"))
  (bind _output_get (set `self.Intensity` (+ Delta (`self.Intensity`))))
  (bind _returnvalue (/ _output_get 100.0))
  (`FXSystemComponent.SetFloatParameter` (`self.ParticleSystem`) "FireIntensity" _returnvalue)
  (`AudioComponent.SetVolumeMultiplier` (`self.Audio`) _returnvalue)
  (if (<= _returnvalue 0.0)
    (`ActorComponent.SetActive` (`self.ParticleSystem`) false false)
    (`AudioComponent.Stop` (`self.Audio`))
    (`PrimitiveComponent.SetCollisionEnabled` (`self.Collision`) "NoCollision")
    (`KismetSystemLibrary.Delay` 1.0)
    (bind _outactors (`GameplayStatics.GetAllActorsOfClass` "/Game/Blueprints/Interfaces/Bridge/SubDisplayInterface.SubDisplayInterface_C"))
    (bind _output (`|GetArrayItem` _outactors))
    (for _array_element (`/Game/Blueprints/Interfaces/Bridge/SubDisplayInterface.RoomNames` _output)
      (if (`KismetStringLibrary.EqualEqual_StrStr` _array_element (`self.Room`))
        (bind _fires (`/Game/Blueprints/Interfaces/Bridge/SubDisplayInterface.Fires` _output))
        (`BlueprintMapLibrary.Map_Add` _fires _array_element (+ (`BlueprintMapLibrary.Map_Find` _fires _array_element) -1))))
    (`self.K2_DestroyActor`)))

(fn `UserConstructionScript`)