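; Alert light Blueprint that flashes a point light when its AlertFlash event fires.
; Four chained timelines (Up, Down2, Up2, Down3) each write a float track, named DoorRotation, to the light's intensity, apparently giving two rise-and-fall pulses.
; Each timeline starts the next on Finished; the first uses Play, while the others use PlayFromStart.
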(event `AlertFlash`
  (bind (_direction _door_rotation) (`Timeline|AlertLightUp`)
    (:`Update`
      (`LightComponent.SetIntensity` (`self.PointLight`) _door_rotation))
    (:`Finished`
      (bind (_direction_2 _door_rotation_2) (`Timeline|AlertLightDown2` :!via `PlayFromStart`)
        (:`Update`
          (`LightComponent.SetIntensity` (`self.PointLight`) _door_rotation_2))
        (:`Finished`
          (bind (_direction_3 _door_rotation_3) (`Timeline|AlertLightUp2` :!via `PlayFromStart`)
            (:`Update`
              (`LightComponent.SetIntensity` (`self.PointLight`) _door_rotation_3))
            (:`Finished`
              (bind (_direction_4 _door_rotation_4) (`Timeline|AlertLightDown3` :!via `PlayFromStart`)
                (:`Update`
                  (`LightComponent.SetIntensity` (`self.PointLight`) _door_rotation_4))))))))))

(fn `UserConstructionScript`)