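; Receptacle actor that holds a usable object at a configurable offset and rotation, optionally starting with one placed at BeginPlay.
; Grabbing makes the first-person player drop the usable, disables its physics, snaps it into place, links both actors and plays audio.
; Save loading reuses the grab path without the player drop or sound.
; Release clears the usable's receptacle link and the holding flag, keeping the most recently held reference.
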(event `self.ReceiveBeginPlay`
  (bind _initialheldusable (`self.InitialHeldUsable`))
  (bind _staticmesh (`/Game/Blueprints/Usables/Usable.StaticMesh` _initialheldusable))
  ;[1 1 1] Setup, putting usable in receptacle if needed
  (`/Engine/EditorBlueprintResources/StandardMacros.IsValid` _initialheldusable
    (:`Is Valid`
      (`PrimitiveComponent.SetSimulatePhysics` _staticmesh false)
      (`SceneComponent.K2_SetWorldLocationAndRotation` _staticmesh (+ (`SceneComponent.K2_GetComponentLocation` (`self.DefaultSceneRoot`)) (`self.HeldObjectOffset`)) (`self.HeldObjectRotation`) false false)
      (set `self.IsHoldingObject?` true)
      (set `self.MostRecentlyHeldObject` (`self.InitialHeldUsable`))
      (set `/Game/Blueprints/Usables/Usable.CurrentReceptacle` self (`self.MostRecentlyHeldObject`)))))

(event `GrabUsable`
  (params (ToGrab :type "/Game/Blueprints/Usables/Usable Object Reference") (`LoadingSave?` :type Boolean))
  (bind _staticmesh (`/Game/Blueprints/Usables/Usable.StaticMesh` ToGrab))
  ;[1 1 1] Grab
  (if (not `LoadingSave?`)
    (bind _asfirst_person_character (cast `/Game/FirstPersonBP/Blueprints/FirstPersonCharacter` (`GameplayStatics.GetPlayerCharacter` 0)))
    (`/Game/FirstPersonBP/Blueprints/FirstPersonCharacter.DropUsable` _asfirst_person_character))
  (`PrimitiveComponent.SetSimulatePhysics` _staticmesh false)
  (`SceneComponent.K2_SetWorldLocationAndRotation` _staticmesh (+ (`SceneComponent.K2_GetComponentLocation` (`self.DefaultSceneRoot`)) (`self.HeldObjectOffset`)) (`self.HeldObjectRotation`) false false)
  (set `self.IsHoldingObject?` true)
  (set `self.MostRecentlyHeldObject` ToGrab)
  (set `/Game/Blueprints/Usables/Usable.CurrentReceptacle` self (`self.MostRecentlyHeldObject`))
  (if (not `LoadingSave?`)
    (`AudioComponent.Play` (`self.Audio`) 0.0)))

(event `ReleaseUsable`
  ;[1 1 1] Release
  (set `/Game/Blueprints/Usables/Usable.CurrentReceptacle` null (`self.MostRecentlyHeldObject`))
  (set `self.IsHoldingObject?` false))

(fn `UserConstructionScript`)