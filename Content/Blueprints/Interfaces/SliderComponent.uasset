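; Slider actor with a Handle that can be dragged with the mouse along the root's right vector, exposing its offset as DeltaY.
; BeginPlay waits briefly, caches the handle's base position and applies InitialDeltaY.
; Hold stores the cursor-to-handle offset; Tick then moves the handle, clamped to ±MaximumDeltaY, until LetGo.
; Mouse position comes from a Visibility cursor trace projected onto that axis by dot product.
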(event `self.ReceiveBeginPlay`
  (bind _initialdeltay (`self.InitialDeltaY`))
  ;[1 1 1] Setup
  (`parent.ReceiveBeginPlay`)
  (`KismetSystemLibrary.Delay` 0.2)
  (set `self.BaseHandlePos` (`SceneComponent.K2_GetComponentLocation` (`self.Handle`)))
  (set `self.DeltaY` _initialdeltay)
  (`self.SetHandleY` _initialdeltay))

(event `Hold`
  ;[1 1 1] Hold and Let Go Events
  (set `self.IsHeld` true)
  (bind _y (`self.GetMouseY`))
  (bind _y_2 (`self.GetHandleY`))
  (set `self.MouseOffset` (- _y _y_2)))

(event `self.ReceiveTick`
  (params (DeltaSeconds :type "Float (single-precision)"))
  (bind _maximumdeltay (`self.MaximumDeltaY`))
  (bind _maximumdeltay_2 (`self.MaximumDeltaY`))
  (bind _returnvalue (* -1 (`self.MaximumDeltaY`)))
  ;[1 1 1] Event Tick, update handle position
  (if (`self.IsHeld`)
    (bind _y (`self.GetMouseY`))
    (bind _returnvalue_2 (- _y (`self.MouseOffset`)))
    (if (> _returnvalue_2 _maximumdeltay)
      (`self.SetHandleY` _maximumdeltay_2)
      (set `self.DeltaY` _maximumdeltay_2)
      (elif (< _returnvalue_2 (* -1 _maximumdeltay))
        (`self.SetHandleY` _returnvalue)
        (set `self.DeltaY` _returnvalue)
        (else
          (`self.SetHandleY` _returnvalue_2)
          (set `self.DeltaY` _returnvalue_2))))))

(event `Let Go`
  ;[1 1 1] Hold and Let Go Events
  (set `self.IsHeld` false))

(fn `GetHandleY`
  (returns (Y :type "Float (double-precision)"))
  (return (`KismetMathLibrary.Dot_VectorVector` (`KismetMathLibrary.Normal` (`SceneComponent.GetRightVector` (`self.DefaultSceneRoot`))) (- (`SceneComponent.K2_GetComponentLocation` (`self.Handle`)) (`self.BaseHandlePos`)))))

(fn `GetMouseY`
  (returns (Y :type "Float (double-precision)"))
  (return (`KismetMathLibrary.Dot_VectorVector` (`KismetMathLibrary.Normal` (`SceneComponent.GetRightVector` (`self.DefaultSceneRoot`))) (- (`.Location` (`GameplayStatics.BreakHitResult` (`PlayerController.GetHitResultUnderCursorByChannel` (`GameplayStatics.GetPlayerController` 0) "TraceTypeQuery1" true))) (`SceneComponent.K2_GetComponentLocation` (`self.DefaultSceneRoot`))))))

(fn `SetHandleY`
  (params (Y :type "Float (double-precision)"))
  (`SceneComponent.K2_SetWorldLocation` (`self.Handle`) (+ (* (`KismetMathLibrary.Normal` (`SceneComponent.GetRightVector` (`self.DefaultSceneRoot`))) Y) (`self.BaseHandlePos`)) false false))

(fn `UserConstructionScript`
  (`parent.UserConstructionScript`))