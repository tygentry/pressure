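; WireConnectComponent is an actor that acts as a connection point for a wire the player carries.
; On overlap with a WireComponent that has no physics, while unconnected, it stores that wire, calls Connect on it with itself, and makes the first-person player character drop the wire.
; Its DropWire function clears the connected flag so it can accept a wire again.
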(event `self.ReceiveActorBeginOverlap`
  (params (OtherActor :type "Actor Object Reference"))
  (if (not (`self.IsConnected`))
    (bind _aswire_component (cast `/Game/Blueprints/Interfaces/WireComponent` OtherActor))
    (if (not (`/Game/Blueprints/Interfaces/WireComponent.HasPhysics` _aswire_component))
      (set `self.ConnectedWire` _aswire_component)
      (set `self.IsConnected` true)
      (`/Game/Blueprints/Interfaces/WireComponent.Connect` _aswire_component self)
      (bind _asfirst_person_character (cast `/Game/FirstPersonBP/Blueprints/FirstPersonCharacter` (`GameplayStatics.GetPlayerCharacter` 0)))
      (`/Game/FirstPersonBP/Blueprints/FirstPersonCharacter.DropWire` _asfirst_person_character))))

(fn `DropWire`
  (set `self.IsConnected` false))

(fn `UserConstructionScript`)