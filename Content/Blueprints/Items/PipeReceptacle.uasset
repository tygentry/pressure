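; Socket actor in a pipe water-flow puzzle that holds, rotates and drops pipe pieces.
; It seats an optional start pipe on BeginPlay and accepts hit straight pipes only at matching scale.
; CheckWaterFlow recurses through IncomingConnections, switching water effects where the line breaks, with tag lookups for the origin T-pipe branches and feed pipe.
; Placing a pipe stops incoming flow; orientation-correctness logic is unwired.
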(event `self.ReceiveTick`
  (params (DeltaSeconds :type "Float (single-precision)"))
  ;[1 1 1] Tracking if current PipeState is correct
)

(event `self.ReceiveBeginPlay`
  (bind _startpipe (`self.StartPipe`))
  ;[1 1 1] Setting up Start Variables and Pipes
  (`parent.ReceiveBeginPlay`)
  (if (`KismetSystemLibrary.IsValid` _startpipe)
    (if (`KismetMathLibrary.ClassIsChildOf` (`GameplayStatics.GetObjectClass` _startpipe) "/Game/Blueprints/Items/StraightPipe1.StraightPipe1_C")
      (set `self.StraightPipeSize` (.y (`SceneComponent.K2_GetComponentScale` (`/Game/Blueprints/Items/Item.DefaultSceneRoot` _startpipe)))))
    (`self.Hold Start Pipe`)
    (set `self.KnockOffRequirement` (`KismetMathLibrary.RandomFloatInRange` 10.0 100.0))))

(event `self.ReceiveHit`
  (params (MyComp :type "PrimitiveComponent Object Reference") (Other :type "Actor Object Reference") (OtherComp :type "PrimitiveComponent Object Reference") (bSelfMoved :type Boolean) (HitLocation :type "Vector Structure") (HitNormal :type "Vector Structure") (NormalImpulse :type "Vector Structure") (Hit :type "HitResult Structure (by ref)"))
  ;[1 1 1] Placing Pipe
  (if (not (`self.isGrabbingObject`))
    (bind _asstraight_pipe_1 (cast `/Game/Blueprints/Items/StraightPipe1` Other)
      (:`then`
        (if (== (`self.StraightPipeSize`) (.y (`SceneComponent.K2_GetComponentScale` (`/Game/Blueprints/Items/Item.DefaultSceneRoot` _asstraight_pipe_1))))
          (`parent.ReceiveHit` MyComp Other OtherComp bSelfMoved HitLocation HitNormal NormalImpulse Hit :!label _label)
          (`self.StopWaterFlowOnIncomingConnections`)))
      (:`CastFailed`
        (goto _label)))))

(event `InitiateFlowOnIncomingPipes`
  (for _array_element (`self.IncomingConnections`)
    (bind _aspipe (cast `/Game/Blueprints/Items/Pipe` (`/Game/Blueprints/Items/ItemReceptacle.MostRecentGrabbedObject` _array_element))
      (:`then`
        (`/Game/Blueprints/Items/Pipe.WaterFlowingOn` _aspipe))
      (:`CastFailed`
        (`KismetSystemLibrary.PrintString` "fuck you lmaaaoaooaoa" true true (struct :`R` 1.0 :`G` 0.892658 :`B` 0.0625 :`A` 1.0))))))

(fn `Check Water Flow`
  (returns (`HasFlow?` :type Boolean) (`SourceReceptacleHasFlow?` :type Boolean))
  (bind _incomingconnections (`self.IncomingConnections`))
  (if (== (`KismetArrayLibrary.Array_Length` _incomingconnections) 0)
    (if (`self.isGrabbingObject`)
      ;[1 1 1] Cause water flow on the t-pipe at the origin
      (bind _outactors (`GameplayStatics.GetAllActorsOfClassWithTag` "PipeReceptacle_C" "UpwardsPathBeginning"))
      (bind _aspipe_receptacle (cast `/Game/Blueprints/Items/PipeReceptacle` (`|GetArrayItem` _outactors)))
      (if (not (`/Game/Blueprints/Items/ItemReceptacle.isGrabbingObject` _aspipe_receptacle))
        (bind _ast_pipe (cast `/Game/Blueprints/Items/T-Pipe` (`self.MostRecentGrabbedObject`)))
        (`/Game/Blueprints/Items/T-Pipe.UpwardsWaterFlowOn` _ast_pipe))
      (bind _outactors_2 (`GameplayStatics.GetAllActorsOfClassWithTag` "PipeReceptacle_C" "LeftwardsPathBeginning"))
      (bind _aspipe_receptacle_2 (cast `/Game/Blueprints/Items/PipeReceptacle` (`|GetArrayItem` _outactors_2)))
      (if (not (`/Game/Blueprints/Items/ItemReceptacle.isGrabbingObject` _aspipe_receptacle_2))
        (bind _ast_pipe_2 (cast `/Game/Blueprints/Items/T-Pipe` (`self.MostRecentGrabbedObject`)))
        (`/Game/Blueprints/Items/T-Pipe.LeftWaterFlowOn` _ast_pipe_2))
      (return true true)
      (else
        ;[1 1 1] Cause water flow on the noninteractive straight pipe flowing into the system
        (bind _outactors_3 (`GameplayStatics.GetAllActorsOfClassWithTag` "/Game/Blueprints/Items/StraightPipe1.StraightPipe1_C" "Flows To Origin"))
        (for _array_element _outactors_3
          (bind _asstraight_pipe_1 (cast `/Game/Blueprints/Items/StraightPipe1` _array_element))
          (`/Game/Blueprints/Items/Pipe.WaterFlowingOn` _asstraight_pipe_1))))
    (else
      ;[1 1 1] Cause water flow normally
      (for _array_element_2 _incomingconnections
        (bind _hasflow_ (`self.Check Water Flow` _array_element_2))
        (if _hasflow_
          (if (`self.isGrabbingObject`)
            (return true true)
            (else
              (`self.InitiateFlowOnIncomingPipes`)
              (return false true)))))
      (bind _aspipe (cast `/Game/Blueprints/Items/Pipe` (`self.MostRecentGrabbedObject`)))
      (`/Game/Blueprints/Items/Pipe.WaterFlowingOff` _aspipe)
      (return false false))))

(fn `Drop Pipe`
  (params (Impulse :type "Vector Structure"))
  (bind _mostrecentgrabbedobject (`self.MostRecentGrabbedObject`))
  (if (`self.isGrabbingObject`)
    (bind _aspipe (cast `/Game/Blueprints/Items/Pipe` _mostrecentgrabbedobject))
    (`/Game/Blueprints/Items/Pipe.WaterFlowingOff` _aspipe)
    (`self.ReleaseObject`)
    (`PrimitiveComponent.AddImpulse` (`/Game/Blueprints/Items/Item.StaticMesh` _mostrecentgrabbedobject) Impulse "None" false)))

(fn `Hold Start Pipe`
  (bind _startpipe (`self.StartPipe`))
  (bind _staticmesh (`/Game/Blueprints/Items/Item.StaticMesh` _startpipe))
  (bind _staticmesh_2 (`/Game/Blueprints/Items/Item.StaticMesh` _startpipe))
  (set `self.RecievedObjectOffset` (- (`SceneComponent.K2_GetComponentLocation` _staticmesh) (`SceneComponent.K2_GetComponentLocation` (`self.DefaultSceneRoot`))))
  (set `self.RecievedObjectRotation` (`SceneComponent.K2_GetComponentRotation` _staticmesh))
  (`PrimitiveComponent.SetSimulatePhysics` _staticmesh_2 false)
  (`SceneComponent.K2_SetWorldLocationAndRotation` _staticmesh_2 (+ (`SceneComponent.K2_GetComponentLocation` (`self.DefaultSceneRoot`)) (`self.RecievedObjectOffset`)) (`self.RecievedObjectRotation`) false true)
  (set `/Game/Blueprints/Items/Item.IsInReceptacle` true _startpipe)
  (`/Game/Blueprints/Items/Item.Set Most Recent Receptacle` _startpipe self) ; cant do this manually from within this blueprint for whatever reason
  (if (not (`self.GrabbedObjectCanBeTaken`))
    (set `/Game/Blueprints/Items/Item.CanBeHeld` false _startpipe))
  (set `self.MostRecentGrabbedObject` _startpipe)
  (set `self.isGrabbingObject` true)
  (set `self.GrabbableObjectsSuperclass` (`GameplayStatics.GetObjectClass` (`self.StartPipe`))))

(fn `Rotate`
  (bind _pipestate (`self.PipeState`))
  (if (`self.isGrabbingObject`)
    (`SceneComponent.K2_AddWorldRotation` (`/Game/Blueprints/Items/Item.StaticMesh` (`self.MostRecentGrabbedObject`)) (struct :`Roll` 90.0) false false)
    (`/Engine/EditorBlueprintResources/StandardMacros.IncrementInt` _pipestate
      (:`  `
        (if (== _pipestate 5)
          (set `self.PipeState` 1))))))

(fn `StopWaterFlowOnIncomingConnections`
  (bind _incomingconnections (`self.IncomingConnections`))
  (bind _mostrecentgrabbedobject (`/Game/Blueprints/Items/ItemReceptacle.MostRecentGrabbedObject` (`|GetArrayItem` _incomingconnections)))
  (if (> (`KismetArrayLibrary.Array_Length` _incomingconnections) 0)
    (if (== (`GameplayStatics.GetObjectClass` _mostrecentgrabbedobject) "/Game/Blueprints/Items/T-Pipe.T-Pipe_C")
      (bind _ast_pipe (cast `/Game/Blueprints/Items/T-Pipe` _mostrecentgrabbedobject))
      (if (`self.ActorHasTag` self "LeftwardsPathBeginning")
        (`/Game/Blueprints/Items/T-Pipe.LeftWaterFlowOff` _ast_pipe)
        (elif (`self.ActorHasTag` self "UpwardsPathBeginning")
          (`/Game/Blueprints/Items/T-Pipe.UpwardsWaterFlowOff` _ast_pipe)
          (else
            (`KismetSystemLibrary.PrintString` "issue in pipe receptacle stop water flowing function"))))
      (else
        ;[1 1 1] Normal flow stopping
        (for _array_element (`self.IncomingConnections`)
          (if (`/Game/Blueprints/Items/ItemReceptacle.isGrabbingObject` _array_element)
            (bind _aspipe (cast `/Game/Blueprints/Items/Pipe` (`/Game/Blueprints/Items/ItemReceptacle.MostRecentGrabbedObject` _array_element)))
            (`/Game/Blueprints/Items/Pipe.WaterFlowingOff` _aspipe)))))
    (else
      ;[1 1 1] Stop water flow on the noninteractive straight pipe flowing into the system
      (bind _outactors (`GameplayStatics.GetAllActorsOfClassWithTag` "/Game/Blueprints/Items/StraightPipe1.StraightPipe1_C" "Flows To Origin"))
      (for _array_element_2 _outactors
        (bind _asstraight_pipe_1 (cast `/Game/Blueprints/Items/StraightPipe1` _array_element_2))
        (`/Game/Blueprints/Items/Pipe.WaterFlowingOff` _asstraight_pipe_1)))))

(fn `UserConstructionScript`
  (`parent.UserConstructionScript`))