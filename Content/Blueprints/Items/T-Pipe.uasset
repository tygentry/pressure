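; T-Pipe item Blueprint that shows water flowing out of a T-junction pipe, extending a parent class's water-flow events.
; Upwards and left flow events each call the parent's on/off handler and activate or deactivate their own particle system (Z and X).
; The general water-off event shuts off both directions, while the general water-on event is empty.
; An unconnected debug print says the T pipe can't do that yet.
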(event `self.WaterFlowingOff`
  (`self.LeftWaterFlowOff`)
  (`self.UpwardsWaterFlowOff`))

(event `self.ReceiveBeginPlay`
  (`parent.ReceiveBeginPlay`))

(event `self.WaterFlowingOn`)

(event `UpwardsWaterFlowOn`
  (`parent.WaterFlowingOn`)
  (`ActorComponent.Activate` (`self.-ZParticleSystem`) false))

(event `UpwardsWaterFlowOff`
  (`parent.WaterFlowingOff`)
  (`ActorComponent.Deactivate` (`self.-ZParticleSystem`)))

(event `LeftWaterFlowOn`
  (`parent.WaterFlowingOn`)
  (`ActorComponent.Activate` (`self.+XParticleSystem1`) false))

(event `LeftWaterFlowOff`
  (`parent.WaterFlowingOff`)
  (`ActorComponent.Deactivate` (`self.+XParticleSystem1`)))

(fn `UserConstructionScript`
  (`parent.UserConstructionScript`))