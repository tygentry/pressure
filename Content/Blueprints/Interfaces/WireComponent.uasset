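; Draggable wire for an interface actor, with a cable attached to a cylinder end that the player plugs into sockets.
; PickUp disables physics and releases any connected socket, while DropWire stops following and re-enables physics.
; While held, Tick moves the end to the cursor trace hit, clamped in Y/Z by Limits and locked to the Cube's X.
; Connect stores the socket and snaps the end onto it.
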(event `self.ReceiveBeginPlay`
  ;[1 1 1] Attaching initial wire to end
  (`parent.ReceiveBeginPlay`)
  (bind _asinterface (cast `/Game/Blueprints/Interfaces/Interface` (`self.GetParentActor`)))
  (set `self.Interface` _asinterface)
  (`CableComponent.SetAttachEndToComponent` (`self.Cable`) (`self.Cylinder`) "None"))

(event `PickUp`
  ;[1 1 1] Setting when player has clicked on wire
  (set `self.FollowMouse` true)
  (`PrimitiveComponent.SetSimulatePhysics` (`self.Cylinder`) false)
  (set `self.HasPhysics` false)
  (if (`self.IsConnected`)
    (`/Game/Blueprints/Interfaces/WireConnectComponent.DropWire` (`self.ConnectedSocket`))
    (set `self.IsConnected` false)))

(event `DropWire`
  ;[1 1 1] Stopping wire from following
  (set `self.FollowMouse` false)
  (`PrimitiveComponent.SetSimulatePhysics` (`self.Cylinder`) true)
  (set `self.HasPhysics` true))

(event `self.ReceiveTick`
  (params (DeltaSeconds :type "Float (single-precision)"))
  ;[1 1 1] Setting wire end to follow player mouse
  (if (`self.FollowMouse`)
    (`self.FollowMouseInBounds`)))

(fn `Connect`
  (params (Connect :type "/Game/Blueprints/Interfaces/WireConnectComponent Object Reference"))
  (set `self.IsConnected` true)
  (bind _output_get (set `self.ConnectedSocket` Connect))
  (set `self.FollowMouse` false)
  (`SceneComponent.K2_SetWorldLocationAndRotation` (`self.Cylinder`) (`SceneComponent.K2_GetComponentLocation` (`/Game/Blueprints/Interfaces/WireConnectComponent.DefaultSceneRoot` _output_get)) (struct :`Yaw` 90.0) false false))

(fn `FollowMouseInBounds`
  (bind _limits (`self.Limits`))
  (bind _returnvalue_x (`KismetMathLibrary.BreakVector` (`SceneComponent.K2_GetComponentLocation` (`self.Cube`))))
  (bind (_output_x _output_y _output_z) (`KismetMathLibrary.BreakVector` (`|GetArrayItem` _limits)))
  (bind (_output_x_2 _output_y_2 _output_z_2) (`KismetMathLibrary.BreakVector` (`|GetArrayItem` _limits 2)))
  (bind (_output_x_3 _output_y_3) (`KismetMathLibrary.BreakVector` (`|GetArrayItem` _limits 3)))
  (bind (_output_x_4 _output_y_4) (`KismetMathLibrary.BreakVector` (`|GetArrayItem` _limits 1)))
  (bind (_bblockinghit _binitialoverlap _time _distance _location) (`GameplayStatics.BreakHitResult` (`PlayerController.GetHitResultUnderCursorByChannel` (`GameplayStatics.GetPlayerController` 0) "TraceTypeQuery1" false)))
  (bind _returnvalue (`KismetMathLibrary.FMin` _output_z (.z _location)))
  (bind _returnvalue_2 (`KismetMathLibrary.FMax` (.z _location) _output_z_2))
  (bind _returnvalue_3 (`KismetMathLibrary.FMin` (.y _location) _output_y_3))
  (bind _returnvalue_4 (`KismetMathLibrary.FMax` (.y _location) _output_y_4))
  (bind _returnvalue_5 (< (`KismetMathLibrary.Abs` (- (.z _location) _output_z)) (`KismetMathLibrary.Abs` (- (.z _location) _output_z_2))))
  (if (< (`KismetMathLibrary.Abs` (- (.y _location) _output_y_4)) (`KismetMathLibrary.Abs` (- (.y _location) _output_y_3)))
    (if _returnvalue_5
      (`SceneComponent.K2_SetWorldLocation` (`self.Cylinder`) (`KismetMathLibrary.MakeVector` _returnvalue_x _returnvalue_4 _returnvalue) false false)
      (else
        (`SceneComponent.K2_SetWorldLocation` (`self.Cylinder`) (`KismetMathLibrary.MakeVector` _returnvalue_x _returnvalue_4 _returnvalue_2) false false)))
    (elif _returnvalue_5
      (`SceneComponent.K2_SetWorldLocation` (`self.Cylinder`) (`KismetMathLibrary.MakeVector` _returnvalue_x _returnvalue_3 _returnvalue) false false)
      (else
        (`SceneComponent.K2_SetWorldLocation` (`self.Cylinder`) (`KismetMathLibrary.MakeVector` _returnvalue_x _returnvalue_3 _returnvalue_2) false false)))))

(fn `UserConstructionScript`
  (`parent.UserConstructionScript`))