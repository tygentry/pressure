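; Usable is a Blueprint for an item that can be used, stopped and checked for whether it can be dropped.
; The use and stop-use events only print placeholder debug strings.
; CheckCanBeDropped runs short Visibility line traces from the static mesh along both directions of its right and up axes.
; Any hit blocks dropping, so the check passes only when all four sides are clear.
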(event `self.ReceiveTick`
  (params (DeltaSeconds :type "Float (single-precision)")))

(event `UseUsable`
  (`KismetSystemLibrary.PrintString` "AAAH"))

(event `StopUsingUsable`
  (`KismetSystemLibrary.PrintString` "ok done"))

(fn `CheckCanBeDropped`
  (returns (`CanBeDropped?` :type Boolean))
  (bind _staticmesh (`self.StaticMesh`))
  (bind _returnvalue (`SceneComponent.K2_GetComponentLocation` _staticmesh))
  (bind _returnvalue_2 (`SceneComponent.GetUpVector` _staticmesh))
  (bind _returnvalue_3 (`SceneComponent.GetRightVector` _staticmesh))
  (bind (_outhit _returnvalue_4) (`KismetSystemLibrary.LineTraceSingle` _returnvalue (+ _returnvalue (* _returnvalue_3 12)) "TraceTypeQuery1"))
  (if _returnvalue_4
    (return false)
    (else
      (bind (_outhit_2 _returnvalue_5) (`KismetSystemLibrary.LineTraceSingle` _returnvalue (+ _returnvalue (* _returnvalue_3 -12)) "TraceTypeQuery1"))
      (if _returnvalue_5
        (return false)
        (else
          (bind (_outhit_3 _returnvalue_6) (`KismetSystemLibrary.LineTraceSingle` _returnvalue (+ _returnvalue (* _returnvalue_2 25)) "TraceTypeQuery1"))
          (if _returnvalue_6
            (return false)
            (else
              (bind (_outhit_4 _returnvalue_7) (`KismetSystemLibrary.LineTraceSingle` _returnvalue (+ _returnvalue (* _returnvalue_2 -25)) "TraceTypeQuery1"))
              (if _returnvalue_7
                (return false)
                (else
                  (return true))))))))))

(fn `UserConstructionScript`)