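; RockMarker is a navigation-support actor representing a rock that a submarine can see or hit, with a list of connected rocks that share its state.
; SeenBySub flags the rock and its connected rocks as Seen.
; RockHitBySub turns off mesh collision on the whole group and moves the meshes far away rather than deleting them, to avoid breaking the display.
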(event `self.ReceiveBeginPlay`)

(event `SeenBySub`
  (set `self.Seen?` true)
  (for _array_element (`self.ConnectedRocks`)
    (set `/Game/Blueprints/NavigationSupport/RockMarker.Seen?` true _array_element)))

(event `self.ReceiveTick`
  (params (DeltaSeconds :type "Float (single-precision)")))

(event `RockHitBySub`
  (bind _staticmesh (`self.StaticMesh`))
  (for _array_element (`self.ConnectedRocks`)
    (bind _asrock_marker (cast `/Game/Blueprints/NavigationSupport/RockMarker` _array_element))
    (bind _staticmesh_2 (`/Game/Blueprints/NavigationSupport/RockMarker.StaticMesh` _asrock_marker))
    (`PrimitiveComponent.SetCollisionEnabled` _staticmesh_2 "NoCollision")
    (`SceneComponent.K2_SetWorldLocation` _staticmesh_2 (5000.0 0.0 0.0) false false))
  (`PrimitiveComponent.SetCollisionEnabled` _staticmesh "NoCollision")
  (`SceneComponent.K2_SetWorldLocation` _staticmesh (3000.0 0.0 0.0) false false) ; move rocks far away instead of deleting to avoid breaking display
)

(fn `UserConstructionScript`)