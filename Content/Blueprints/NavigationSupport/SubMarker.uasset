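; Physics-driven submarine marker for navigation, moving among rock and wall markers and feeding the speed and depth gauges.
; Tick applies thrust from throttle and powered batteries, steers by angular impulses toward the rudder wheel's heading, and resets out-of-bounds positions.
; Hits trigger HitEventController bumps or speed-scaled rock impacts, with a line trace clearing wall-rubbing state.
; ImminentCollisionCheck traces ahead, reporting each unseen rock once.
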(event `UpdateGauges`
  (bind _returnvalue (`PrimitiveComponent.GetPhysicsLinearVelocity` (`self.StaticMesh`) "None"))
  (set `/Game/Blueprints/Interfaces/Non-InteractiveInterfaceComponents/GaugeComponent.TrackedVariable` (`KismetMathLibrary.VSize` _returnvalue) (`self.SubSpeedGauge`))
  (set `/Game/Blueprints/Interfaces/Non-InteractiveInterfaceComponents/GaugeComponent.TrackedVariable` (`self.Depth`) (`self.SubDepthGauge`)))

(event `self.ReceiveTick`
  (params (DeltaSeconds :type "Float (single-precision)"))
  (bind _staticmesh (`self.StaticMesh`))
  (bind _rudderwheel (`self.RudderWheel`))
  ;[1 1 1] Tick Loop
  (`self.OutOfBoundsCheck`)
  (`self.CheckForWallCollision`)
  (`self.UpdateGauges`)
  (set `self.DesiredRotation` (+ (* 30 (/ (`/Game/Blueprints/Interfaces/TurnableComponent.DeltaRot` _rudderwheel) (`/Game/Blueprints/Interfaces/TurnableComponent.MaxDeltaRot` _rudderwheel))) 180.0))
  (bind _output_get (set `self.CurrentRotation` (.yaw (`SceneComponent.K2_GetComponentRotation` (`self.StaticMesh`)))))
  (if (< _output_get 0.0)
    (set `self.CurrentRotation` (+ _output_get 360.0)))
  (if (not (`self.TurningTooFar?`))
    (`PrimitiveComponent.AddForce` _staticmesh (* (* (`KismetMathLibrary.Normal` (`SceneComponent.GetRightVector` _staticmesh)) (* 25 (`self.Throttle`))) (/ (`KismetMathLibrary.Conv_IntToDouble` (`self.PoweredBatteries`)) 3.0)) "None" false) ; add force from throttle
  )
  (`PrimitiveComponent.AddAngularImpulseInRadians` (`self.StaticMesh`) (`KismetMathLibrary.MakeVector` 0.0 0.0 (/ (`/Game/Blueprints/Interfaces/TurnableComponent.DeltaRot` (`self.RudderWheel`)) 2.0)) "None" false) ; turn
  (if (> (`self.DesiredRotation`) (`self.CurrentRotation`))
    (`PrimitiveComponent.AddAngularImpulseInRadians` (`self.StaticMesh`) (`KismetMathLibrary.MakeVector` 0.0 0.0 150.0) "None" false) ; clockwise
    (else
      (`PrimitiveComponent.AddAngularImpulseInRadians` (`self.StaticMesh`) (`KismetMathLibrary.MakeVector` 0.0 0.0 -150.0) "None" false) ; counterclockwise
    ))
  (if (`KismetMathLibrary.NearlyEqual_FloatFloat` (`self.CurrentRotation`) (`self.DesiredRotation`) 1.0)
    (`PrimitiveComponent.SetPhysicsAngularVelocityInDegrees` (`self.StaticMesh`) (0.0 0.0 0.0) false "None")))

(event `self.ReceiveHit`
  (params (MyComp :type "PrimitiveComponent Object Reference") (Other :type "Actor Object Reference") (OtherComp :type "PrimitiveComponent Object Reference") (bSelfMoved :type Boolean) (HitLocation :type "Vector Structure") (HitNormal :type "Vector Structure") (NormalImpulse :type "Vector Structure") (Hit :type "HitResult Structure (by ref)"))
  (bind _returnvalue (`GameplayStatics.GetObjectClass` Other))
  (bind _hiteventcontroller (`self.HitEventController`))
  (bind _staticmesh (`self.StaticMesh`))
  ;[1 1 1] Hitting rock or wall
  (if (`KismetMathLibrary.ClassIsChildOf` _returnvalue "/Game/Blueprints/NavigationSupport/RockMarker.RockMarker_C")
    (bind _asrock_marker (cast `/Game/Blueprints/NavigationSupport/RockMarker` Other))
    (`/Game/Blueprints/NavigationSupport/RockMarker.RockHitBySub` _asrock_marker)
    (bind _returnvalue_2 (`PrimitiveComponent.GetPhysicsLinearVelocity` _staticmesh "None"))
    (`PrimitiveComponent.AddImpulse` _staticmesh (* _returnvalue_2 -0.8) "None" true)
    (bind _returnvalue_3 (`KismetMathLibrary.VSize` _returnvalue_2))
    (if (> _returnvalue_3 20.0)
      (`/Game/Blueprints/Controllers/HitEventController.HitEventRock` _hiteventcontroller (* HitNormal -1) (/ (- (`KismetMathLibrary.FClamp` _returnvalue_3 20.0 120.0) 20.0) 100.0))
      (`KismetSystemLibrary.PrintString` (`KismetStringLibrary.Conv_DoubleToString` _returnvalue_3))
      (else
        (`/Game/Blueprints/Controllers/HitEventController.BumpEvent` _hiteventcontroller)))
    (elif (== _returnvalue "/Game/Blueprints/NavigationSupport/WallMarker.WallMarker_C")
      (if (not (`self.IsRubbingAgainstWall`))
        (`KismetSystemLibrary.PrintString` (`KismetSystemLibrary.GetDisplayName` Other))
        (set `self.IsRubbingAgainstWall` true)
        (set `self.WallCollisionDirection` (* (- HitLocation (`SceneComponent.K2_GetComponentLocation` (`self.StaticMesh`))) 1.5))
        (`/Game/Blueprints/Controllers/HitEventController.BumpEvent` (`self.HitEventController`))))))

(event `OutOfBoundsCheck`
  (bind _staticmesh (`self.StaticMesh`))
  (bind _staticmesh_2 (`self.StaticMesh`))
  (bind _y (.y (`SceneComponent.K2_GetComponentLocation` _staticmesh)))
  ;[1 1 1] Out of bounds check, need to improve
  (if (> (`KismetMathLibrary.Abs` (.x (`SceneComponent.K2_GetComponentLocation` _staticmesh))) 1200.0)
    (`KismetSystemLibrary.PrintString` "Hello")
    (`SceneComponent.K2_SetWorldLocation` _staticmesh (`KismetMathLibrary.MakeVector` 0.0 _y (.z (`SceneComponent.K2_GetComponentLocation` _staticmesh))) false false)
    (`PrimitiveComponent.SetPhysicsLinearVelocity` _staticmesh_2 (0.0 0.0 0.0) false "None" :!label _label)
    (`PrimitiveComponent.SetPhysicsAngularVelocityInDegrees` _staticmesh_2 (0.0 0.0 0.0) false "None")
    (elif (not (< _y 0.0))
      (`SceneComponent.K2_SetWorldLocation` _staticmesh (0.0 -880.0 1300.0) false false)
      (goto _label))))

(event `CheckForWallCollision`
  (bind _returnvalue (`SceneComponent.K2_GetComponentLocation` (`self.StaticMesh`)))
  ;[1 1 1] Check for wall collision
  (if (`self.IsRubbingAgainstWall`)
    (bind (_outhit _returnvalue_2) (`KismetSystemLibrary.LineTraceSingle` :`Start` _returnvalue :`End` (+ _returnvalue (`self.WallCollisionDirection`)) :`TraceChannel` "TraceTypeQuery1" :`DrawDebugType` "ForDuration" :`DrawTime` 1.0))
    (if (not _returnvalue_2)
      (set `self.IsRubbingAgainstWall` false))))

(fn `ImminentCollisionCheck`
  (returns (`CollisionImminent?` :type Boolean))
  (bind _staticmesh (`self.StaticMesh`))
  (bind _returnvalue (+ (`SceneComponent.K2_GetComponentLocation` _staticmesh) (0.0 0.0 50.0)))
  (bind (_outhit _returnvalue_2) (`KismetSystemLibrary.LineTraceSingle` :`Start` _returnvalue :`End` (+ _returnvalue (* (`SceneComponent.GetRightVector` _staticmesh) 850)) :`TraceChannel` "TraceTypeQuery1" :`DrawDebugType` "ForDuration"))
  (if _returnvalue_2
    (bind _asrock_marker (cast `/Game/Blueprints/NavigationSupport/RockMarker` (`.HitActor` (`GameplayStatics.BreakHitResult` _outhit)))
      (:`then`
        (if (`/Game/Blueprints/NavigationSupport/RockMarker.Seen?` _asrock_marker)
          (return false)
          (else
            (`/Game/Blueprints/NavigationSupport/RockMarker.SeenBySub` _asrock_marker)
            (return true))))
      (:`CastFailed`
        _)))
  (return false))

(fn `UserConstructionScript`)