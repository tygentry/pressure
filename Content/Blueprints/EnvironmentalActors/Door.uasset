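; Door actor that swings open and closed when ChangeState is triggered.
; A timeline drives the hinge's yaw from its starting rotation by a configurable span, clockwise or counterclockwise, and plays in reverse to close.
; Opening plays a sound at the door and lets pawns pass through by ignoring their collision, while closing restores blocking immediately.
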(event `ChangeState`
  ;[1 1 1] change state
  (if (`self.DoorOpen?`)
    (`self.CloseDoor`)
    (else
      (`self.OpenDoor`))))

(event `self.ReceiveBeginPlay`
  ;[1 1 1] Setup
  (set `self.InitialRot` (`SceneComponent.K2_GetComponentRotation` (`self.hinge`))))

(event `OpenDoor`
  (bind _hinge (`self.hinge`))
  (bind _roll (.roll (`self.InitialRot`)))
  (bind _pitch (.pitch (`self.InitialRot`)))
  (bind _yaw (.yaw (`self.InitialRot`)))
  ;[1 1 1] Open/Close
  (set `self.DoorOpen?` true)
  (`PrimitiveComponent.SetCollisionResponseToChannel` (`self.door`) "ECC_Pawn" "ECR_Ignore")
  (`GameplayStatics.PlaySoundAtLocation` "/Game/SFX/DoorOpenCue.DoorOpenCue" (`SceneComponent.K2_GetComponentLocation` (`self.DefaultSceneRoot`)) (struct) 1.0 1.0 0.0 "/Game/SFX/PipeClangAttenuation.PipeClangAttenuation" null null)
  (bind (_direction _door_rotation) (`Timeline|DoorTimeline` :!via `PlayFromStart` :!label _label)
    (:`Update`
      (if (`self.OpenClockwise`)
        (bind _returnvalue (* (/ _door_rotation 100.0) (`self.DoorSpan`)))
        (`SceneComponent.K2_SetWorldRotation` _hinge (`KismetMathLibrary.MakeRotator` _roll _pitch (- _yaw _returnvalue)) false false)
        (else
          (`SceneComponent.K2_SetWorldRotation` _hinge (`KismetMathLibrary.MakeRotator` _roll _pitch (+ _yaw _returnvalue)) false false))))))

(event `CloseDoor`
  ;[1 1 1] Open/Close
  (set `self.DoorOpen?` false)
  (`PrimitiveComponent.SetCollisionResponseToChannel` (`self.door`) "ECC_Pawn" "ECR_Block")
  (goto _label :!via `ReverseFromEnd`))

(fn `UserConstructionScript`)