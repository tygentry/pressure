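; Physics cup prop that plays ceramic impact sounds when it hits something.
; On Hit, it ignores weak contacts by checking both mesh velocity and impulse magnitude, then picks a light, medium or heavy cue from the speed.
; Sounds play at the mesh location with slight random pitch, and a DoOnce reset after a short delay throttles repeated triggers.
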(event `self.ReceiveHit`
  (params (MyComp :type "PrimitiveComponent Object Reference") (Other :type "Actor Object Reference") (OtherComp :type "PrimitiveComponent Object Reference") (bSelfMoved :type Boolean) (HitLocation :type "Vector Structure") (HitNormal :type "Vector Structure") (NormalImpulse :type "Vector Structure") (Hit :type "HitResult Structure (by ref)"))
  (bind _returnvalue (`KismetMathLibrary.RandomFloatInRange` 0.99 1.01))
  (bind _returnvalue_2 (`SceneComponent.K2_GetComponentLocation` (`self.StaticMesh`)))
  (bind _returnvalue_3 (`PrimitiveComponent.GetPhysicsLinearVelocity` (`self.StaticMesh`) "None"))
  (bind _returnvalue_4 (`KismetMathLibrary.VSize` _returnvalue_3))
  (if (and (> _returnvalue_4 30.0) (> (`KismetMathLibrary.VSize` NormalImpulse) 600.0))
    (`/Engine/EditorBlueprintResources/StandardMacros.DoOnce` false :!label _label
      (:`Completed`
        (if (< _returnvalue_4 200.0)
          (`GameplayStatics.PlaySoundAtLocation` "/Game/SFX/CeramicCollisionLightCue.CeramicCollisionLightCue" _returnvalue_2 (struct) 1.0 _returnvalue 0.0 "/Game/SFX/PipeClangAttenuation.PipeClangAttenuation" null null)
          (`KismetSystemLibrary.Delay` 0.2)
          (goto _label :!via `Reset`)
          (elif (< _returnvalue_4 500.0)
            (`GameplayStatics.PlaySoundAtLocation` "/Game/SFX/CeramicCollisionMedCue.CeramicCollisionMedCue" _returnvalue_2 (struct) 1.0 _returnvalue 0.0 "/Game/SFX/PipeClangAttenuation.PipeClangAttenuation" null null)
            (`KismetSystemLibrary.Delay` 0.2)
            (goto _label :!via `Reset`)
            (else
              (`GameplayStatics.PlaySoundAtLocation` "/Game/SFX/CeramicCollisionHeavyCue.CeramicCollisionHeavyCue" _returnvalue_2 (struct) 1.0 _returnvalue 0.0 "/Game/SFX/PipeClangAttenuation.PipeClangAttenuation" null null)
              (`KismetSystemLibrary.Delay` 0.2)
              (goto _label :!via `Reset`))))))))

(fn `UserConstructionScript`
  (`parent.UserConstructionScript`))