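; CornerPipe1 is a corner pipe item Blueprint that shows a particle effect while water flows through it.
; It extends a parent class's water-flow on and off events, calling the parent logic and then activating or deactivating its ParticleSystem.
; BeginPlay calls the off event, so the pipe starts with the effect stopped.
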(event `self.ReceiveBeginPlay`
  (`parent.ReceiveBeginPlay`)
  (`self.WaterFlowingOff`))

(event `self.WaterFlowingOn`
  (`parent.WaterFlowingOn`)
  (`ActorComponent.Activate` (`self.ParticleSystem`) false))

(event `self.WaterFlowingOff`
  (`parent.WaterFlowingOff`)
  (`ActorComponent.Deactivate` (`self.ParticleSystem`)))

(fn `UserConstructionScript`
  (`parent.UserConstructionScript`))